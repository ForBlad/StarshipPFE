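; BP_Cruser is a work-in-progress AI enemy ship that chases and shoots the player, ramming for damage and self-destructing.
; Tick sphere-traces two ranges: Bp_Vaisseau in attack range triggers impulses and rate-limited projectiles, otherwise any follow-range hit triggers look-at and AIMoveTo.
; With no hit, a random MultiGate picks impulse moves using directional overlap flags.
; Opposite move events share the same impulse vectors, and the Fire1 shot is unconnected.
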(event OnComponentBeginOverlap(Frontal)
  (params (OverlappedComponent :type Primitive%20Component%20Object%20Reference) (OtherActor :type Actor%20Object%20Reference) (OtherComp :type Primitive%20Component%20Object%20Reference) (OtherBodyIndex :type Integer) (bFromSweep :type Boolean) (SweepResult :type Hit%20Result%20Structure%20%28by%20ref%29))
  ;[0 1 1] Collisions Bool
  (Variables|Default|SetFront true))

(event OnComponentEndOverlap(Frontal)
  (params (OverlappedComponent :type Primitive%20Component%20Object%20Reference) (OtherActor :type Actor%20Object%20Reference) (OtherComp :type Primitive%20Component%20Object%20Reference) (OtherBodyIndex :type Integer))
  ;[0 1 1] Collisions Bool
  (Variables|Default|SetFront false))

(event OnComponentBeginOverlap(Front_Left)
  (params (OverlappedComponent :type Primitive%20Component%20Object%20Reference) (OtherActor :type Actor%20Object%20Reference) (OtherComp :type Primitive%20Component%20Object%20Reference) (OtherBodyIndex :type Integer) (bFromSweep :type Boolean) (SweepResult :type Hit%20Result%20Structure%20%28by%20ref%29))
  ;[0 1 1] Collisions Bool
  (Variables|Default|SetFrontLeft true))

(event OnComponentEndOverlap(Front_Left)
  (params (OverlappedComponent :type Primitive%20Component%20Object%20Reference) (OtherActor :type Actor%20Object%20Reference) (OtherComp :type Primitive%20Component%20Object%20Reference) (OtherBodyIndex :type Integer))
  ;[0 1 1] Collisions Bool
  (Variables|Default|SetFrontLeft false))

(event OnComponentBeginOverlap(Arrière_Right)
  (params (OverlappedComponent :type Primitive%20Component%20Object%20Reference) (OtherActor :type Actor%20Object%20Reference) (OtherComp :type Primitive%20Component%20Object%20Reference) (OtherBodyIndex :type Integer) (bFromSweep :type Boolean) (SweepResult :type Hit%20Result%20Structure%20%28by%20ref%29))
  ;[0 1 1] Collisions Bool
  (Variables|Default|SetRearRight true))

(event OnComponentEndOverlap(Arrière_Right)
  (params (OverlappedComponent :type Primitive%20Component%20Object%20Reference) (OtherActor :type Actor%20Object%20Reference) (OtherComp :type Primitive%20Component%20Object%20Reference) (OtherBodyIndex :type Integer))
  ;[0 1 1] Collisions Bool
  (Variables|Default|SetRearRight false))

(event OnComponentBeginOverlap(Arrière_Left)
  (params (OverlappedComponent :type Primitive%20Component%20Object%20Reference) (OtherActor :type Actor%20Object%20Reference) (OtherComp :type Primitive%20Component%20Object%20Reference) (OtherBodyIndex :type Integer) (bFromSweep :type Boolean) (SweepResult :type Hit%20Result%20Structure%20%28by%20ref%29))
  ;[0 1 1] Collisions Bool
  (Variables|Default|SetRearLeft true))

(event OnComponentEndOverlap(Arrière_Left)
  (params (OverlappedComponent :type Primitive%20Component%20Object%20Reference) (OtherActor :type Actor%20Object%20Reference) (OtherComp :type Primitive%20Component%20Object%20Reference) (OtherBodyIndex :type Integer))
  ;[0 1 1] Collisions Bool
  (Variables|Default|SetRearLeft false))

(event OnComponentBeginOverlap(Arrière)
  (params (OverlappedComponent :type Primitive%20Component%20Object%20Reference) (OtherActor :type Actor%20Object%20Reference) (OtherComp :type Primitive%20Component%20Object%20Reference) (OtherBodyIndex :type Integer) (bFromSweep :type Boolean) (SweepResult :type Hit%20Result%20Structure%20%28by%20ref%29))
  ;[0 1 1] Collisions Bool
  (Variables|Default|SetRear true))

(event OnComponentEndOverlap(Arrière)
  (params (OverlappedComponent :type Primitive%20Component%20Object%20Reference) (OtherActor :type Actor%20Object%20Reference) (OtherComp :type Primitive%20Component%20Object%20Reference) (OtherBodyIndex :type Integer))
  ;[0 1 1] Collisions Bool
  (Variables|Default|SetRear false))

(event OnComponentBeginOverlap(Droite)
  (params (OverlappedComponent :type Primitive%20Component%20Object%20Reference) (OtherActor :type Actor%20Object%20Reference) (OtherComp :type Primitive%20Component%20Object%20Reference) (OtherBodyIndex :type Integer) (bFromSweep :type Boolean) (SweepResult :type Hit%20Result%20Structure%20%28by%20ref%29))
  ;[0 1 1] Collisions Bool
  (Variables|Default|SetRight true))

(event OnComponentEndOverlap(Droite)
  (params (OverlappedComponent :type Primitive%20Component%20Object%20Reference) (OtherActor :type Actor%20Object%20Reference) (OtherComp :type Primitive%20Component%20Object%20Reference) (OtherBodyIndex :type Integer))
  ;[0 1 1] Collisions Bool
  (Variables|Default|SetRight false))

(event OnComponentBeginOverlap(Front_Right)
  (params (OverlappedComponent :type Primitive%20Component%20Object%20Reference) (OtherActor :type Actor%20Object%20Reference) (OtherComp :type Primitive%20Component%20Object%20Reference) (OtherBodyIndex :type Integer) (bFromSweep :type Boolean) (SweepResult :type Hit%20Result%20Structure%20%28by%20ref%29))
  ;[0 1 1] Collisions Bool
  (Variables|Default|SetFrontRight true))

(event OnComponentBeginOverlap(Gauche)
  (params (OverlappedComponent :type Primitive%20Component%20Object%20Reference) (OtherActor :type Actor%20Object%20Reference) (OtherComp :type Primitive%20Component%20Object%20Reference) (OtherBodyIndex :type Integer) (bFromSweep :type Boolean) (SweepResult :type Hit%20Result%20Structure%20%28by%20ref%29))
  ;[0 1 1] Collisions Bool
  (Variables|Default|SetLeft true))

(event OnComponentEndOverlap(Gauche)
  (params (OverlappedComponent :type Primitive%20Component%20Object%20Reference) (OtherActor :type Actor%20Object%20Reference) (OtherComp :type Primitive%20Component%20Object%20Reference) (OtherBodyIndex :type Integer))
  ;[0 1 1] Collisions Bool
  (Variables|Default|SetLeft false))

(event OnComponentEndOverlap(Front_Right)
  (params (OverlappedComponent :type Primitive%20Component%20Object%20Reference) (OtherActor :type Actor%20Object%20Reference) (OtherComp :type Primitive%20Component%20Object%20Reference) (OtherBodyIndex :type Integer))
  ;[0 1 1] Collisions Bool
  (Variables|Default|SetFrontRight false))

(event Custom|Move%20Left
  (bind _cube (Variables|Default|GetCube))
  ;[0 1 1] Movements forward / backward / Right / Left
  (Physics|AddImpulse _cube (* (Math|Vector|GetRightVector _cube) (Variables|Default|GetSpeed%20-%20%28y%29)) "None" true))

(event Custom|FrontMove
  (bind _cube (Variables|Default|GetCube))
  ;[0 1 1] Movements forward / backward / Right / Left
  (Physics|AddImpulse _cube (* (Math|Vector|GetForwardVector _cube) (Variables|Default|GetSpeed%20+%20%28x%29)) "None" true))

(event Custom|RearMove
  (bind _cube (Variables|Default|GetCube))
  ;[0 1 1] Movements forward / backward / Right / Left
  (Physics|AddImpulse _cube (* (Math|Vector|GetForwardVector _cube) (Variables|Default|GetSpeed%20-%20%28x%29)) "None" true))

(event Custom|Move%20Right
  (bind _cube (Variables|Default|GetCube))
  ;[0 1 1] Movements forward / backward / Right / Left
  (Physics|AddImpulse _cube (* (Math|Vector|GetRightVector _cube) (Variables|Default|GetSpeed%20+%20%28y%29)) "None" true))

(event Custom|Move
  ;[0 1 1] Movements when collision
  (Utilities|FlowControl|MultiGate true true 0
    (:Out%200
      (if (not (Variables|Default|GetFront))
        (CallFunction|FrontMove)))
    (:Out%201
      (if (Variables|Default|GetRear)
        (CallFunction|FrontMove)
        (else
          (CallFunction|RearMove))))
    (:Out%202
      (if (Variables|Default|GetRight)
        (CallFunction|MoveRight)
        (else
          (CallFunction|MoveLeft))))
    (:Out%203
      (if (Variables|Default|GetLeft)
        (CallFunction|MoveRight)
        (else
          (CallFunction|MoveLeft))))))

(event EventTick
  (params (DeltaSeconds :type Float%20%28single-precision%29))
  (bind _returnvalue (Game|Player|GetPlayerPawn 0))
  (bind _returnvalue_2 (Transformation|GetActorLocation))
  (bind _returnvalue_3 (Transformation|GetActorLocation))
  (bind _fire (Variables|Default|GetFire))
  (bind _returnvalue_4 (Transformation|GetWorldTransform _fire))
  ;[0 1 1] Box "if detect the player" Start To Attack
  (bind _outhit (Collision|SphereTraceByChannel _returnvalue_2 _returnvalue_2 (Variables|Default|GetRange%20Attack%20Player) "TraceTypeQuery1" false 0 "ForOneFrame"))
  ;[0 1 1] Hit Result "if it's player" Following Him
  (if (Utilities|Enum|Equal(Enum) (Utilities|GetDisplayName (.HitActor (Collision|BreakHitResult _outhit))) "Bp_Vaisseau")
    (CallFunction|MoveLeft)
    (CallFunction|RearMove)
    ;[0 1 1] Tir
    (Utilities|FlowControl|DoOnce false :!label _label
      (:Completed
        (Game|SpawnActorfromClass "/Game/Loic/AI_WIP_Behavior/PRojectile/BP_Small_AI_Projectile.BP_Small_AI_Projectile_C" (Math|Transform|MakeTransform (.location _returnvalue_4) (.rotation _returnvalue_4) (Math|Vector|MakeVector 0.09 0.05 0.05)) "Undefined" 0 0)
        (Utilities|FlowControl|Delay (Variables|Default|GetRateofFire))
        (goto _label Reset)))
    (else
      (bind _outhit_2 (Collision|SphereTraceByChannel _returnvalue_3 _returnvalue_3 (Variables|Default|GetRange%20Follow%20Player) "TraceTypeQuery1" false 0 "ForOneFrame"))
      (if (.bBlockingHit (Collision|BreakHitResult _outhit_2))
        (CallFunction|FrontMove)
        (Transformation|SetRelativeRotation (Variables|Default|GetCube) (Math|Rotator|FindLookatRotation (Transformation|GetActorLocation) (Transformation|GetActorLocation _returnvalue)) false false)
        (AI|AIMoveTo 0 "0, 0, 0" _returnvalue 5.0 false)
        (else
          (CallFunction|Move))))))

(event Game|Damage|EventAnyDamage
  (params (Damage :type Float%20%28single-precision%29) (DamageType :type Damage%20Type%20Object%20Reference) (InstigatedBy :type Controller%20Object%20Reference) (DamageCauser :type Actor%20Object%20Reference))
  ;[0 1 1] Damage
  (Variables|Default|SetHealth (Math|Float|Clamp(Float) (- (Variables|Default|GetHealth) Damage) 0.0 (Variables|Default|GetMaxHealth)))
  (if (<= (Variables|Default|GetHealth) 0.0)
    (Actor|DestroyActor)))

(event Collision|EventHit
  (params (MyComp :type Primitive%20Component%20Object%20Reference) (Other :type Actor%20Object%20Reference) (OtherComp :type Primitive%20Component%20Object%20Reference) (bSelfMoved :type Boolean) (HitLocation :type Vector :default "0, 0, 0") (HitNormal :type Vector :default "0, 0, 0") (NormalImpulse :type Vector :default "0, 0, 0") (Hit :type Hit%20Result%20Structure%20%28by%20ref%29))
  ;[0 1 1] Damage
  (Utilities|Casting|CastToBP_ProjectilePlayerBase Other
    (:CastFailed
      (bind _asbp_player (Utilities|Casting|CastToBP_Player Other))
      (Game|Damage|ApplyDamage _asbp_player 5e+01 0 0)
      (Actor|DestroyActor))))

(fn ConstructionScript)