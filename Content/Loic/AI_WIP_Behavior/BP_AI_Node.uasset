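; Waypoint node for AI fighter tracks: the node flagged first registers itself with its owning AI spawner on BeginPlay.
; When a non-following fighter's hull enters the sphere, it is sent to NextNode (gated by DoOnce) and takes the node's rotation coefficient.
; The last node loops it to the first or targets a far point derived from the arrow's direction.
; FindNextNode's nearest-neighbour linking is disconnected, and debug prints remain.
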(event OnComponentBeginOverlap(Sphere1)
  (params (OverlappedComponent :type Primitive%20Component%20Object%20Reference) (OtherActor :type Actor%20Object%20Reference) (OtherComp :type Primitive%20Component%20Object%20Reference) (OtherBodyIndex :type Integer) (bFromSweep :type Boolean) (SweepResult :type Hit%20Result%20Structure%20%28by%20ref%29))
  (bind _owneraispawner (Variables|Default|GetOwnerAISpawner))
  (Development|PrintString "HelHHHHHHlo")
  (bind _asai_fighter_new_2 (Utilities|Casting|CastToAI_Fighter_New2 (Components|GetOwner OtherComp)))
  (if (and (not (Variables|/Game/Loic/AI_WIP_Behavior/AI_Fighter_New2.AI_Fighter_New2_C|GetFollowShip _asai_fighter_new_2)) (Components|ComponentHasTag OtherComp "Hull"))
    (Development|PrintString "TRUEEE")
    (if (Variables|Default|GetIsLast)
      (Development|PrintString "IS LAST")
      (if (Variables|/Game/Loic/AI_WIP_Behavior/BP_AI_Spawner.BP_AI_Spawner_C|GetloopTrack _owneraispawner)
        (Default|TraveltoNextTarget _asai_fighter_new_2 (Variables|/Game/Loic/AI_WIP_Behavior/BP_AI_Spawner.BP_AI_Spawner_C|GetFirstTrackNode _owneraispawner))
        (Variables|/Game/Loic/AI_WIP_Behavior/AI_Fighter_New2.AI_Fighter_New2_C|SetTiltEntropy _asai_fighter_new_2 1.0 :!label _label)
        (Variables|/Game/Loic/AI_WIP_Behavior/AI_Fighter_New2.AI_Fighter_New2_C|SetRotationCoefficient _asai_fighter_new_2 (Variables|Default|GetRotationCoefficient))
        (else
          (Variables|/Game/Loic/AI_WIP_Behavior/AI_Fighter_New2.AI_Fighter_New2_C|SetlastLocation _asai_fighter_new_2 (Transformation|GetWorldTransform (Variables|/Game/Loic/AI_WIP_Behavior/AI_Fighter_New2.AI_Fighter_New2_C|GetHull _asai_fighter_new_2)))
          (Variables|/Game/Loic/AI_WIP_Behavior/AI_Fighter_New2.AI_Fighter_New2_C|SetLastFrameDirection _asai_fighter_new_2 (Math|Vector|GetForwardVector (Variables|/Game/Loic/AI_WIP_Behavior/AI_Fighter_New2.AI_Fighter_New2_C|GetHull _asai_fighter_new_2)))
          (Variables|/Game/Loic/AI_WIP_Behavior/AI_Fighter_New2.AI_Fighter_New2_C|SetTargetCoords _asai_fighter_new_2 (Math|Transform|MakeTransform (* (Math|Vector|GetForwardVector (Variables|Default|GetArrow)) 1e+04) "0, 0, 0" "1,1,1"))))
      (elif (Variables|Default|GetdoOnce)
        (Default|TraveltoNextTarget (stale _asai_fighter_new_2) (Variables|Default|GetNextNode))
        (goto _label)))))

(event OnComponentEndOverlap(Sphere1)
  (params (OverlappedComponent :type Primitive%20Component%20Object%20Reference) (OtherActor :type Actor%20Object%20Reference) (OtherComp :type Primitive%20Component%20Object%20Reference) (OtherBodyIndex :type Integer)))

(event Custom|kek
  (if (Variables|Default|GetIsFirst)
    (CallFunction|FindNextNode self)
    (Variables|/Game/Loic/AI_WIP_Behavior/BP_AI_Spawner.BP_AI_Spawner_C|SetFirstTrackNode (Variables|Default|GetOwnerAISpawner) self)))

(event EventBeginPlay
  (if (Variables|Default|GetIsFirst)
    (CallFunction|FindNextNode self)
    (Variables|/Game/Loic/AI_WIP_Behavior/BP_AI_Spawner.BP_AI_Spawner_C|SetFirstTrackNode (Variables|Default|GetOwnerAISpawner) self)))

(event Collision|EventActorBeginOverlap
  (params (OtherActor :type Actor%20Object%20Reference)))

(event EventTick
  (params (DeltaSeconds :type Float%20%28single-precision%29)))

(fn ConstructionScript)

(fn FindNextNode
  (params (LastNode :type BP%20AI%20Node%20Object%20Reference)))