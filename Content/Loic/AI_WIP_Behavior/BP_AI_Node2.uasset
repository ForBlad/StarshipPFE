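; Work-in-progress waypoint node for AI fighter tracks, linked to an owning AI spawner.
; The node flagged first registers as the spawner's FirstTrackNode on BeginPlay and calls FindNextNode, whose nearest-node chaining and looping logic is disconnected.
; Sphere overlap stores the fighter and, unless the node is last, sends it to NextNode.
; Tick re-issues travel when the stored ship's hull sits at the node's centre; debug prints remain throughout.
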(event OnComponentBeginOverlap(Sphere1)
  (params (OverlappedComponent :type Primitive%20Component%20Object%20Reference) (OtherActor :type Actor%20Object%20Reference) (OtherComp :type Primitive%20Component%20Object%20Reference) (OtherBodyIndex :type Integer) (bFromSweep :type Boolean) (SweepResult :type Hit%20Result%20Structure%20%28by%20ref%29))
  (bind _asai_fighter_new (Utilities|Casting|CastToAI_Fighter_New OtherActor))
  (if (Variables|/Game/Loic/AI_WIP_Behavior/BP_AI_Spawner.BP_AI_Spawner_C|GetspawnWithoutTrack (Variables|Default|GetOwnerAISpawner))
    (Development|PrintString (Utilities|GetObjectName (Variables|/Game/Loic/AI_WIP_Behavior/AI_Fighter_New.AI_Fighter_New_C|GetTestActorTarget _asai_fighter_new)) true true "(R=0.000000,G=0.660000,B=1.000000,A=1.000000)" 5.0))
  (Math|Integer|IncrementInt (Variables|Default|GetVAR)
    (:%20%20
      (Variables|Default|Setship _asai_fighter_new)
      (if (Variables|Default|GetIsLast)
        (Development|PrintString "IS LAST / AI NODE")
        (else
          (Default|TraveltoNextNode _asai_fighter_new (Variables|Default|GetNextNode))
          (Development|PrintString (Utilities|String|ToString(Vector) (.location (Variables|/Game/Loic/AI_WIP_Behavior/AI_Fighter_New.AI_Fighter_New_C|GetlastLocation _asai_fighter_new))) true true "(R=0.000000,G=0.660000,B=1.000000,A=1.000000)" 3e+01))))))

(event OnComponentEndOverlap(Sphere1)
  (params (OverlappedComponent :type Primitive%20Component%20Object%20Reference) (OtherActor :type Actor%20Object%20Reference) (OtherComp :type Primitive%20Component%20Object%20Reference) (OtherBodyIndex :type Integer))
  (Utilities|Casting|CastToAI_Fighter_New OtherActor))

(event Custom|kek
  (if (Variables|Default|GetIsFirst)
    (CallFunction|FindNextNode self)
    (Variables|/Game/Loic/AI_WIP_Behavior/BP_AI_Spawner.BP_AI_Spawner_C|SetFirstTrackNode (Variables|Default|GetOwnerAISpawner) self)))

(event EventBeginPlay
  (if (Variables|Default|GetIsFirst)
    (CallFunction|FindNextNode self)
    (Variables|/Game/Loic/AI_WIP_Behavior/BP_AI_Spawner.BP_AI_Spawner_C|SetFirstTrackNode (Variables|Default|GetOwnerAISpawner) self)))

(event Collision|EventActorBeginOverlap
  (params (OtherActor :type Actor%20Object%20Reference)))

(event EventTick
  (params (DeltaSeconds :type Float%20%28single-precision%29))
  (if (Math|Vector|Equal(Vector) (Transformation|GetWorldLocation (Variables|/Game/Loic/AI_WIP_Behavior/AI_Fighter_New.AI_Fighter_New_C|GetHull (Variables|Default|Getship))) (Transformation|GetWorldLocation (Variables|Default|GetDefaultSceneRoot self)) 1.0)
    (Default|TraveltoNextNode (stale OnComponentBeginOverlap(Sphere1) _asai_fighter_new) (Variables|Default|GetNextNode))
    (Development|PrintString "")))

(fn ConstructionScript)

(fn FindNextNode
  (params (LastNode :type BP%20AI%20Node%20Object%20Reference)))