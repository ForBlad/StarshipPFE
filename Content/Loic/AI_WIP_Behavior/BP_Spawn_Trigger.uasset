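; One-shot trigger that, when the starship enters, either fires all linked enemy and special spawners then destroys itself, or runs a wave room.
; Wave rooms poll by timer, spawning up to five waves from unused, off-screen spawners matched by ship class.
; WaveCounter tallies kills to flag wave completion, and linked doors open after the last wave.
; Indicator meshes and lights turn red on entry, then blue as waves progress.
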(event OnComponentBeginOverlap(Trigger)
  (params (OverlappedComponent :type Primitive%20Component%20Object%20Reference) (OtherActor :type Actor%20Object%20Reference) (OtherComp :type Primitive%20Component%20Object%20Reference) (OtherBodyIndex :type Integer) (bFromSweep :type Boolean) (SweepResult :type Hit%20Result%20Structure%20%28by%20ref%29))
  (Utilities|Casting|CastToBp_Starship OtherActor)
  (Utilities|FlowControl|DoOnce false
    (:Completed
      (Utilities|FlowControl|Sequence
        (:then_0
          (CallFunction|ChangeLightColor "/Game/Steven/StevenGPE/Materials/M_Red_Instance.M_Red_Instance" "/Game/Steven/StevenGPE/Materials/M_Blue.M_Blue" (Variables|Default|Getred)))
        (:then_1
          (if (Variables|Default|GetWaveRoomSpawner?)
            (Audio|PlaySound2D "/Game/Assets/Audio/SOUNDBANK/UI/UI_MENU_GAMEOVER/UI_MENU_GameOver_01.UI_MENU_GameOver_01" 1e+01 0.8 0.0 0 0)
            (CallFunction|WaveSpawner)
            (else
              (for _array_element (Variables|Default|GetSpawnersToTrigger)
                (Default|Spawn _array_element "NewEnumerator0" (Variables|/Game/Loic/AI_WIP_Behavior/BP_AI_Spawner.BP_AI_Spawner_C|GetType%20Of%20Cruiser%20%28if%20cruiser%29 _array_element)))
              (for _array_element_2 (Variables|Default|GetSpecialEnemiesToTrigger)
                (Default|Spawn _array_element_2))
              (Actor|DestroyActor self))))))))

(event Custom|Spawn%20Wave%201
  (params (NewParam :type Array%20of%20ShipClassEnum1%20Enums :default "NewEnumerator0"))
  (bind _spawnerstotrigger (Variables|Default|GetSpawnersToTrigger))
  (for _array_element NewParam
    (bind _array_element_2 (Utilities|Array|ForEachLoopwithBreak _spawnerstotrigger :!label _label)
      (:LoopBody
        (bind _isonscreen_ (Default|IsonScreen? _array_element_2))
        (if (Math|Boolean|ANDBoolean (Utilities|Enum|Equal(Enum) (.Value (Utilities|Map|Find (Variables|Default|GetShipTypeMap) _array_element)) (Variables|/Game/Loic/AI_WIP_Behavior/BP_AI_Spawner.BP_AI_Spawner_C|GetShip%20Class _array_element_2)) (not _isonscreen_) (not (Variables|/Game/Loic/AI_WIP_Behavior/BP_AI_Spawner.BP_AI_Spawner_C|GetUsed%20In%20Current%20Wave _array_element_2)))
          (Default|Spawn _array_element_2 _array_element "NewEnumerator0")
          (Variables|/Game/Loic/AI_WIP_Behavior/BP_AI_Spawner.BP_AI_Spawner_C|SetUsed%20In%20Current%20Wave _array_element_2 true)
          (goto _label Break)))))
  (for _array_element_3 _spawnerstotrigger
    (Variables|/Game/Loic/AI_WIP_Behavior/BP_AI_Spawner.BP_AI_Spawner_C|SetUsed%20In%20Current%20Wave _array_element_3 false)))

(event Custom|Wave%20Spawner
  (bind _wavenumber (Variables|Default|GetWaveNumber))
  (Utilities|Time|SetTimerbyEvent (delegate Custom|Wave%20Spawner) 0.5 true)
  (if (Variables|Default|GetWaveFinished)
    (Variables|Default|SetWaveFinished false)
    (switch int (Variables|Default|GetWaveNumber)
      (:0
        (Variables|Default|SetCurrent%20Wave (Variables|Default|GetWave%201))
        (Variables|Default|SetTotalEnemiesInWave (Utilities|Array|Length (Variables|Default|GetCurrent%20Wave)) :!label _label)
        (CallFunction|ChangeLightColor "/Game/Steven/StevenGPE/Materials/M_Red_Instance.M_Red_Instance" "/Game/Steven/StevenGPE/Materials/M_Blue.M_Blue" (Variables|Default|Getblue))
        (if (> (Utilities|Array|Length (Variables|Default|GetCurrent%20Wave)) 0)
          (Utilities|FlowControl|Delay (Variables|Default|GetTriggerDelay))
          (Variables|Default|SetTriggerDelay (Variables|Default|GetTimeBetweenWaves))
          (CallFunction|SpawnWave1 (Variables|Default|GetCurrent%20Wave))
          (Math|Integer|IncrementInt _wavenumber
            (:%20%20
              (Development|PrintString (Utilities|String|ToString(Integer) _wavenumber))))
          (else
            (Utilities|FlowControl|Delay 2.0 :!label _label_2)
            (Audio|PlaySound2D "/Game/Assets/Audio/SOUNDBANK/UI/UI_MENU_GAMEOVER/success3.success3" 7.0 1.0 0.0 0 0)
            (for _array_element (Variables|Default|GetDoorsToOpen)
              (Variables|/Game/Blueprints/DoorsNew/Door_Parent.Door_Parent_C|SetButtonsNeeded _array_element 0)
              (Default|OpenDoor _array_element)))))
      (:1
        (Variables|Default|SetCurrent%20Wave (Variables|Default|GetWave%202))
        (goto _label))
      (:2
        (Variables|Default|SetCurrent%20Wave (Variables|Default|GetWave%203))
        (goto _label))
      (:3
        (Variables|Default|SetCurrent%20Wave (Variables|Default|GetWave%204))
        (goto _label))
      (:4
        (Variables|Default|SetCurrent%20Wave (Variables|Default|GetWave%205))
        (goto _label))
      (:5
        (goto _label_2)))))

(event Custom|Change%20Light%20Color
  (params (Red%20Color :type Material%20Instance%20Object%20Reference) (Blue%20Color :type Material%20Instance%20Object%20Reference) (Light%20Color :type Linear%20Color%20Structure))
  (bind _changing_poinlight (Variables|Default|GetChanging%20PoinLight))
  (bind _wavenumber (Variables|Default|GetWaveNumber))
  (bind _staticmeshes (Variables|Default|GetStaticMeshes))
  (bind _returnvalue (- _wavenumber 1))
  (bind _output (Utilities|Array|Get(acopy) _staticmeshes _returnvalue))
  (bind _staticmeshcomponent (Variables|/Script/Engine.StaticMeshActor|GetStaticMeshComponent _output))
  ;[1 1 1] SET MESH AND LIGHT COLOR
  (if (== _wavenumber 0)
    (for _array_element _staticmeshes
      (Utilities|IsValid (Variables|/Script/Engine.StaticMeshActor|GetStaticMeshComponent _array_element)
        (:Is%20Valid
          (Rendering|Material|SetMaterial (Variables|/Script/Engine.StaticMeshActor|GetStaticMeshComponent _array_element) 1 Red%20Color)
          (Utilities|IsValid (Variables|/Script/Engine.Light|GetLightComponent (Utilities|Array|Get(acopy) _changing_poinlight (Variables|Default|GetLightNumber)))
            (:Is%20Valid
              (Rendering|Components|Light|SetLightColor (Variables|/Script/Engine.Light|GetLightComponent (Utilities|Array|Get(acopy) _changing_poinlight (Variables|Default|GetLightNumber))) Light%20Color true)
              (bind _result (Math|Integer|IncrementInt (Variables|Default|GetLightNumber))
                (:%20%20
                  (Rendering|Components|Light|SetLightColor (Variables|/Script/Engine.Light|GetLightComponent (Utilities|Array|Get(acopy) _changing_poinlight _result)) Light%20Color true)
                  (Math|Integer|IncrementInt (Variables|Default|GetLightNumber)))))))))
    (else
      (Utilities|FlowControl|Sequence
        (:then_0
          (Utilities|FlowControl|DoOnce false
            (:Completed
              (Variables|Default|SetLightNumber 0))))
        (:then_1
          (Utilities|IsValid _staticmeshcomponent
            (:Is%20Valid
              (Rendering|Material|SetMaterial _staticmeshcomponent 1 Blue%20Color)
              (Rendering|Components|Light|SetLightColor (Variables|/Script/Engine.Light|GetLightComponent (Utilities|Array|Get(acopy) _changing_poinlight (Variables|Default|GetLightNumber))) Light%20Color true)
              (bind _result_2 (Math|Integer|IncrementInt (Variables|Default|GetLightNumber))
                (:%20%20
                  (Rendering|Components|Light|SetLightColor (Variables|/Script/Engine.Light|GetLightComponent (Utilities|Array|Get(acopy) _changing_poinlight _result_2)) Light%20Color true)
                  (Math|Integer|IncrementInt (Variables|Default|GetLightNumber)))))))))))

(event EventBeginPlay)

(event Collision|EventActorBeginOverlap
  (params (OtherActor :type Actor%20Object%20Reference)))

(event EventTick
  (params (DeltaSeconds :type Float%20%28single-precision%29)))

(fn ConstructionScript)

(fn SpawnWave
  (params (Ship%20Type :type Array%20of%20ShipClassEnum1%20Enums :default "NewEnumerator0"))
  (bind _spawnerstotrigger (Variables|Default|GetSpawnersToTrigger))
  (for _array_element Ship%20Type
    (bind _array_element_2 (Utilities|Array|ForEachLoopwithBreak _spawnerstotrigger :!label _label)
      (:LoopBody
        (bind _isonscreen_ (Default|IsonScreen? _array_element_2))
        (if (Math|Boolean|ANDBoolean (Utilities|Enum|Equal(Enum) (.Value (Utilities|Map|Find (Variables|Default|GetShipTypeMap) _array_element)) (Variables|/Game/Loic/AI_WIP_Behavior/BP_AI_Spawner.BP_AI_Spawner_C|GetShip%20Class _array_element_2)) (not _isonscreen_) (not (Variables|/Game/Loic/AI_WIP_Behavior/BP_AI_Spawner.BP_AI_Spawner_C|GetUsed%20In%20Current%20Wave _array_element_2)))
          (Default|Spawn _array_element_2 _array_element "NewEnumerator0")
          (Variables|/Game/Loic/AI_WIP_Behavior/BP_AI_Spawner.BP_AI_Spawner_C|SetUsed%20In%20Current%20Wave _array_element_2 true)
          (goto _label Break)))))
  (for _array_element_3 _spawnerstotrigger
    (Variables|/Game/Loic/AI_WIP_Behavior/BP_AI_Spawner.BP_AI_Spawner_C|SetUsed%20In%20Current%20Wave _array_element_3 false)))

(fn WaveCounter
  (bind _result (Math|Integer|IncrementInt (Variables|Default|GetEnemiesKilledInWave))
    (:%20%20
      (if (== _result (Variables|Default|GetTotalEnemiesInWave))
        (Variables|Default|SetWaveFinished (== _result (Variables|Default|GetTotalEnemiesInWave)))
        (Variables|Default|SetEnemiesKilledInWave 0)
        (Audio|SpawnSound2D "/Game/Assets/Audio/SOUNDBANK/SFX/SFX_SHIP/CRUISER/SFX_SHIP_CRUISER_Triggered_03.SFX_SHIP_CRUISER_Triggered_03" 6.0 1.0 0.0 0)))))