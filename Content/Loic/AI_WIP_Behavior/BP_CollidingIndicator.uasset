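; BP_CollidingIndicator is a helper actor that keeps an EnemyIndicator widget on screen over the AI that owns it, pinned near the screen edges.
; BeginPlay creates the widget for player 0, with no add-to-viewport call here.
; Each Tick projects AiOwner's location to screen, applies OffsetPosition and clamps it within viewport margins.
; It deprojects that point to move its own root into world space, then reprojects the root to position the widget.
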(event EventBeginPlay
  (bind _returnvalue (UserInterface|CreateWidget "/Game/Loic/AI_WIP_Behavior/EnemyIndicator.EnemyIndicator_C" (Game|GetPlayerController 0)))
  (Variables|Default|SetIndicatorWidget _returnvalue))

(event Collision|EventActorBeginOverlap
  (params (OtherActor :type Actor%20Object%20Reference)))

(event EventTick
  (params (DeltaSeconds :type Float%20%28single-precision%29))
  (bind _returnvalue (Game|GetPlayerController 0))
  (bind _offsetposition (Variables|Default|GetOffsetPosition))
  (bind _offsetposition_2 (Variables|Default|GetOffsetPosition))
  (bind _ai_owner (Variables|Default|GetAi_Owner))
  (bind _returnvalue_2 (Transformation|GetActorLocation _ai_owner))
  (bind _returnvalue_3 (/ _offsetposition 2.0))
  (bind (_sizex _sizey) (HUD|GetViewportSize _returnvalue))
  (bind _returnvalue_4 (Math|Float|Truncate _offsetposition_2))
  (bind _returnvalue_5 (Math|Conversions|ToFloat(Integer) _returnvalue_4))
  (bind _screenposition (Class|GameplayStatics|ProjectWorldtoScreen _returnvalue _returnvalue_2 false))
  (Transformation|SetWorldLocation (Variables|Default|GetDefaultSceneRoot) (.WorldPosition (Class|GameplayStatics|DeprojectScreentoWorld _returnvalue (Math|Vector2D|MakeVector2D (Math|Float|Clamp(Float) (+ (.x _screenposition) _returnvalue_3) 25.0 (+ (- (Math|Conversions|ToFloat(Integer) _sizex) 25.0) _returnvalue_5)) (Math|Float|Clamp(Float) (+ (.y _screenposition) _returnvalue_3) 25.0 (+ (- (Math|Conversions|ToFloat(Integer) _sizey) 25.0) _returnvalue_5))))) false false)
  (Class|UserWidget|SetPositioninViewport (Variables|Default|GetIndicatorWidget) (.ScreenPosition (Class|GameplayStatics|ProjectWorldtoScreen _returnvalue (Transformation|GetWorldLocation (Variables|Default|GetDefaultSceneRoot)) false)) true))

(fn ConstructionScript)