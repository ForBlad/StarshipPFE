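; Placed spawner for AI cruisers and fighters that registers with a Trigger and hides its class-preview meshes at play.
; Spawn waits a start delay, then creates one ship without a track, or loops with delays up to NumberOfShips.
; Ships get speed and path settings, with fighters sent along the track when one is used.
; Wave-room mode forces trackless spawning, and AIDestroyed advances the Trigger's wave counter.
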(event Custom|Spawn
  (params (Cruiser%20Type :type ShipClassEnum1%20Enum :default "NewEnumerator0"))
  (bind _initial_speed (Variables|Default|GetInitial%20Speed))
  (bind _ship_class (Variables|Default|GetShip%20Class))
  (bind _ai_class (Variables|Default|GetAI%20Class))
  (bind _arrow (Variables|Default|GetArrow))
  (bind _value (Utilities|Map|Find _ai_class _ship_class))
  (bind _returnvalue (Transformation|GetWorldTransform _arrow))
  ;[1 1 1] SPAWN
  (Utilities|FlowControl|Delay (Variables|Default|GetDelayStart))
  (if (Variables|Default|GetspawnWithoutTrack)
    (if (== _value "/Game/Loic/AI_WIP_Behavior/AI_Cruser2.AI_Cruser2_C") :!label _label
      (bind _returnvalue_2 (Game|SpawnActorfromClass "/Game/Loic/AI_WIP_Behavior/AI_Cruser2.AI_Cruser2_C" (Math|Transform|MakeTransform (.location _returnvalue) (.rotation _returnvalue) "0.750000,0.750000,0.750000") "Undefined" self (.Value (Utilities|Map|Find (Variables|Default|GetCruiser%20Type%20Map) Cruiser%20Type)) 0))
      (Variables|/Game/Loic/AI_WIP_Behavior/AI_Cruser2.AI_Cruser2_C|SetSpeed%20+%20%28x%29 _returnvalue_2 _initial_speed :!label _label_2)
      (if (Variables|Default|GetWaveRoom?)
        (Variables|/Game/Loic/AI_WIP_Behavior/AI_Cruser2.AI_Cruser2_C|SetisWaifuSafe? _returnvalue_2 false)
        (else
          (Variables|/Game/Loic/AI_WIP_Behavior/AI_Cruser2.AI_Cruser2_C|SetstickToPath _returnvalue_2 (Variables|Default|GetstayOnTrack))))
      (Math|Integer|IncrementInt (Variables|Default|Geti)
        (:%20%20
          (Variables|/Game/Loic/AI_WIP_Behavior/AI_Cruser2.AI_Cruser2_C|SetMoveFront _returnvalue_2 true)
          (Variables|/Game/Loic/AI_WIP_Behavior/AI_Cruser2.AI_Cruser2_C|SetFollowShip _returnvalue_2 true)))
      (else
        (bind _returnvalue_3 (Game|SpawnActorfromClass _value (Math|Transform|MakeTransform (.location _returnvalue) (.rotation _returnvalue) "0.750000,0.750000,0.750000") "Undefined" self 0))
        (bind _asai_fighter_new_2 (Utilities|Casting|CastToAI_Fighter_New2 _returnvalue_3)
          (:then
            (Utilities|Array|Add (Variables|Default|GetSpawned_Enemies) _asai_fighter_new_2)
            (Variables|/Game/Loic/AI_WIP_Behavior/AI_Fighter_New2.AI_Fighter_New2_C|SetMySpawner _asai_fighter_new_2 self)
            (Variables|/Game/Loic/AI_WIP_Behavior/AI_Fighter_New2.AI_Fighter_New2_C|SetSpeed%20+%20%28x%29 _asai_fighter_new_2 _initial_speed)
            (if (Variables|Default|GetWaveRoom?)
              (Variables|/Game/Loic/AI_WIP_Behavior/AI_Fighter_New2.AI_Fighter_New2_C|SetstickToPath _asai_fighter_new_2 false)
              (Default|AlternativeActivation _asai_fighter_new_2)
              (else
                (Variables|/Game/Loic/AI_WIP_Behavior/AI_Fighter_New2.AI_Fighter_New2_C|SetstickToPath _asai_fighter_new_2 (Variables|Default|GetstayOnTrack))
                (if (Variables|Default|GetspawnWithoutTrack)
                  _
                  (else
                    (Default|OffYouGo _asai_fighter_new_2 (Variables|Default|GetFirstTrackNode))))))
            (Math|Integer|IncrementInt (Variables|Default|Geti)
              (:%20%20
                (Variables|/Game/Loic/AI_WIP_Behavior/AI_Fighter_New2.AI_Fighter_New2_C|SetMoveFront _asai_fighter_new_2 true))))
          (:CastFailed
            (goto _label_2)))))
    (else
      ;[1 1 1] WHILE LOOP WITH DELAY
      (if (< (Variables|Default|Geti) (Variables|Default|GetNumberOfShips)) :!label _label_3
        (Utilities|FlowControl|Sequence
          (:then_0
            (goto _label))
          (:then_1
            (Utilities|FlowControl|Delay (Variables|Default|GetDelayBetweenSpawns))
            (goto _label_3)))))))

(event EventBeginPlay
  (bind _trigger (Variables|Default|GetTrigger))
  (Rendering|SetVisibility (Variables|Default|GetStaticMesh) false false)
  (Rendering|SetVisibility (Variables|Default|GetStaticMesh1) false false)
  (Utilities|IsValid _trigger
    (:Is%20Valid
      (Utilities|Array|Add (Variables|/Game/Loic/AI_WIP_Behavior/BP_Spawn_Trigger.BP_Spawn_Trigger_C|GetSpawnersToTrigger _trigger) self))
    (:Is%20Not%20Valid
      _))
  (if (Variables|Default|GetWaveRoom?)
    (Variables|Default|SetstayOnTrack false)
    (Variables|Default|SetspawnWithoutTrack true)
    (Variables|Default|SetloopTrack false)))

(event Collision|EventActorBeginOverlap
  (params (OtherActor :type Actor%20Object%20Reference)))

(event EventTick
  (params (DeltaSeconds :type Float%20%28single-precision%29)))

(fn ConstructionScript
  (bind _staticmesh (Variables|Default|GetStaticMesh))
  (bind _staticmesh1 (Variables|Default|GetStaticMesh1))
  (if (Utilities|Enum|Equal(Enum) (Variables|Default|GetShip%20Class) "NewEnumerator0")
    (Rendering|SetVisibility _staticmesh true false)
    (Rendering|SetVisibility _staticmesh1 false false)
    (else
      (Rendering|SetVisibility _staticmesh1 true false)
      (Rendering|SetVisibility _staticmesh false false))))

(fn IsonScreen?
  (bind _returnvalue (Game|GetPlayerController 0))
  (bind _returnvalue_2 (Viewport|GetViewportSize))
  (bind _staticmesh (Variables|Default|GetStaticMesh))
  (bind _returnvalue_3 (Transformation|GetWorldLocation _staticmesh))
  (bind _screenlocation (Class|PlayerController|ProjectWorldLocationtoScreen _returnvalue _returnvalue_3 false))
  (return (Math|Boolean|ANDBoolean (> (.x _screenlocation) 0.0) (> (.y _screenlocation) 0.0) (< (.x _screenlocation) (.x _returnvalue_2)) (< (.y _screenlocation) (.y _returnvalue_2)))))

(fn AIDestroyed
  (if (Variables|Default|GetWaveRoom?)
    (Default|WaveCounter (Variables|Default|GetTrigger))))