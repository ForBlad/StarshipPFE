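; Work-in-progress enemy that fires radial bursts of projectiles while the player's starship is within range.
; BeginPlay precomputes a ring of spawn offsets around the cube and starts the timed RespectWomenMode event.
; That event triggers short repeated volleys via KeepYourHandsOffOfHer, with Shoot spawning an outward projectile and muzzle effect at each offset.
; Despite its name, Spin only oscillates two dynamic materials on Tick; off-screen indicator and aimed-fire logic are disconnected.
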(event Custom|RespectWomenMode
  (Utilities|Time|SetTimerbyEvent (delegate Custom|RespectWomenMode) 8.0 true 0.5)
  (Variables|Default|SetBurstIncr 0)
  (CallFunction|KeepYourHandsOffOfHer!))

(event Custom|Keep%20Your%20Hands%20Off%20Of%20Her!
  (if (< (Math|Vector|VectorLength (- (Transformation|GetWorldLocation (Variables|/Script/Engine.Actor|GetRootComponent (Variables|Default|Getship))) (Transformation|GetWorldLocation (Variables|Default|GetHull)))) (Variables|Default|GetloseInterestRange))
    (Utilities|WhileLoopwithDelay (< (Variables|Default|GetBurstIncr) 3) 0.2
      (:Loop%20Body
        (Math|Integer|IncrementInt (Variables|Default|GetBurstIncr)
          (:%20%20
            (CallFunction|Shoot)))))))

(event EventBeginPlay
  (bind _returnvalue (Actor|GetActorOfClass "/Game/Thibaud/Blueprints/Player/Bp_Starship.Bp_Starship_C"))
  (Variables|Default|Setship _returnvalue)
  (CallFunction|SetUpBulletSpawners)
  (CallFunction|RespectWomenMode)
  (bind _returnvalue_2 (Rendering|Material|CreateDynamicMaterialInstance (Variables|Default|GetCube) 0 "/Game/Assets/Materials/M_Greenish_L.M_Greenish_L" "None" :!class /Script/Engine.PrimitiveComponent))
  (Variables|Default|SetDyn_Mat_Greenish _returnvalue_2)
  (bind _returnvalue_3 (Rendering|Material|CreateDynamicMaterialInstance (Variables|Default|GetCube1) 0 "/Game/Assets/Materials/M_Purple_L.M_Purple_L" "None" :!class /Script/Engine.PrimitiveComponent))
  (Variables|Default|SetDyn_Mat_Purple _returnvalue_3))

(event Collision|EventActorBeginOverlap
  (params (OtherActor :type Actor%20Object%20Reference)))

(event EventTick
  (params (DeltaSeconds :type Float%20%28single-precision%29))
  (CallFunction|Spin DeltaSeconds))

(fn ConstructionScript)

(fn Spin
  (params (DeltaTime :type Float%20%28single-precision%29))
  (if (or (< (Variables|Default|GetMatLerpAlpha) 0.0) (> (Variables|Default|GetMatLerpAlpha) 1.0))
    (Variables|Default|SetLerpControlValue (* (Variables|Default|GetLerpControlValue) -1.0)))
  (bind _output_get (Variables|Default|SetMatLerpAlpha (+ (+ (* (Variables|Default|GetLerpControlValue) DeltaTime) 0.0) (Variables|Default|GetMatLerpAlpha))))
  (Rendering|Material|SetScalarParameterValue (Variables|Default|GetDyn_Mat_Greenish) "LerpAlpha" _output_get :!class /Script/Engine.MaterialInstanceDynamic)
  (Rendering|Material|SetScalarParameterValue (Variables|Default|GetDyn_Mat_Purple) "LerpAlpha" _output_get :!class /Script/Engine.MaterialInstanceDynamic))

(fn Shoot
  (bind _hull (Variables|Default|GetHull))
  (bind _returnvalue (Transformation|GetWorldLocation _hull))
  (for _array_element (Variables|Default|GetBulletSpawners)
    (Game|SpawnActorfromClass "/Game/Blueprints/Projectiles/BP_ProjectileEnemyTwo.BP_ProjectileEnemyTwo_C" (Math|Transform|MakeTransform (+ _array_element _returnvalue) (Math|Rotator|MakeRotator (.roll (Math|Conversions|RotationFromXVector (Math|Vector|GetUnitDirection(Vector) _returnvalue (+ _array_element _returnvalue)))) (.pitch (Math|Conversions|RotationFromXVector (Math|Vector|GetUnitDirection(Vector) _returnvalue (+ _array_element _returnvalue)))) (.yaw (Math|Conversions|RotationFromXVector (Math|Vector|GetUnitDirection(Vector) _returnvalue (+ _array_element _returnvalue))))) "0.100000,0.100000,0.100000") "AdjustIfPossibleButAlwaysSpawn" 0 "(R=0.567708,G=0.016375,B=0.518136,A=0.000000)" 0)
    (Effects|SpawnEmitterAttached "/Game/Léa/FX/Particle/P_Muzzle_laser_ennemy.P_Muzzle_laser_ennemy" 0 "None" (+ _array_element _returnvalue))
    (Development|PrintString (Utilities|String|ToString(Vector) (Math|Vector|GetUnitDirection(Vector) _returnvalue (+ _array_element _returnvalue))))))

(fn IsonScreen?
  (bind _returnvalue (Game|GetPlayerController 0))
  (bind _returnvalue_2 (Viewport|GetViewportSize))
  (bind _hull (Variables|Default|GetHull))
  (bind _returnvalue_3 (Transformation|GetWorldLocation _hull))
  (bind _screenlocation (Class|PlayerController|ProjectWorldLocationtoScreen _returnvalue _returnvalue_3 false))
  (return (Math|Boolean|ANDBoolean (> (.x _screenlocation) 0.0) (> (.y _screenlocation) 0.0) (< (.x _screenlocation) (.x _returnvalue_2)) (< (.y _screenlocation) (.y _returnvalue_2)))))

(fn SetUpBulletSpawners
  (bind _self self)
  (bind _cube (Variables|Default|GetCube _self))
  (bind _returnvalue (Transformation|GetWorldLocation _cube))
  (bind _returnvalue_2 (+ _returnvalue "100.000000, 0, 0"))
  (bind _returnvalue_3 (Math|Vector|GetUnitDirection(Vector) _returnvalue _returnvalue_2))
  (while (< (Variables|Default|GetBS_Incr) 355.0)
    (Utilities|Array|Add (Variables|Default|GetBulletSpawners) (Math|Vector|RotateVectorAroundAxis (Math|Vector|MakeVector (* (.x _returnvalue_3) 1e+02) (* (.y _returnvalue_3) 1e+02) (* (.z _returnvalue_3) 1e+02)) (Variables|Default|GetBS_Incr) (Math|Vector|GetUpVector _cube)))
    (Variables|Default|SetBS_Incr (+ (Variables|Default|GetBS_Incr) 5.0))))