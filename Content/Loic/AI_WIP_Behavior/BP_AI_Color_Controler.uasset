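; Work-in-progress AI color controller that paints colored enemies with player identity colors, apparently to force a change of gunner.
; ForcedGunnerChange gathers players at valid non-combat posts, then gives each of the enemy's paintable material slots a randomly picked player's IdentityCircle material.
; GiveUniqueColor is a stub that only fetches all colored enemies, and a debug print remains in ForcedGunnerChange.
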(event EventBeginPlay)

(event Collision|EventActorBeginOverlap
  (params (OtherActor :type Actor%20Object%20Reference)))

(event EventTick
  (params (DeltaSeconds :type Float%20%28single-precision%29)))

(fn ConstructionScript)

(fn GiveUniqueColor
  (params (Enemy :type Actor%20Object%20Reference))
  (Actor|GetAllActorsOfClass "/Game/Loic/AI_WIP_Behavior/BP_Colored_Enemy_Parent.BP_Colored_Enemy_Parent_C"))

(fn ForcedGunnerChange
  (params (Enemy :type AI%20Missile%20Object%20Reference))
  (bind _availableplayerarray (Variables|Default|GetAvailablePlayerArray))
  (Development|PrintString "fffffffFFFFF")
  (bind _outactors (Actor|GetAllActorsOfClass "/Game/Thibaud/Blueprints/Player/BP_Player.BP_Player_C"))
  (for _array_element _outactors
    (Utilities|IsValid (Variables|/Game/Thibaud/Blueprints/Player/BP_Player.BP_Player_C|GetCurrentPost _array_element)
      (:Is%20Valid
        (if (not (Variables|/Game/Thibaud/Blueprints/Player/Post/BPA_Post_Parent.BPA_Post_Parent_C|GetIsCombatPost? (Variables|/Game/Thibaud/Blueprints/Player/BP_Player.BP_Player_C|GetCurrentPost _array_element)))
          (Utilities|Array|Add (Variables|Default|GetAvailablePlayerArray) _array_element)))))
  (bind (_mesh _areas_to_color) (Default|GiveAreastoPaint Enemy))
  (for _array_element_2 _areas_to_color
    (Rendering|Material|SetMaterial _mesh _array_element_2 (Rendering|Material|GetMaterial (Variables|/Game/Thibaud/Blueprints/Player/BP_Player.BP_Player_C|GetIdentity%20Circle (Utilities|Array|Get(acopy) _availableplayerarray (Math|Random|RandomIntegerinRange 0 (- (Utilities|Array|Length _availableplayerarray) 1)))) 0))))