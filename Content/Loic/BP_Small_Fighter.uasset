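; Enemy small fighter that chases and shoots the player ship, driven by Tick.
; Two sphere traces set follow and attack ranges, triggering cube impulses, look-at rotation, AIMoveTo and rate-limited projectile spawning.
; Colliding with BP_Player deals damage and explodes the fighter, as does zero health; ship overlap staggers and destroys it.
; Side overlap flags are set but unread, and RearMove pushes along the same vector as FrontMove.
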(event OnComponentBeginOverlap(Frontal)
  (params (OverlappedComponent :type Primitive%20Component%20Object%20Reference) (OtherActor :type Actor%20Object%20Reference) (OtherComp :type Primitive%20Component%20Object%20Reference) (OtherBodyIndex :type Integer) (bFromSweep :type Boolean) (SweepResult :type Hit%20Result%20Structure%20%28by%20ref%29))
  ;[0 1 1] Collisions Bool
  (Variables|Default|SetFront true))

(event OnComponentEndOverlap(Frontal)
  (params (OverlappedComponent :type Primitive%20Component%20Object%20Reference) (OtherActor :type Actor%20Object%20Reference) (OtherComp :type Primitive%20Component%20Object%20Reference) (OtherBodyIndex :type Integer))
  ;[0 1 1] Collisions Bool
  (Variables|Default|SetFront false))

(event OnComponentBeginOverlap(Cube)
  (params (OverlappedComponent :type Primitive%20Component%20Object%20Reference) (OtherActor :type Actor%20Object%20Reference) (OtherComp :type Primitive%20Component%20Object%20Reference) (OtherBodyIndex :type Integer) (bFromSweep :type Boolean) (SweepResult :type Hit%20Result%20Structure%20%28by%20ref%29))
  ;[0 1 1] Ram Ennemi
  (Utilities|FlowControl|Sequence
    (:then_0
      (Utilities|Casting|CastToBp_Vaisseau OtherActor)
      (Utilities|FlowControl|DoOnce false :!label _label
        (:Completed
          (Variables|Default|SetStaggered true)
          (Utilities|FlowControl|Delay 1.0)
          (Variables|Default|SetStaggered false)
          (goto _label Reset))))
    (:then_1
      (if (Variables|Default|GetStaggered)
        (Actor|DestroyActor)))))

(event OnComponentBeginOverlap(Arrière)
  (params (OverlappedComponent :type Primitive%20Component%20Object%20Reference) (OtherActor :type Actor%20Object%20Reference) (OtherComp :type Primitive%20Component%20Object%20Reference) (OtherBodyIndex :type Integer) (bFromSweep :type Boolean) (SweepResult :type Hit%20Result%20Structure%20%28by%20ref%29))
  ;[0 1 1] Collisions Bool
  (Variables|Default|SetRear true))

(event OnComponentEndOverlap(Arrière)
  (params (OverlappedComponent :type Primitive%20Component%20Object%20Reference) (OtherActor :type Actor%20Object%20Reference) (OtherComp :type Primitive%20Component%20Object%20Reference) (OtherBodyIndex :type Integer))
  ;[0 1 1] Collisions Bool
  (Variables|Default|SetRear false))

(event OnComponentBeginOverlap(Droite)
  (params (OverlappedComponent :type Primitive%20Component%20Object%20Reference) (OtherActor :type Actor%20Object%20Reference) (OtherComp :type Primitive%20Component%20Object%20Reference) (OtherBodyIndex :type Integer) (bFromSweep :type Boolean) (SweepResult :type Hit%20Result%20Structure%20%28by%20ref%29))
  ;[0 1 1] Collisions Bool
  (Variables|Default|SetRight true))

(event OnComponentEndOverlap(Droite)
  (params (OverlappedComponent :type Primitive%20Component%20Object%20Reference) (OtherActor :type Actor%20Object%20Reference) (OtherComp :type Primitive%20Component%20Object%20Reference) (OtherBodyIndex :type Integer))
  ;[0 1 1] Collisions Bool
  (Variables|Default|SetRight false))

(event OnComponentBeginOverlap(Gauche)
  (params (OverlappedComponent :type Primitive%20Component%20Object%20Reference) (OtherActor :type Actor%20Object%20Reference) (OtherComp :type Primitive%20Component%20Object%20Reference) (OtherBodyIndex :type Integer) (bFromSweep :type Boolean) (SweepResult :type Hit%20Result%20Structure%20%28by%20ref%29))
  ;[0 1 1] Collisions Bool
  (Variables|Default|SetLeft true))

(event OnComponentEndOverlap(Gauche)
  (params (OverlappedComponent :type Primitive%20Component%20Object%20Reference) (OtherActor :type Actor%20Object%20Reference) (OtherComp :type Primitive%20Component%20Object%20Reference) (OtherBodyIndex :type Integer))
  ;[0 1 1] Collisions Bool
  (Variables|Default|SetLeft false))

(event Custom|Move%20Left
  (bind _cube (Variables|Default|GetCube))
  ;[0 1 1] Impulse forward / backward / Right / Left
  (Physics|AddImpulse _cube (* (Math|Vector|GetRightVector _cube) (Variables|Default|GetSpeed%20-%20%28y%29)) "None" true))

(event Custom|FrontMove
  (bind _cube (Variables|Default|GetCube))
  ;[0 1 1] Impulse forward / backward / Right / Left
  (Physics|AddImpulse _cube (* (Math|Vector|GetForwardVector _cube) (Variables|Default|GetSpeed%20+%20%28x%29)) "None" true))

(event Custom|RearMove
  (bind _cube (Variables|Default|GetCube))
  ;[0 1 1] Impulse forward / backward / Right / Left
  (Physics|AddImpulse _cube (* (Math|Vector|GetForwardVector _cube) (Variables|Default|GetSpeed%20-%20%28x%29)) "None" true))

(event Custom|Move%20Right
  (bind _cube (Variables|Default|GetCube))
  ;[0 1 1] Impulse forward / backward / Right / Left
  (Physics|AddImpulse _cube (* (Math|Vector|GetRightVector _cube) (Variables|Default|GetSpeed%20+%20%28y%29)) "None" true))

(event EventTick
  (params (DeltaSeconds :type Float%20%28single-precision%29))
  (bind _returnvalue (Transformation|GetActorLocation))
  (bind _returnvalue_2 (Transformation|GetActorLocation))
  (bind _returnvalue_3 (Game|Player|GetPlayerPawn 0))
  (bind _fire (Variables|Default|GetFire))
  (bind _returnvalue_4 (Transformation|GetWorldTransform _fire))
  ;[0 1 1] Box "if detect the player"
  (Utilities|FlowControl|Sequence
    (:then_0
      (bind _outhit (Collision|SphereTraceByChannel _returnvalue _returnvalue (Variables|Default|GetRange%20Follow%20Player) "TraceTypeQuery1" false 0 "ForOneFrame"))
      (if (Utilities|Enum|Equal(Enum) (Utilities|GetDisplayName (.HitActor (Collision|BreakHitResult _outhit))) "Bp_Vaisseau")
        (CallFunction|FrontMove)
        (Transformation|SetRelativeRotation (Variables|Default|GetCube) (Math|Rotator|FindLookatRotation (Transformation|GetActorLocation) (Transformation|GetActorLocation _returnvalue_3)) false false)
        (AI|AIMoveTo 0 "0, 0, 0" _returnvalue_3 5.0 false)
        (elif (.bBlockingHit (Collision|BreakHitResult _outhit))
          (CallFunction|FrontMove)
          (else
            (CallFunction|RearMove)))))
    (:then_1
      (bind _outhit_2 (Collision|SphereTraceByChannel _returnvalue_2 _returnvalue_2 (Variables|Default|GetRange%20Attack%20Player) "TraceTypeQuery1" false 0 "ForOneFrame"))
      (if (Utilities|Enum|Equal(Enum) (Utilities|GetDisplayName (.HitActor (Collision|BreakHitResult _outhit_2))) "Bp_Vaisseau")
        (CallFunction|MoveLeft)
        (CallFunction|RearMove)
        (Transformation|SetRelativeRotation (Variables|Default|GetCube) (Math|Rotator|FindLookatRotation (Transformation|GetActorLocation) (Transformation|GetActorLocation (Game|Player|GetPlayerPawn 0))) false false)
        ;[0 1 1] Tir
        (Utilities|FlowControl|DoOnce false :!label _label
          (:Completed
            (Game|SpawnActorfromClass "/Game/Blueprints/Projectiles/BP_ProjectileEnemyOne.BP_ProjectileEnemyOne_C" (Math|Transform|MakeTransform (.location _returnvalue_4) (.rotation _returnvalue_4) (Math|Vector|MakeVector 0.09 0.05 0.05)) "Undefined" 0 "(R=0.739583,G=0.049854,B=0.000000,A=0.000000)" 0)
            (Effects|SpawnEmitterAttached "/Game/Assets/Particles/Lea_particles/Muzzle_laser/P_Muzzle_laser.P_Muzzle_laser" (Variables|Default|GetFire) "None")
            (Utilities|FlowControl|Delay (Variables|Default|GetRateofFire))
            (goto _label Reset)))))))

(event Game|Damage|EventAnyDamage
  (params (Damage :type Float%20%28single-precision%29) (DamageType :type Damage%20Type%20Object%20Reference) (InstigatedBy :type Controller%20Object%20Reference) (DamageCauser :type Actor%20Object%20Reference))
  ;[0 1 1] Apply Damage BTW Player & AI
  (Variables|Default|SetHealth (Math|Float|Clamp(Float) (- (Variables|Default|GetHealth) Damage) 0.0 (Variables|Default|GetMaxHealth)))
  (if (<= (Variables|Default|GetHealth) 0.0)
    (CallFunction|IsHealth<=0ParticleatLocation)))

(event Collision|EventHit
  (params (MyComp :type Primitive%20Component%20Object%20Reference) (Other :type Actor%20Object%20Reference) (OtherComp :type Primitive%20Component%20Object%20Reference) (bSelfMoved :type Boolean) (HitLocation :type Vector :default "0, 0, 0") (HitNormal :type Vector :default "0, 0, 0") (NormalImpulse :type Vector :default "0, 0, 0") (Hit :type Hit%20Result%20Structure%20%28by%20ref%29))
  ;[0 1 1] Apply Damage BTW Player & AI
  (Utilities|Casting|CastToBP_ProjectilePlayerBase Other
    (:CastFailed
      (bind _asbp_player (Utilities|Casting|CastToBP_Player Other))
      (Game|Damage|ApplyDamage _asbp_player 5e+01 0 0)
      (CallFunction|IsHealth<=0ParticleatLocation))))

(fn ConstructionScript)

(fn IsHealth<=0ParticleatLocation
  (Effects|SpawnEmitteratLocation "/Game/Assets/Particles/Lea_particles/Explosion_colored_blue/P_Explosion_3D_blue.P_Explosion_3D_blue" (Transformation|GetWorldLocation (Variables|Default|GetCube)))
  (Actor|DestroyActor))