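; Timed lock button, likely for synchronized activation, that triggers when damage drains its health to zero.
; On trigger it flags itself active, messages a linked actor and slides to its ON position, returning OFF after SynchroDelay and re-arming without restoring health.
; A separate overlap handler holds a one-shot that destroys the button and sends the same message, though its Bp_Vaisseau cast branches are empty.
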(event OnComponentBeginOverlap(Button)
  (params (OverlappedComponent :type Primitive%20Component%20Object%20Reference) (OtherActor :type Actor%20Object%20Reference) (OtherComp :type Primitive%20Component%20Object%20Reference) (OtherBodyIndex :type Integer) (bFromSweep :type Boolean) (SweepResult :type Hit%20Result%20Structure%20%28by%20ref%29))
  (Utilities|Casting|CastToBp_Vaisseau OtherActor
    (:then
      _)
    (:CastFailed
      _))
  (Utilities|FlowControl|DoOnce false
    (:Completed
      (Components|DestroyComponent (Variables|Default|GetButton))
      (Class|BPIConnection|Connection?(Message) (Variables|Default|GetActor?)))))

(event EventBeginPlay
  (bind _button (Variables|Default|GetButton))
  (Rendering|Material|CreateDynamicMaterialInstance _button 0 (Rendering|Material|GetMaterial _button 0) "None" :!class /Script/Engine.PrimitiveComponent)
  (Rendering|Material|SetMaterial (Variables|Default|GetButton) 0 (Variables|Default|GetMaterial)))

(event Game|Damage|EventAnyDamage
  (params (Damage :type Float%20%28single-precision%29) (DamageType :type Damage%20Type%20Object%20Reference) (InstigatedBy :type Controller%20Object%20Reference) (DamageCauser :type Actor%20Object%20Reference))
  (bind _button (Variables|Default|GetButton))
  (bind _button_2 (Variables|Default|GetButton))
  (Variables|Default|SetHealth (Math|Float|Clamp(Float) (- (Variables|Default|GetHealth) Damage) 0.0 (Variables|Default|GetMaxHealth)))
  (if (<= (Variables|Default|GetHealth) 0.0)
    (Utilities|FlowControl|DoOnce false :!label _label
      (:Completed
        (Variables|Default|Setbutton_isActivated true)
        (Class|BPIConnection|Connection?(Message) (Variables|Default|GetActor?))
        (Components|MoveComponentTo _button_2 (Variables|/Script/Engine.SceneComponent|GetRelativeLocation (Variables|Default|GetSceneON)) (Variables|/Script/Engine.SceneComponent|GetRelativeRotation _button_2) false false 1.0 false)
        (Utilities|FlowControl|Delay (Variables|Default|GetSynchroDelay))
        (Variables|Default|Setbutton_isActivated false)
        (Components|MoveComponentTo _button (Variables|/Script/Engine.SceneComponent|GetRelativeLocation (Variables|Default|GetSceneOFF)) (Variables|/Script/Engine.SceneComponent|GetRelativeRotation _button) false false 1.0 false)
        (goto _label Reset)))))

(fn ConstructionScript)