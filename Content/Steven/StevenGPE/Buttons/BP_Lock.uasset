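; BP_Lock is a damageable button lock that notifies a linked actor when triggered.
; Damage lowers clamped health; at zero it flags the button as activated, sends ConnectionMessage to the linked Actor and slides the button to the SceneON position, once.
; A separate one-shot overlap path destroys the button and sends the same message, with a Bp_Starship cast that has empty branches.
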(event OnComponentBeginOverlap(Button)
  (params (OverlappedComponent :type Primitive%20Component%20Object%20Reference) (OtherActor :type Actor%20Object%20Reference) (OtherComp :type Primitive%20Component%20Object%20Reference) (OtherBodyIndex :type Integer) (bFromSweep :type Boolean) (SweepResult :type Hit%20Result%20Structure%20%28by%20ref%29))
  (Utilities|Casting|CastToBp_Starship OtherActor
    (:then
      _)
    (:CastFailed
      _))
  (Utilities|FlowControl|DoOnce false
    (:Completed
      (Components|DestroyComponent (Variables|Default|GetButton))
      (Class|BPIConnection|Connection?(Message) (Variables|Default|GetActor?)))))

(event Game|Damage|EventAnyDamage
  (params (Damage :type Float%20%28single-precision%29) (DamageType :type Damage%20Type%20Object%20Reference) (InstigatedBy :type Controller%20Object%20Reference) (DamageCauser :type Actor%20Object%20Reference))
  (bind _button (Variables|Default|GetButton))
  (Variables|Default|SetHealth (Math|Float|Clamp(Float) (- (Variables|Default|GetHealth) Damage) 0.0 (Variables|Default|GetMaxHealth)))
  (if (<= (Variables|Default|GetHealth) 0.0)
    (Utilities|FlowControl|DoOnce false
      (:Completed
        (Variables|Default|Setbutton_isActivated true)
        (Class|BPIConnection|Connection?(Message) (Variables|Default|GetActor?))
        (Components|MoveComponentTo _button (Variables|/Script/Engine.SceneComponent|GetRelativeLocation (Variables|Default|GetSceneON)) (Variables|/Script/Engine.SceneComponent|GetRelativeRotation _button) false false 1.0 false)))))

(fn ConstructionScript)