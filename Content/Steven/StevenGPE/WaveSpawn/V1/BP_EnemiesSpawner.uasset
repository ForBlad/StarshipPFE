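; Wave manager that spawns fighters, cruisers and missile launchers once the player overlaps its trigger, then opens the boss doors after three waves.
; Looping one-second timers spawn each type from cast-sorted spawn points, random for fighters and cruisers, always the first for missile launchers.
; Tick prunes destroyed enemies from WaveActors.
; When a type's count runs out and WaveActors is empty, the next wave loads per-wave counts with a sound cue.
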(event OnComponentBeginOverlap(WaveSpawnTrigger)
  (params (OverlappedComponent :type Primitive%20Component%20Object%20Reference) (OtherActor :type Actor%20Object%20Reference) (OtherComp :type Primitive%20Component%20Object%20Reference) (OtherBodyIndex :type Integer) (bFromSweep :type Boolean) (SweepResult :type Hit%20Result%20Structure%20%28by%20ref%29))
  (Utilities|Casting|CastToBP_Player OtherActor)
  (CallFunction|SpawningFighters)
  (CallFunction|SpawiningCruisers)
  (CallFunction|SpawningMissileLaunchers))

(event Custom|ActivateFighterSpawner
  (bind _fighternumber (Variables|Default|GetFighterNumber))
  (bind _fighterspawnlist (Variables|Default|GetFighterSpawnList))
  (bind _wavenumber (Variables|Default|GetWaveNumber))
  ;[1 1 1] SpawnFighter
  (if (> _fighternumber 0)
    (bind _actor (Default|SpawnFighters (Utilities|Array|Get(acopy) _fighterspawnlist (Math|Random|RandomIntegerinRange 0 (- (Utilities|Array|Length _fighterspawnlist) 1)))))
    (Utilities|Array|Add (Variables|Default|GetWaveActors) _actor)
    (Math|Integer|DecrementInt _fighternumber)
    (else
      ;[1 1 1] WaveManagement
      (Utilities|FlowControl|Delay 0.1)
      (if (and (== (Utilities|Array|Length (Variables|Default|GetWaveActors)) 0) (< (Variables|Default|GetWaveNumber) 4))
        (Utilities|FlowControl|Delay 1.0)
        (Math|Integer|IncrementInt _wavenumber
          (:%20%20
            (Audio|SpawnSound2D "/Game/Assets/Audio/SOUNDBANK/SFX/SFX_SHIP/MISSILE_CRUISER/SFX_SHIP_MISSILE_CRUISER_Triggered_02.SFX_SHIP_MISSILE_CRUISER_Triggered_02" 1.0 1.0 0.0 0)
            (CallFunction|CalculateEnemiesNumber)
            (if (== _wavenumber 4)
              ;[1 1 1] BossDoorOpening
              (if (and (== (Variables|Default|GetWaveNumber) 4) (== (Variables|Default|GetTotalNumberOfEnemies) 0))
                (for _array_element (Variables|Default|GetDoorToOpen)
                  (Default|OpenDoor _array_element))))))))))

(event Custom|ActivateMissileLauncherSpawners
  (bind _missilelaunchernumber (Variables|Default|GetMissileLauncherNumber))
  (bind _wavenumber (Variables|Default|GetWaveNumber))
  ;[1 1 1] SpawnMissileLauncher
  (if (> _missilelaunchernumber 0)
    (bind _actor (Default|SpawnMissileLaunchers (Utilities|Array|Get(acopy) (Variables|Default|GetMissileLauncherSpawnList))))
    (Utilities|Array|Add (Variables|Default|GetWaveActors) _actor)
    (Math|Integer|DecrementInt _missilelaunchernumber)
    (else
      ;[1 1 1] WaveManagement
      (Utilities|FlowControl|Delay 0.1)
      (if (and (== (Utilities|Array|Length (Variables|Default|GetWaveActors)) 0) (< (Variables|Default|GetWaveNumber) 4))
        (Utilities|FlowControl|Delay 1.0)
        (Math|Integer|IncrementInt _wavenumber
          (:%20%20
            (Audio|SpawnSound2D "/Game/Assets/Audio/SOUNDBANK/SFX/SFX_SHIP/MISSILE_CRUISER/SFX_SHIP_MISSILE_CRUISER_Triggered_02.SFX_SHIP_MISSILE_CRUISER_Triggered_02" 1.0 1.0 0.0 0)
            (CallFunction|CalculateEnemiesNumber)
            (if (== _wavenumber 4)
              ;[1 1 1] BossDoorOpening
              (if (and (== (Variables|Default|GetWaveNumber) 4) (== (Variables|Default|GetTotalNumberOfEnemies) 0))
                (for _array_element (Variables|Default|GetDoorToOpen)
                  (Default|OpenDoor _array_element))))))))))

(event Custom|SpawningMissileLaunchers
  ;[1 1 1] SpawnMissileLauncher
  (for _array_element (Variables|Default|GetSpawners)
    (bind _asbp_missile_launcher_spawn_point (Utilities|Casting|CastToBP_MissileLauncherSpawnPoint _array_element))
    (Utilities|Array|Add (Variables|Default|GetMissileLauncherSpawnList) _asbp_missile_launcher_spawn_point))
  (Utilities|Time|SetTimerbyEvent (delegate Custom|ActivateMissileLauncherSpawners) 1.0 true))

(event Custom|SpawningFighters
  ;[1 1 1] SpawnFighter
  (for _array_element (Variables|Default|GetSpawners)
    (bind _asbp_fighter_spawn_point (Utilities|Casting|CastToBP_FighterSpawnPoint _array_element))
    (Utilities|Array|Add (Variables|Default|GetFighterSpawnList) _asbp_fighter_spawn_point))
  (Utilities|Time|SetTimerbyEvent (delegate Custom|ActivateFighterSpawner) 1.0 true))

(event Custom|ActivateCruiserSpawners
  (bind _cruisernumber (Variables|Default|GetCruiserNumber))
  (bind _cruiserspawnlist (Variables|Default|GetCruiserSpawnList))
  (bind _wavenumber (Variables|Default|GetWaveNumber))
  ;[1 1 1] SpawnCruiser
  (if (> _cruisernumber 0)
    (bind _actor (Default|SpawnCruisers (Utilities|Array|Get(acopy) _cruiserspawnlist (Math|Random|RandomIntegerinRange 0 (- (Utilities|Array|Length _cruiserspawnlist) 1)))))
    (Utilities|Array|Add (Variables|Default|GetWaveActors) _actor)
    (Math|Integer|DecrementInt _cruisernumber)
    (else
      ;[1 1 1] WaveManagement
      (Utilities|FlowControl|Delay 0.1)
      (if (and (== (Utilities|Array|Length (Variables|Default|GetWaveActors)) 0) (< (Variables|Default|GetWaveNumber) 4))
        (Utilities|FlowControl|Delay 1.0)
        (Math|Integer|IncrementInt _wavenumber
          (:%20%20
            (Audio|SpawnSound2D "/Game/Assets/Audio/SOUNDBANK/SFX/SFX_SHIP/MISSILE_CRUISER/SFX_SHIP_MISSILE_CRUISER_Triggered_02.SFX_SHIP_MISSILE_CRUISER_Triggered_02" 1.0 1.0 0.0 0)
            (CallFunction|CalculateEnemiesNumber)
            (if (== _wavenumber 4)
              ;[1 1 1] BossDoorOpening
              (if (and (== (Variables|Default|GetWaveNumber) 4) (== (Variables|Default|GetTotalNumberOfEnemies) 0))
                (for _array_element (Variables|Default|GetDoorToOpen)
                  (Default|OpenDoor _array_element))))))))))

(event Custom|SpawiningCruisers
  ;[1 1 1] SpawnCruiser
  (for _array_element (Variables|Default|GetSpawners)
    (bind _asbp_cruiser_spawn_point (Utilities|Casting|CastToBP_CruiserSpawnPoint _array_element))
    (Utilities|Array|Add (Variables|Default|GetCruiserSpawnList) _asbp_cruiser_spawn_point))
  (Utilities|Time|SetTimerbyEvent (delegate Custom|ActivateCruiserSpawners) 1.0 true))

(event EventTick
  (params (DeltaSeconds :type Float%20%28single-precision%29))
  (bind _waveactors (Variables|Default|GetWaveActors))
  (Utilities|FlowControl|Sequence
    (:then_0
      (Variables|Default|SetTotalNumberOfEnemies (+ (Variables|Default|GetFighterNumber) (Variables|Default|GetCruiserNumber) (Variables|Default|GetMissileLauncherNumber)))
      (for _array_element _waveactors
        (Utilities|IsValid _array_element
          (:Is%20Not%20Valid
            (Utilities|Array|RemoveItem _waveactors _array_element)))))))

(fn ConstructionScript)

(fn CalculateEnemiesNumber
  (bind _wavefightersnber (Variables|Default|GetWaveFightersNber))
  (bind _wavecruisersnber (Variables|Default|GetWaveCruisersNber))
  (bind _wavemissilelaunchersnber (Variables|Default|GetWaveMissileLaunchersNber))
  (switch int (Variables|Default|GetWaveNumber)
    (:1
      (Variables|Default|SetFighterNumber (Utilities|Array|Get(acopy) _wavefightersnber))
      (Variables|Default|SetCruiserNumber (Utilities|Array|Get(acopy) _wavecruisersnber))
      (Variables|Default|SetMissileLauncherNumber (Utilities|Array|Get(acopy) _wavemissilelaunchersnber)))
    (:2
      (Variables|Default|SetFighterNumber (Utilities|Array|Get(acopy) _wavefightersnber 1))
      (Variables|Default|SetCruiserNumber (Utilities|Array|Get(acopy) _wavecruisersnber 1))
      (Variables|Default|SetMissileLauncherNumber (Utilities|Array|Get(acopy) _wavemissilelaunchersnber 1)))
    (:3
      (Variables|Default|SetFighterNumber (Utilities|Array|Get(acopy) _wavefightersnber 2))
      (Variables|Default|SetCruiserNumber (Utilities|Array|Get(acopy) _wavecruisersnber 2))
      (Variables|Default|SetMissileLauncherNumber (Utilities|Array|Get(acopy) _wavemissilelaunchersnber 2)))))