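; BP_CruiserSpawnPoint is a spawn point that creates an AI_Cruser1 cruiser on request, provided no starship is in the way.
; Box overlap events set a ShipAroundC flag when a Bp_Starship enters and clear it when one leaves.
; SpawnCruisers reports failure while the flag is set; otherwise it passes a DoOnce, spawns a half-scale cruiser at its own transform and returns it with a success flag.
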(event OnComponentBeginOverlap(Box)
  (params (OverlappedComponent :type Primitive%20Component%20Object%20Reference) (OtherActor :type Actor%20Object%20Reference) (OtherComp :type Primitive%20Component%20Object%20Reference) (OtherBodyIndex :type Integer) (bFromSweep :type Boolean) (SweepResult :type Hit%20Result%20Structure%20%28by%20ref%29))
  (Utilities|Casting|CastToBp_Starship OtherActor)
  (Variables|Default|SetShip_Around_C true))

(event OnComponentEndOverlap(Box)
  (params (OverlappedComponent :type Primitive%20Component%20Object%20Reference) (OtherActor :type Actor%20Object%20Reference) (OtherComp :type Primitive%20Component%20Object%20Reference) (OtherBodyIndex :type Integer))
  (Utilities|Casting|CastToBp_Starship OtherActor)
  (Variables|Default|SetShip_Around_C false))

(fn ConstructionScript)

(fn SpawnCruisers
  (bind _returnvalue (Transformation|GetActorTransform))
  (if (Variables|Default|GetShip_Around_C)
    (return 0 false)
    (else
      (Utilities|FlowControl|DoOnce false
        (:Completed
          (bind _returnvalue_2 (Game|SpawnActorfromClass "/Game/Loic/AI_WIP_Behavior/AI_Cruser1.AI_Cruser1_C" (Math|Transform|MakeTransform (.location _returnvalue) (.rotation _returnvalue) "0.500000,0.500000,0.500000") "Undefined" 0 0))
          (return _returnvalue_2 true))))))