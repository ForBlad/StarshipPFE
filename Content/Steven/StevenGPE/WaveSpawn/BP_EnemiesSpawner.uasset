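; Enemy wave spawner that starts when the Bp_Vaisseau ship overlaps its trigger.
; Three looping timers spawn fighters and cruisers at random spawn points, and missile launchers at the first listed one, until each count empties.
; Emptied timers share a check that, once no enemies remain, advances the wave and recalculates counts.
; Wave 4 zeroes all counts and calls ConnectionMessage for the boss door opening.
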(event OnComponentBeginOverlap(WaveSpawnTrigger)
  (params (OverlappedComponent :type Primitive%20Component%20Object%20Reference) (OtherActor :type Actor%20Object%20Reference) (OtherComp :type Primitive%20Component%20Object%20Reference) (OtherBodyIndex :type Integer) (bFromSweep :type Boolean) (SweepResult :type Hit%20Result%20Structure%20%28by%20ref%29))
  (Utilities|Casting|CastToBp_Vaisseau OtherActor)
  (Utilities|FlowControl|Sequence
    (:then_0
      (CallFunction|SpawningFighters))
    (:then_1
      (CallFunction|SpawiningCruisers))
    (:then_2
      (CallFunction|SpawningMissileLaunchers))))

(event Custom|ActivateFighterSpawner
  (bind _fighterspawnlist (Variables|Default|GetFighterSpawnList))
  ;[1 1 1] SpawnFighter
  (if (> (Variables|Default|GetFighterNumber) 0)
    (Default|SpawnFighters (Utilities|Array|Get(acopy) _fighterspawnlist (Math|Random|RandomIntegerinRange 0 (- (Utilities|Array|Length _fighterspawnlist) 1))))
    (Math|Integer|DecrementInt (Variables|Default|GetFighterNumber))
    (else
      ;[1 1 1] WaveManagement
      (bind _outactors (Actor|GetAllActorsOfClass "/Game/Loic/AI_WIP_Behavior/AI_Fighter1.AI_Fighter1_C"))
      (if (Math|Boolean|ANDBoolean (<= (Utilities|Array|Length _outactors) 0) (<= (Utilities|Array|Length (stale Custom|ActivateCruiserSpawners _outactors)) 0) (<= (Utilities|Array|Length (stale Custom|ActivateMissileLauncherSpawners _outactors)) 0) (< (Variables|Default|GetWaveNumber) 4))
        (Utilities|FlowControl|Delay 2.0)
        (Math|Integer|IncrementInt (Variables|Default|GetWaveNumber)
          (:%20%20
            (CallFunction|CalculateEnemiesNumber)
            ;[1 1 1] BossDoorOpening
            (if (== (Variables|Default|GetWaveNumber) 4)
              (Class|BPIConnection|Connection?(Message) (Variables|Default|GetActor)))))))))

(event Custom|ActivateMissileLauncherSpawners
  ;[1 1 1] SpawnMissileLauncher
  (if (> (Variables|Default|GetMissileLauncherNumber) 0)
    (Default|SpawnMissileLaunchers (Utilities|Array|Get(acopy) (Variables|Default|GetMissileLauncherSpawnList)))
    (Math|Integer|DecrementInt (Variables|Default|GetMissileLauncherNumber))
    (else
      ;[1 1 1] WaveManagement
      (bind _outactors (Actor|GetAllActorsOfClass "/Game/Loic/AI_WIP_Behavior/AI_Missile.AI_missile_C"))
      (if (Math|Boolean|ANDBoolean (<= (Utilities|Array|Length (stale Custom|ActivateFighterSpawner _outactors)) 0) (<= (Utilities|Array|Length (stale Custom|ActivateCruiserSpawners _outactors)) 0) (<= (Utilities|Array|Length _outactors) 0) (< (Variables|Default|GetWaveNumber) 4))
        (Utilities|FlowControl|Delay 2.0)
        (Math|Integer|IncrementInt (Variables|Default|GetWaveNumber)
          (:%20%20
            (CallFunction|CalculateEnemiesNumber)
            ;[1 1 1] BossDoorOpening
            (if (== (Variables|Default|GetWaveNumber) 4)
              (Class|BPIConnection|Connection?(Message) (Variables|Default|GetActor)))))))))

(event Custom|SpawningMissileLaunchers
  ;[1 1 1] SpawnMissileLauncher
  (bind _outactors (Actor|GetAllActorsOfClass "/Game/Steven/StevenGPE/WaveSpawn/SpawnPoints/BP_MissileLauncherSpawnPoint.BP_MissileLauncherSpawnPoint_C"))
  (Variables|Default|SetMissileLauncherSpawnList _outactors)
  (Utilities|Time|SetTimerbyEvent (delegate Custom|ActivateMissileLauncherSpawners) 1.0 true))

(event Custom|SpawningFighters
  ;[1 1 1] SpawnFighter
  (bind _outactors (Actor|GetAllActorsOfClass "/Game/Steven/StevenGPE/WaveSpawn/SpawnPoints/BP_FighterSpawnPoint.BP_FighterSpawnPoint_C"))
  (Variables|Default|SetFighterSpawnList _outactors)
  (Utilities|Time|SetTimerbyEvent (delegate Custom|ActivateFighterSpawner) 1.0 true))

(event Custom|ActivateCruiserSpawners
  (bind _cruiserspawnlist (Variables|Default|GetCruiserSpawnList))
  ;[1 1 1] SpawnCruiser
  (if (> (Variables|Default|GetCruiserNumber) 0)
    (Default|SpawnCruisers (Utilities|Array|Get(acopy) _cruiserspawnlist (Math|Random|RandomIntegerinRange 0 (- (Utilities|Array|Length _cruiserspawnlist) 1))))
    (Math|Integer|DecrementInt (Variables|Default|GetCruiserNumber))
    (else
      ;[1 1 1] WaveManagement
      (bind _outactors (Actor|GetAllActorsOfClass "/Game/Loic/AI_WIP_Behavior/AI_Cruser1.AI_Cruser1_C"))
      (if (Math|Boolean|ANDBoolean (<= (Utilities|Array|Length (stale Custom|ActivateFighterSpawner _outactors)) 0) (<= (Utilities|Array|Length _outactors) 0) (<= (Utilities|Array|Length (stale Custom|ActivateMissileLauncherSpawners _outactors)) 0) (< (Variables|Default|GetWaveNumber) 4))
        (Utilities|FlowControl|Delay 2.0)
        (Math|Integer|IncrementInt (Variables|Default|GetWaveNumber)
          (:%20%20
            (CallFunction|CalculateEnemiesNumber)
            ;[1 1 1] BossDoorOpening
            (if (== (Variables|Default|GetWaveNumber) 4)
              (Class|BPIConnection|Connection?(Message) (Variables|Default|GetActor)))))))))

(event Custom|SpawiningCruisers
  ;[1 1 1] SpawnCruiser
  (bind _outactors (Actor|GetAllActorsOfClass "/Game/Steven/StevenGPE/WaveSpawn/SpawnPoints/BP_CruiserSpawnPoint.BP_CruiserSpawnPoint_C"))
  (Variables|Default|SetCruiserSpawnList _outactors)
  (Utilities|Time|SetTimerbyEvent (delegate Custom|ActivateCruiserSpawners) 1.0 true))

(fn ConstructionScript)

(fn CalculateEnemiesNumber
  (Utilities|FlowControl|Sequence
    (:then_0
      (Variables|Default|SetFighterNumber (- (* (Variables|Default|GetWaveNumber) 7) (* (Variables|Default|GetWaveNumber) 4))))
    (:then_1
      (Variables|Default|SetCruiserNumber (Variables|Default|GetWaveNumber)))
    (:then_2
      (Variables|Default|SetMissileLauncherNumber 1))
    (:then_3
      (if (== (Variables|Default|GetWaveNumber) 4)
        (Variables|Default|SetFighterNumber 0)
        (Variables|Default|SetCruiserNumber 0)
        (Variables|Default|SetMissileLauncherNumber 0)))))