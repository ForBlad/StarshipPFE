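; BP_WaveManager runs enemy waves: a countdown, then a spawn driven by a data table row matching the wave number.
; On BeginPlay it sorts spawn points into Fighter, Cruiser and Missile Launcher lists.
; Each row entry spawns its enemy count at random points of the matching type, tracking the actors.
; A delay loop polls until all are invalid; no next-wave step follows.
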(event Custom|CE_StartCountDown
  ;[1 1 1] Countdown
  (bind _returnvalue (Utilities|Time|SetTimerbyEvent (delegate Custom|Count) 1.0 true))
  (Variables|Default|SetTime 5))

(event Custom|Count
  ;[1 1 1] Countdown
  (Development|PrintString (Utilities|String|ToString(Integer) (Variables|Default|GetTime)))
  (Math|Integer|DecrementInt (Variables|Default|GetTime)
    (:%20%20
      (if (== (Variables|Default|GetTime) 0)
        (Utilities|Time|ClearandInvalidateTimerbyHandle (stale Custom|CE_StartCountDown _returnvalue))
        (Utilities|FlowControl|Delay 1.0)
        (CallFunction|BeginWave)))))

(event Custom|BeginWave
  ;[1 1 1] SpawnEnemiesForWaves
  (bind _returnvalue (Utilities|GetDataTableRow (Variables|Default|GetEnemyDataTable) (Utilities|String|StringToName (Utilities|String|ToString(Integer) (Variables|Default|GetWaveNumber))))
    (:then
      (for _array_element (Utilities|Struct|BreakS_WaveInfo _returnvalue)
        (CallFunction|SpawnEnemies _array_element))
      (CallFunction|StartCheackingifEnemiesAreDead))
    (:RowNotFound
      (Development|PrintString "NoRow"))))

(event Custom|StartCheackingIfEnemiesAreDead
  (bind _aredead__1 (CallFunction|CheckifAllEnemiesAreDead :!label _label))
  (if (not _aredead__1)
    (Utilities|FlowControl|Delay 0.2)
    (goto _label)))

(event EventBeginPlay
  ;[1 1 1] EnemiesSpawnerReferences
  (bind _outactors (Actor|GetAllActorsOfClass "/Game/Steven/StevenGPE/WaveSpawn/V2/BP_WaveSpawnPoint.BP_WaveSpawnPoint_C"))
  (bind _output_get (Variables|Default|SetEnemies_SpawnPoints _outactors))
  (for _array_element _output_get
    (switch Utilities|FlowControl|Switch|SwitchonE_EnemyTypes (Variables|/Game/Steven/StevenGPE/WaveSpawn/V2/BP_WaveSpawnPoint.BP_WaveSpawnPoint_C|GetSpawnerType _array_element)
      (:NewEnumerator0
        (Utilities|Array|Add (Variables|Default|GetE_Fighter) _array_element))
      (:NewEnumerator1
        (Utilities|Array|Add (Variables|Default|GetE_Cruiser) _array_element))
      (:NewEnumerator2
        (Utilities|Array|Add (Variables|Default|GetE_MissileLauncher) _array_element))))
  (CallFunction|CEStartCountDown))

(fn ConstructionScript)

(fn CheckifAllEnemiesAreDead
  (LocalVariables|SetAreDead%20? true)
  (for _array_element (Variables|Default|GetCurrentEnemies)
    (Utilities|IsValid _array_element
      (:Is%20Valid
        (LocalVariables|SetAreDead%20? false))))
  (return (LocalVariables|GetAreDead%20?)))

(fn SpawnEnemies
  (params (S_EnemyInfo :type S%20Enemy%20Info%20Structure%20%28by%20ref%29))
  (LocalVariables|SetEnemyInfoRef S_EnemyInfo)
  (LocalVariables|SetCurrentSpawnPoints (Utilities|Select :Index (.EnemyType (Utilities|Struct|BreakS_EnemyInfo S_EnemyInfo)) :NewEnumerator0 (Variables|Default|GetE_Fighter) :NewEnumerator1 (Variables|Default|GetE_Cruiser) :NewEnumerator2 (Variables|Default|GetE_MissileLauncher)))
  (for _index (range 1 (.enemiesnumber (LocalVariables|GetEnemyInfoRef)))
    (bind _returnvalue (Game|SpawnActorfromClass (.enemyclass (LocalVariables|GetEnemyInfoRef)) (Transformation|GetWorldTransform (Variables|/Game/Steven/StevenGPE/WaveSpawn/V2/BP_WaveSpawnPoint.BP_WaveSpawnPoint_C|GetWaveSpawnScene (Utilities|Array|Get(acopy) (LocalVariables|GetCurrentSpawnPoints) (Math|Random|RandomIntegerinRange 0 (Utilities|Array|LastIndex (LocalVariables|GetCurrentSpawnPoints)))))) "AdjustIfPossibleButAlwaysSpawn" 0 0))
    (Utilities|Array|Add (Variables|Default|GetCurrentEnemies) _returnvalue)))