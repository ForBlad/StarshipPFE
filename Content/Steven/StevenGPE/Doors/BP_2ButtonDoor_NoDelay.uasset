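; A force field door that opens when both linked no-delay button locks are activated.
; The Connection? event checks the first two locks, then a timeline scales the force field along X and disables door collision when finished.
; If CloseTheDoor is set, a starship overlapping the close trigger runs a second scale timeline that restores collision.
; An AreAllButtonsActivated helper checks every lock but is not called here.
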(event OnComponentBeginOverlap(SynchDoorCloseTrigger)
  (params (OverlappedComponent :type Primitive%20Component%20Object%20Reference) (OtherActor :type Actor%20Object%20Reference) (OtherComp :type Primitive%20Component%20Object%20Reference) (OtherBodyIndex :type Integer) (bFromSweep :type Boolean) (SweepResult :type Hit%20Result%20Structure%20%28by%20ref%29))
  (if (Variables|Default|GetCloseTheDoor)
    (Utilities|Casting|CastToBp_Starship OtherActor)
    (bind _float (Timeline|Timeline_0 PlayFromStart)
      (:Update
        (Transformation|SetRelativeScale3D (Variables|Default|GetGPE_Door_Base_ForceField) (Math|Vector|MakeVector _float 9.25 8.25)))
      (:Finished
        (Collision|SetCollisionEnabled (Variables|Default|GetDoor_Collision) "QueryAndPhysics")))))

(event EventConnection?
  (bind _bp_nodelaylock (Variables|Default|GetBP_NoDelayLock))
  (if (and (Variables|/Game/Steven/StevenGPE/Buttons/BP_NodelayLock.BP_NodelayLock_C|Getbutton_isActivated (Utilities|Array|Get(acopy) _bp_nodelaylock)) (Variables|/Game/Steven/StevenGPE/Buttons/BP_NodelayLock.BP_NodelayLock_C|Getbutton_isActivated (Utilities|Array|Get(acopy) _bp_nodelaylock 1)))
    (bind _float (Timeline|Timeline PlayFromStart)
      (:Update
        (Transformation|SetRelativeScale3D (Variables|Default|GetGPE_Door_Base_ForceField) (Math|Vector|MakeVector _float 9.25 8.25)))
      (:Finished
        (Collision|SetCollisionEnabled (Variables|Default|GetDoor_Collision) "NoCollision")))))

(fn ConstructionScript)

(fn AreAllButtonsActivated?
  (for _array_element (Variables|Default|GetBP_NoDelayLock)
    (if (not (Variables|/Game/Steven/StevenGPE/Buttons/BP_NodelayLock.BP_NodelayLock_C|Getbutton_isActivated _array_element))
      (return false)))
  (return true))