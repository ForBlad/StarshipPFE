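; Boss door actor that opens or moves along a path and closes behind the player's starship.
; The Connection? event plays a timeline that drives the door's location and rotation along a spline.
; When a Bp_Starship overlaps CloseTrigger, a second timeline repeatedly calls MoveComponentTo toward the BossDoorReturnScene location, using the timeline value as the move duration.
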(event OnComponentBeginOverlap(CloseTrigger)
  (params (OverlappedComponent :type Primitive%20Component%20Object%20Reference) (OtherActor :type Actor%20Object%20Reference) (OtherComp :type Primitive%20Component%20Object%20Reference) (OtherBodyIndex :type Integer) (bFromSweep :type Boolean) (SweepResult :type Hit%20Result%20Structure%20%28by%20ref%29))
  (Utilities|Casting|CastToBp_Starship OtherActor)
  (bind _movement (Timeline|CloseMovement Play)
    (:Update
      (Components|MoveComponentTo (Variables|Default|GetDoor) (Variables|/Script/Engine.SceneComponent|GetRelativeLocation (Variables|Default|GetBossDoorReturnScene)) "0, 0, 0" false false _movement false))))

(event Collision|EventActorBeginOverlap
  (params (OtherActor :type Actor%20Object%20Reference)))

(event EventConnection?
  (bind _spline (Variables|Default|GetSpline))
  (bind _door (Variables|Default|GetDoor))
  (bind _movement (Timeline|T_Movement Play)
    (:Update
      (Transformation|SetWorldTransform _door (Math|Transform|MakeTransform (Spline|GetLocationatDistanceAlongSpline _spline (* (Spline|GetSplineLength _spline) _movement) "World") (Spline|GetRotationatDistanceAlongSpline _spline (* (Spline|GetSplineLength _spline) _movement) "World") (Variables|/Script/Engine.SceneComponent|GetRelativeScale3D _door)) false false))))

(fn ConstructionScript)