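; Door actor that moves along a spline when its Connection? event fires, driven by a timeline.
; If CloseTheDoor is set, a starship entering the close trigger starts, once only, a move to the NormalDoorReturnScene position.
; That move calls MoveComponentTo on every timeline update, using the timeline value as duration.
; BeginPlay creates a dynamic material instance for the door and sets its Material variable on it.
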(event OnComponentBeginOverlap(NormalDoorCloseTrigger)
  (params (OverlappedComponent :type Primitive%20Component%20Object%20Reference) (OtherActor :type Actor%20Object%20Reference) (OtherComp :type Primitive%20Component%20Object%20Reference) (OtherBodyIndex :type Integer) (bFromSweep :type Boolean) (SweepResult :type Hit%20Result%20Structure%20%28by%20ref%29))
  (if (Variables|Default|GetCloseTheDoor?)
    (Utilities|FlowControl|DoOnce false
      (:Completed
        (Utilities|Casting|CastToBp_Starship OtherActor)
        (bind _movement (Timeline|Movement Play)
          (:Update
            (Components|MoveComponentTo (Variables|Default|GetDoor) (Variables|/Script/Engine.SceneComponent|GetRelativeLocation (Variables|Default|GetNormalDoorReturnScene)) "0, 0, 0" false false _movement false)))))))

(event Collision|EventActorBeginOverlap
  (params (OtherActor :type Actor%20Object%20Reference)))

(event EventBeginPlay
  (bind _door (Variables|Default|GetDoor))
  (Rendering|Material|CreateDynamicMaterialInstance _door 0 (Rendering|Material|GetMaterial _door 0) "None" :!class /Script/Engine.PrimitiveComponent)
  (Rendering|Material|SetMaterial (Variables|Default|GetDoor) 0 (Variables|Default|GetMaterial)))

(event EventTick
  (params (DeltaSeconds :type Float%20%28single-precision%29)))

(event EventConnection?
  (bind _spline (Variables|Default|GetSpline))
  (bind _movement (Timeline|T_Movement Play)
    (:Update
      (Transformation|SetWorldLocation (Variables|Default|GetDoor) (Spline|GetLocationatDistanceAlongSpline _spline (* (Spline|GetSplineLength _spline) _movement) "World") false false))))

(fn ConstructionScript)