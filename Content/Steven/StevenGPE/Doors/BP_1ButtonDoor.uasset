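; One-button door Blueprint with a force field that opens on connection and an optional closing behavior.
; The Connection? event plays an opening sound, animates the force field's X scale through a timeline, then destroys that component.
; When CloseTheDoor is set, a Bp_Starship entering the close trigger starts a Movement timeline that drives MoveComponentTo toward the return scene component's location.
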(event OnComponentBeginOverlap(NormalDoorCloseTrigger)
  (params (OverlappedComponent :type Primitive%20Component%20Object%20Reference) (OtherActor :type Actor%20Object%20Reference) (OtherComp :type Primitive%20Component%20Object%20Reference) (OtherBodyIndex :type Integer) (bFromSweep :type Boolean) (SweepResult :type Hit%20Result%20Structure%20%28by%20ref%29))
  (if (Variables|Default|GetCloseTheDoor?)
    (Utilities|Casting|CastToBp_Starship OtherActor)
    (bind _movement (Timeline|Movement Play)
      (:Update
        (Components|MoveComponentTo 0 (Variables|/Script/Engine.SceneComponent|GetRelativeLocation (Variables|Default|GetNormalDoorReturnScene)) "0, 0, 0" false false _movement false)))))

(event Collision|EventActorBeginOverlap
  (params (OtherActor :type Actor%20Object%20Reference)))

(event EventBeginPlay)

(event EventTick
  (params (DeltaSeconds :type Float%20%28single-precision%29)))

(event EventConnection?
  (bind _gpe_door_base_forcefield (Variables|Default|GetGPE_Door_Base_ForceField))
  (Audio|PlaySoundatLocation "/Game/Assets/Audio/SOUNDBANK/ENVIRONMENT/ENV_DOOR_Open_Orange.ENV_DOOR_Open_Orange" "0, 0, 0" "0, 0, 0" 1.0 1.0 0.0 0 0 0)
  (bind _float (Timeline|Timeline Play)
    (:Update
      (Transformation|SetRelativeScale3D _gpe_door_base_forcefield (Math|Vector|MakeVector _float 6.25 1e+01)))
    (:Finished
      (Components|DestroyComponent _gpe_door_base_forcefield))))

(fn ConstructionScript)