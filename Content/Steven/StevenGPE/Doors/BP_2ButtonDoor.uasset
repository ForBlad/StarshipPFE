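; BP_2ButtonDoor is a door that moves along a spline when two linked BPSynchroLock buttons are both activated.
; Connection? checks both locks, then a FlipFlop alternately plays or reverses a timeline driving the door's spline position and rotation.
; If CloseTheDoor is set, a Bp_Starship overlapping the trigger moves the door toward a close-position component.
; AreAllButtonsActivated checks every lock but goes unused in these graphs.
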(event OnComponentBeginOverlap(SynchDoorCloseTrigger)
  (params (OverlappedComponent :type Primitive%20Component%20Object%20Reference) (OtherActor :type Actor%20Object%20Reference) (OtherComp :type Primitive%20Component%20Object%20Reference) (OtherBodyIndex :type Integer) (bFromSweep :type Boolean) (SweepResult :type Hit%20Result%20Structure%20%28by%20ref%29))
  (if (Variables|Default|GetCloseTheDoor)
    (Utilities|Casting|CastToBp_Starship OtherActor)
    (bind _movement (Timeline|Timeline_0 Play)
      (:Update
        (Components|MoveComponentTo (Variables|Default|GetDoor) (Variables|/Script/Engine.SceneComponent|GetRelativeLocation (Variables|Default|GetSynchDoorCloseScene)) "0, 0, 0" false false _movement false)))))

(event EventConnection?
  (bind _bp_synchrolock (Variables|Default|GetBP_SynchroLock))
  (bind _spline (Variables|Default|GetSpline))
  (bind _door (Variables|Default|GetDoor))
  (if (and (Variables|/Game/Steven/StevenGPE/Buttons/BP_SynchroLock.BP_SynchroLock_C|Getbutton_isActivated (Utilities|Array|Get(acopy) _bp_synchrolock)) (Variables|/Game/Steven/StevenGPE/Buttons/BP_SynchroLock.BP_SynchroLock_C|Getbutton_isActivated (Utilities|Array|Get(acopy) _bp_synchrolock 1)))
    (Utilities|FlowControl|FlipFlop
      (:A
        (bind _movement (Timeline|T_Movement Play)
          (:Update
            (Transformation|SetWorldTransform _door (Math|Transform|MakeTransform (Spline|GetLocationatDistanceAlongSpline _spline (* (Spline|GetSplineLength _spline) _movement) "World") (Spline|GetRotationatDistanceAlongSpline _spline (* (Spline|GetSplineLength _spline) _movement) "World") (Variables|/Script/Engine.SceneComponent|GetRelativeScale3D _door)) false false))))
      (:B
        (Timeline|T_Movement Reverse)))))

(event EventBeginPlay
  (bind _door (Variables|Default|GetDoor))
  (Rendering|Material|CreateDynamicMaterialInstance _door 0 (Rendering|Material|GetMaterial _door 0) "None" :!class /Script/Engine.PrimitiveComponent)
  (Rendering|Material|SetMaterial (Variables|Default|GetDoor) 0 (Variables|Default|GetMaterial)))

(fn ConstructionScript)

(fn AreAllButtonsActivated?
  (for _array_element (Variables|Default|GetBP_SynchroLock)
    (if (not (Variables|/Game/Steven/StevenGPE/Buttons/BP_SynchroLock.BP_SynchroLock_C|Getbutton_isActivated _array_element))
      (return false)))
  (return true))