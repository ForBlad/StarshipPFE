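; BP_FlipFlopDoor is a door that slides back and forth along a spline, driven by two flip-flop lock buttons.
; Tick polls both locks, playing the T_Movement timeline when only the first is active and reversing it when only the second is.
; The timeline maps its value to distance along the spline, setting the door's location and rotation while keeping its scale.
; AreAllButtonsActivated is an unfinished stub with no effect.
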(event EventTick
  (params (DeltaSeconds :type Float%20%28single-precision%29))
  (bind _bp_flipfloplock (Variables|Default|GetBP_FlipFlopLock))
  (bind _door (Variables|Default|GetDoor))
  (bind _bp_flipfloplock_2 (Variables|Default|GetBP_FlipFlopLock))
  (bind _spline (Variables|Default|GetSpline))
  (if (and (Variables|/Game/Steven/StevenGPE/Buttons/BP_FlipFlopLock.BP_FlipFlopLock_C|Getbutton_isActivated (Utilities|Array|Get(acopy) _bp_flipfloplock_2)) (not (Variables|/Game/Steven/StevenGPE/Buttons/BP_FlipFlopLock.BP_FlipFlopLock_C|Getbutton_isActivated (Utilities|Array|Get(acopy) _bp_flipfloplock_2 1))))
    (CallFunction|Connection?)
    (elif (and (Variables|/Game/Steven/StevenGPE/Buttons/BP_FlipFlopLock.BP_FlipFlopLock_C|Getbutton_isActivated (Utilities|Array|Get(acopy) _bp_flipfloplock 1)) (not (Variables|/Game/Steven/StevenGPE/Buttons/BP_FlipFlopLock.BP_FlipFlopLock_C|Getbutton_isActivated (Utilities|Array|Get(acopy) _bp_flipfloplock))))
      (bind _movement (Timeline|T_Movement Reverse)
        (:Update
          (Transformation|SetWorldTransform _door (Math|Transform|MakeTransform (Spline|GetLocationatDistanceAlongSpline _spline (* (Spline|GetSplineLength _spline) _movement) "World") (Spline|GetRotationatDistanceAlongSpline _spline (* (Spline|GetSplineLength _spline) _movement) "World") (Variables|/Script/Engine.SceneComponent|GetRelativeScale3D _door)) false false))))))

(event EventBeginPlay
  (bind _door (Variables|Default|GetDoor))
  (Rendering|Material|CreateDynamicMaterialInstance _door 0 (Rendering|Material|GetMaterial _door 0) "None" :!class /Script/Engine.PrimitiveComponent)
  (Rendering|Material|SetMaterial (Variables|Default|GetDoor) 0 (Variables|Default|GetMaterial)))

(event EventConnection?
  (bind _door (Variables|Default|GetDoor))
  (bind _spline (Variables|Default|GetSpline))
  (bind _movement (Timeline|T_Movement Play)
    (:Update
      (Transformation|SetWorldTransform _door (Math|Transform|MakeTransform (Spline|GetLocationatDistanceAlongSpline _spline (* (Spline|GetSplineLength _spline) _movement) "World") (Spline|GetRotationatDistanceAlongSpline _spline (* (Spline|GetSplineLength _spline) _movement) "World") (Variables|/Script/Engine.SceneComponent|GetRelativeScale3D _door)) false false))))

(fn ConstructionScript)

(fn AreAllButtonsActivated?
  (bind _bp_flipfloplock (Variables|Default|GetBP_FlipFlopLock))
  (if (not (Variables|/Game/Steven/StevenGPE/Buttons/BP_FlipFlopLock.BP_FlipFlopLock_C|Getbutton_isActivated (Utilities|Array|Get(acopy) _bp_flipfloplock)))
    (if (Variables|/Game/Steven/StevenGPE/Buttons/BP_FlipFlopLock.BP_FlipFlopLock_C|Getbutton_isActivated (Utilities|Array|Get(acopy) _bp_flipfloplock 1))
      _)))