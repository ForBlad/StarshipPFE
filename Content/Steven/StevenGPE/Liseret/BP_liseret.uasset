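; BP_liseret is a spline-drawn trim strip that lights up through its emissive material when the LightOn event fires.
; The construction script builds a collision-free, Z-forward cylinder spline mesh between each pair of LiseretSpline points, matching locations and tangents.
; Each segment's dynamic material call takes MatRef as source and writes the result back to it.
; LightOn plays a timeline that drives the Emissive parameter on that final MatRef.
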(event Custom|LightOn
  (bind _emissivechange (Timeline|Timeline_1 Play)
    (:Update
      (Rendering|Material|SetScalarParameterValue (Variables|Default|GetMatRef) "Emissive" _emissivechange :!class /Script/Engine.MaterialInstanceDynamic))))

(fn ConstructionScript
  (bind _liseret_spline (Variables|Default|GetLiseret_Spline))
  (for _index (range 0 (- (Spline|GetNumberOfSplinePoints (Variables|Default|GetLiseret_Spline)) 2))
    (bind _returnvalue (AddComponent|AddSplineMeshComponent false))
    (bind _returnvalue_2 (Rendering|Material|CreateDynamicMaterialInstance _returnvalue 0 (stale _output_get) "None" :!class /Script/Engine.PrimitiveComponent))
    (bind _output_get (Variables|Default|SetMatRef _returnvalue_2))
    (Collision|SetCollisionEnabled _returnvalue "NoCollision")
    (Components|StaticMesh|SetStaticMesh _returnvalue "/Game/Steven/StevenGPE/Liseret/LiseretCylinder.LiseretCylinder")
    (SplineMesh|SetForwardAxis _returnvalue "Z" true)
    (Transformation|AttachComponentToComponent _returnvalue (Variables|Default|GetLiseret_Spline) "None" "KeepRelative" "KeepRelative" "KeepRelative" true)
    (SplineMesh|SetStartandEnd _returnvalue (.Location (Spline|GetLocationandTangentatSplinePoint _liseret_spline _index "Local")) (.Tangent (Spline|GetLocationandTangentatSplinePoint _liseret_spline _index "Local")) (.Location (Spline|GetLocationandTangentatSplinePoint _liseret_spline (+ _index 1) "Local")) (.Tangent (Spline|GetLocationandTangentatSplinePoint _liseret_spline (+ _index 1) "Local")) true :!class /Script/Engine.SplineMeshComponent)))