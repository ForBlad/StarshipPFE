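; Door Blueprint that opens once all of its linked synchro-lock buttons are activated.
; The Connection? event checks every entry in the BPSynchroLock array for ButtonIsActivated.
; When all are active, the T_Movement timeline slides the door along a spline, matching its position and rotation while keeping its scale.
; The file contains no closing or reverse logic.
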(event EventConnection?
  (bind _spline (Variables|Default|GetSpline))
  (bind _door (Variables|Default|GetDoor))
  (bind _bool (CallFunction|AreAllButtonsActivated?))
  (if _bool
    (bind _movement (Timeline|T_Movement PlayFromStart)
      (:Update
        (Transformation|SetWorldTransform _door (Math|Transform|MakeTransform (Spline|GetLocationatDistanceAlongSpline _spline (* (Spline|GetSplineLength _spline) _movement) "World") (Spline|GetRotationatDistanceAlongSpline _spline (* (Spline|GetSplineLength _spline) _movement) "World") (Variables|/Script/Engine.SceneComponent|GetRelativeScale3D _door)) false false)))))

(fn ConstructionScript)

(fn AreAllButtonsActivated?
  (for _array_element (Variables|Default|GetBP_SynchroLock)
    (if (not (Variables|/Game/Steven/StevenGPE/BP_SynchroLock.BP_SynchroLock_C|Getbutton_isActivated _array_element))
      (return false)))
  (return true))