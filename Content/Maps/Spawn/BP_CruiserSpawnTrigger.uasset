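; A spawn trigger that creates AI_Cruser1 cruiser enemies at its Scene location when the player, matched by display name BP_Player, first overlaps it.
; In single mode it spawns one cruiser and destroys itself.
; With SpawnMultiple, it spawns slightly smaller cruisers in a delayed, self-calling loop gated by a resettable DoOnce, decrementing NbreEnnemi while at least LimitMax and destroying itself at zero.
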(event OnComponentBeginOverlap(Trigger)
  (params (OverlappedComponent :type Primitive%20Component%20Object%20Reference) (OtherActor :type Actor%20Object%20Reference) (OtherComp :type Primitive%20Component%20Object%20Reference) (OtherBodyIndex :type Integer) (bFromSweep :type Boolean) (SweepResult :type Hit%20Result%20Structure%20%28by%20ref%29))
  (if (Utilities|Enum|Equal(Enum) (Utilities|GetDisplayName OtherActor) "BP_Player")
    (Utilities|FlowControl|DoOnce false
      (:Completed
        (if (Variables|Default|GetSpawn_Multiple)
          (if (>= (Variables|Default|GetNbre_ennemi) (Variables|Default|GetLimit_Max))
            (Utilities|FlowControl|DoOnce false
              (:Completed
                (Game|SpawnActorfromClass "/Game/Loic/AI_WIP_Behavior/AI_Cruser1.AI_Cruser1_C" (Math|Transform|MakeTransform (Transformation|GetWorldLocation (Variables|Default|GetScene)) "0, 0, 0" "0.600000,0.600000,0.600000") "Undefined" 0 0)
                (Variables|Default|SetNbre_ennemi (- (Variables|Default|GetNbre_ennemi) 1))
                (if (== (Variables|Default|GetNbre_ennemi) 0)
                  (Actor|DestroyActor)
                  (else
                    (CallFunction|ResetDoOnce)
                    (Utilities|FlowControl|Delay (Variables|Default|GetTimer_Spawn))
                    (CallFunction|RepeatSpawnMob))))))
          (else
            (Game|SpawnActorfromClass "/Game/Loic/AI_WIP_Behavior/AI_Cruser1.AI_Cruser1_C" (Math|Transform|MakeTransform (Transformation|GetWorldLocation (Variables|Default|GetScene)) "0, 0, 0" "0.700000,0.700000,0.700000") "Undefined" 0 0)
            (Actor|DestroyActor)))))))

(event Custom|Repeat_SpawnMob
  (if (>= (Variables|Default|GetNbre_ennemi) (Variables|Default|GetLimit_Max))
    (Utilities|FlowControl|DoOnce false
      (:Completed
        (Game|SpawnActorfromClass "/Game/Loic/AI_WIP_Behavior/AI_Cruser1.AI_Cruser1_C" (Math|Transform|MakeTransform (Transformation|GetWorldLocation (Variables|Default|GetScene)) "0, 0, 0" "0.600000,0.600000,0.600000") "Undefined" 0 0)
        (Variables|Default|SetNbre_ennemi (- (Variables|Default|GetNbre_ennemi) 1))
        (if (== (Variables|Default|GetNbre_ennemi) 0)
          (Actor|DestroyActor)
          (else
            (CallFunction|ResetDoOnce)
            (Utilities|FlowControl|Delay (Variables|Default|GetTimer_Spawn))
            (CallFunction|RepeatSpawnMob)))))))

(event Custom|ResetDoOnce
  (Utilities|FlowControl|DoOnce false) ; enters at Reset
)

(fn ConstructionScript)