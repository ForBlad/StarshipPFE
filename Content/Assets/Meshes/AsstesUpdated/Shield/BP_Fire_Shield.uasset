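; Fire shield Blueprint that shows impacts on its Forcefield component and glows up or down with shield power.
; On hit, it plays a random sound (the fourth wired one is unreachable), spawns an impact emitter and feeds the hit point and a timeline-driven radius into the dynamic material.
; BeginPlay creates the shield's dynamic material, whose Emissive parameter is animated by separate ShieldPowered and ShieldDown timelines.
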(event OnComponentHit(Forcefield)
  (params (HitComponent :type Primitive%20Component%20Object%20Reference) (OtherActor :type Actor%20Object%20Reference) (OtherComp :type Primitive%20Component%20Object%20Reference) (NormalImpulse :type Vector :default "0, 0, 0") (Hit :type Hit%20Result%20Structure%20%28by%20ref%29))
  (bind _forcefield (Variables|Default|GetForcefield))
  (bind _returnvalue (Transformation|GetWorldLocation _forcefield))
  (switch int (Math|Random|RandomInteger 3)
    (:0
      (Audio|PlaySoundatLocation "/Game/Assets/Audio/SOUNDBANK/SFX/SFX_SHIP/MAINSHIP/MAINSHIP_SHIELD/SFX_SHIP_MAINSHIP_Shield_TakingHit_01.SFX_SHIP_MAINSHIP_Shield_TakingHit_01" _returnvalue "0, 0, 0" 1.0 1.0 0.0 0 0 0))
    (:1
      (Audio|PlaySoundatLocation "/Game/Assets/Audio/SOUNDBANK/SFX/SFX_SHIP/MAINSHIP/MAINSHIP_SHIELD/SFX_SHIP_MAINSHIP_Shield_TakingHit_02.SFX_SHIP_MAINSHIP_Shield_TakingHit_02" _returnvalue "0, 0, 0" 1.0 1.0 0.0 0 0 0))
    (:2
      (Audio|PlaySoundatLocation "/Game/Assets/Audio/SOUNDBANK/SFX/SFX_SHIP/MAINSHIP/MAINSHIP_SHIELD/SFX_SHIP_MAINSHIP_Shield_TakingHit_03.SFX_SHIP_MAINSHIP_Shield_TakingHit_03" _returnvalue "0, 0, 0" 1.0 1.0 0.0 0 0 0))
    (:3
      (Audio|PlaySoundatLocation "/Game/Assets/Audio/SOUNDBANK/SFX/SFX_SHIP/MAINSHIP/MAINSHIP_SHIELD/SFX_SHIP_MAINSHIP_Shield_TakingHit_04.SFX_SHIP_MAINSHIP_Shield_TakingHit_04" _returnvalue "0, 0, 0" 1.0 1.0 0.0 0 0 0)))
  (bind _returnvalue_2 (Rendering|Material|CreateDynamicMaterialInstance (Variables|Default|GetForcefield) 0 0 "None" :!class /Script/Engine.PrimitiveComponent))
  (Rendering|Material|SetVectorParameterValue _returnvalue_2 "pos" (Math|Conversions|ToLinearColor(Vector) (.impactpoint Hit)) :!class /Script/Engine.MaterialInstanceDynamic)
  (Effects|SpawnEmitteratLocation "/Game/Léa/FX/Particle/P_Shield_impactv2.P_Shield_impactv2" (.impactpoint Hit) (Math|Rotator|MakeRotfromX (.impactnormal Hit)))
  (bind _newtrack_0 (Timeline|animate PlayFromStart)
    (:Update
      (Rendering|Material|SetScalarParameterValue _returnvalue_2 "radius" (* _newtrack_0 2e+01) :!class /Script/Engine.MaterialInstanceDynamic))))

(event Custom|ShieldPowered
  (bind _emissive_busstoooo (Timeline|EMISSIVE%20BOOOOOST PlayFromStart)
    (:Update
      (Rendering|Material|SetScalarParameterValue (Variables|Default|GetRaiseEmissive) "Emissive" _emissive_busstoooo :!class /Script/Engine.MaterialInstanceDynamic))))

(event Custom|Shield%20Down
  (bind _emissive_busstoooo (Timeline|Emissive%20down PlayFromStart)
    (:Update
      (Rendering|Material|SetScalarParameterValue (Variables|Default|GetRaiseEmissive) "Emissive" _emissive_busstoooo :!class /Script/Engine.MaterialInstanceDynamic))))

(event EventBeginPlay
  (bind _returnvalue (Rendering|Material|CreateDynamicMaterialInstance (Variables|Default|GetForcefield) 0 "/Game/Assets/Particles/Shield/M_Shield_activev2_Inst.M_Shield_activev2_Inst" "None" :!class /Script/Engine.PrimitiveComponent))
  (Variables|Default|SetRaiseEmissive _returnvalue))

(fn ConstructionScript)