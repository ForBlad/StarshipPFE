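; Player character for a four-player starship crew game, with per-player colors, ship respawn points and controller rumble.
; Once four players spawn, it numbers and initializes them; leaving the ship's collision triggers respawn.
; Inputs move the character, operate nearby posts (snapped to by timeline), pilot, handle kits and extinguishers, or taunt.
; Nearest posts and pickups come from distance scans over all actors, and Tick tilts the player with the hull.
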(event OnComponentEndOverlap(CapsuleComponent)
  (params (OverlappedComponent :type Primitive%20Component%20Object%20Reference) (OtherActor :type Actor%20Object%20Reference) (OtherComp :type Primitive%20Component%20Object%20Reference) (OtherBodyIndex :type Integer))
  ;[1 1 1] Spawn on positions at Init or on Falling Off
  (bind _asbp_starship (Utilities|Casting|CastToBp_Starship OtherActor))
  (if (== (Variables|/Game/Thibaud/Blueprints/Player/Bp_Starship.Bp_Starship_C|GetCollision_Ship _asbp_starship) OtherComp)
    (for (_array_element _array_index) (stale Custom|PlayerInit _output_get)
      (if (== _array_index (Variables|Default|GetPlayerNumber))
        (Transformation|SetWorldLocation (Variables|Collision|GetCapsuleComponent) (Transformation|GetWorldLocation _array_element) false true)
        (CallFunction|StartTauntNoShake)))))

(event Custom|StartTaunt
  ;[1 1 1] Taunt
  (if (< (/ (Math|Vector|VectorLength (Transformation|GetVelocity)) (Variables|/Script/Engine.CharacterMovementComponent|GetMaxWalkSpeed (Variables|Character|GetCharacterMovement))) 0.01)
    (Utilities|FlowControl|Sequence
      (:then_0
        (Game|Feedback|PlayDynamicForceFeedback (Variables|Default|GetCurrentController) 0.08 3.0 true true true true))
      (:then_1
        (Variables|Default|SetTauntOn? true)
        (Utilities|FlowControl|Delay 3.0)
        (CallFunction|StopTaunt)))))

(event Custom|MoveToPost
  (bind _self self)
  (bind _currentpost (Variables|Default|GetcurrentPost))
  (bind _returnvalue (Transformation|GetActorLocation _self))
  (bind _characterdirection (Variables|/Game/Thibaud/Blueprints/Player/Post/BPA_Post_Parent.BPA_Post_Parent_C|GetCharacterDirection _currentpost))
  (bind _returnvalue_2 (Transformation|GetWorldLocation _characterdirection))
  (bind _returnvalue_3 (Transformation|GetWorldRotation _characterdirection))
  ;[1 1 1] MOVE TO POST
  (bind _newtrack_0 (Timeline|Timeline_0 PlayFromStart)
    (:Update
      (Transformation|SetActorLocation (Math|Vector|Lerp(Vector) (Math|Vector|MakeVector (.x _returnvalue) (.y _returnvalue) (.z _returnvalue)) (Math|Vector|MakeVector (.x _returnvalue_2) (.y _returnvalue_2) (.z _returnvalue)) _newtrack_0) false true)
      (Transformation|SetActorRotation (Math|Rotator|Lerp(Rotator) (Transformation|GetActorRotation _self) (Math|Rotator|MakeRotator (.roll _returnvalue_3) (.pitch _returnvalue_3) (+ (.yaw _returnvalue_3) 9e+01)) _newtrack_0 true) true))))

(event Custom|StopTaunt
  ;[1 1 1] Taunt
  (Variables|Default|SetTauntOn? false)
  (Game|Feedback|PlayDynamicForceFeedback (Variables|Default|GetCurrentController) 0.08 3.0 true true true true) ; enters at Stop
)

(event Custom|PlayerInit
  (bind _playernumber (Variables|Default|GetPlayerNumber))
  (bind _identity_circle (Variables|Default|GetIdentity%20Circle))
  (Utilities|FlowControl|Sequence
    (:then_0
      ;[1 1 1] Player Colors
      (Rendering|Material|SetMaterial (Variables|Character|GetMesh) 0 (Utilities|Array|Get(acopy) (Variables|Default|GetPlayerColors) _playernumber))
      (Rendering|Material|SetMaterial _identity_circle 0 (Utilities|Array|Get(acopy) (Variables|Default|GetCircleColors) _playernumber))
      (Components|StaticMesh|SetStaticMesh _identity_circle (Utilities|Array|Get(acopy) (Variables|Default|GetCircle%20Mesh) _playernumber))
      (bind _returnvalue (Actor|GetActorOfClass "/Game/Thibaud/Blueprints/Player/Bp_Starship.Bp_Starship_C"))
      (Variables|Default|SetBPA%20Vaisseau _returnvalue))
    (:then_1
      ;[1 1 1] Spawn on positions at Init or on Falling Off
      (bind _returnvalue_2 (Actor|GetActorOfClass "/Game/Thibaud/Blueprints/Player/Bp_Starship.Bp_Starship_C"))
      (bind _output_get (Variables|Default|SetRespawnPositions (Utilities|Array|MakeArray (Variables|/Game/Thibaud/Blueprints/Player/Bp_Starship.Bp_Starship_C|GetRespawn_Position _returnvalue_2) (Variables|/Game/Thibaud/Blueprints/Player/Bp_Starship.Bp_Starship_C|GetRespawn_Position1 _returnvalue_2) (Variables|/Game/Thibaud/Blueprints/Player/Bp_Starship.Bp_Starship_C|GetRespawn_Position2 _returnvalue_2) (Variables|/Game/Thibaud/Blueprints/Player/Bp_Starship.Bp_Starship_C|GetRespawn_Position3 _returnvalue_2))))
      (for (_array_element _array_index) _output_get
        (if (== _array_index (Variables|Default|GetPlayerNumber))
          (Transformation|SetWorldLocation (Variables|Collision|GetCapsuleComponent) (Transformation|GetWorldLocation _array_element) false true)
          (CallFunction|StartTauntNoShake))))))

(event Custom|StartTauntNoShake
  ;[1 1 1] Taunt
  (Variables|Default|SetTauntOn? true)
  (Utilities|FlowControl|Delay 3.0)
  (CallFunction|StopTaunt))

(event Custom|ForceFeedback
  (params (Intensity :type Float%20%28single-precision%29) (Duration :type Float%20%28single-precision%29) (LargeOn? :type Boolean))
  ;[1 1 1] Controller Shake from other BPs
  (Game|Feedback|PlayDynamicForceFeedback (Variables|Default|GetCurrentController) Intensity Duration LargeOn? true LargeOn? true))

(event EventTick
  (params (DeltaSeconds :type Float%20%28single-precision%29))
  (bind _rootcomponent (Variables|Transformation|GetRootComponent))
  (bind _bpa_vaisseau (Variables|Default|GetBPA%20Vaisseau))
  (bind _returnvalue (Transformation|GetWorldRotation _rootcomponent))
  (bind _ship_hull (Variables|/Game/Thibaud/Blueprints/Player/Bp_Starship.Bp_Starship_C|GetShip%20Hull _bpa_vaisseau))
  (bind _returnvalue_2 (Transformation|GetWorldRotation _ship_hull))
  (bind _returnvalue_3 (Transformation|GetWorldRotation _ship_hull))
  (bind _returnvalue_4 (Class|KismetMathLibrary|NegateRotator _returnvalue_3))
  (bind _returnvalue_5 (Math|Rotator|MakeRotator (.pitch _returnvalue_4) (.roll _returnvalue_4) (.yaw _returnvalue)))
  (bind _returnvalue_6 (Class|KismetMathLibrary|NegateRotator _returnvalue_5))
  ;[1 1 1] Tilt with Ship Hull
  (Transformation|SetWorldRotation _rootcomponent (Math|Rotator|MakeRotator (.pitch _returnvalue_6) (.roll _returnvalue_6) (.yaw _returnvalue)) false false)
  (Transformation|SetWorldRotation (Variables|Default|GetIdentity%20Circle) (Math|Rotator|MakeRotator (.roll _returnvalue_2) (.pitch _returnvalue_2) (.yaw _returnvalue_2)) false false))

(event EventBeginPlay
  ;[1 1 1] Wait until all Players spawned to Initialize
  (bind _returnvalue (Actor|GetActorOfClass "/Game/Thibaud/Blueprints/Player/Bp_Starship.Bp_Starship_C"))
  (bind _result (Math|Integer|IncrementInt (Variables|/Game/Thibaud/Blueprints/Player/Bp_Starship.Bp_Starship_C|GetPlayersSpawned _returnvalue))
    (:%20%20
      (if (>= _result 4)
        (Utilities|FlowControl|DoOnce false
          (:Completed
            (bind _outactors (Actor|GetAllActorsOfClass "BP_Player_C"))
            (for (_array_element _array_index) _outactors
              (Variables|BP_Player_C|SetPlayerNumber _array_element _array_index)
              (bind _asplayer_controller (Utilities|Casting|CastToPlayerController (Pawn|GetController _array_element)))
              (Variables|BP_Player_C|SetCurrentController _array_element _asplayer_controller)
              (CallFunction|PlayerInit _array_element))))))))

(event Input|ActionEvents|InputActionInteraction
  (params (Key :type Key%20Structure :default "None"))
  (bind _self self)
  (bind _currentpost (Variables|Default|GetCurrentPost))
  (bind _currentpickup (Variables|Default|GetCurrentPickup))
  (:Pressed
    ;[1 1 1] NEW INTERACTION
    (if (Variables|Default|GetCurrentlyUsingA%20Post?)
      (Default|PostDeactivate _currentpost _self)
      (Game|Feedback|PlayDynamicForceFeedback (Variables|Default|GetCurrentController) 0.2 0.2 false true false true :!label _label)
      (else
        (bind (_post_in_range_ _nearest_post) (CallFunction|FindNearestPost->SettoCurrentPostifinDistance))
        (if (and _post_in_range_ (not (Variables|/Game/Thibaud/Blueprints/Player/Post/BPA_Post_Parent.BPA_Post_Parent_C|GetIsOccupied? _nearest_post)))
          (Default|PostActivate _currentpost _self)
          (Utilities|FlowControl|Sequence
            (:then_0
              (if (!= (Utilities|GetClass _currentpost) "/Game/Thibaud/Blueprints/Player/Post/BPA_Post_Logistics.BPA_Post_Logistics_C")
                (CallFunction|MovetoPost)
                (Variables|Default|SetTauntOn? false)
                (if (Variables|Default|GetCurrentlyHoldingAnObject?)
                  (Default|Pick/DropItem _currentpickup self)
                  (bind _asbpa_kits_extinguisher (Utilities|Casting|CastToBPA_Kits_Extinguisher _currentpickup))
                  (Default|StopExtinguishing _asbpa_kits_extinguisher))))
            (:then_1
              (goto _label))))))))

(event Input|ActionEvents|InputActionUse
  (params (Key :type Key%20Structure :default "None"))
  (bind _currentpickup (Variables|Default|GetCurrentPickup))
  (bind _currentlyholdinganobject_ (Variables|Default|GetCurrentlyHoldingAnObject?))
  (bind _returnvalue (Utilities|IsValid _currentpickup))
  (bind _returnvalue_2 (and _currentlyholdinganobject_ _returnvalue))
  (:Pressed
    ;[1 1 1] Extinguish
    (if _returnvalue_2
      (bind _asbpa_kits_extinguisher (Utilities|Casting|CastToBPA_Kits_Extinguisher _currentpickup))
      (Default|UseExtinguisher _asbpa_kits_extinguisher self)))
  (:Released
    (if _returnvalue_2
      (bind _asbpa_kits_extinguisher_2 (Utilities|Casting|CastToBPA_Kits_Extinguisher _currentpickup))
      (Default|StopExtinguishing _asbpa_kits_extinguisher_2))))

(event Input|ActionEvents|InputActionDrop
  (params (Key :type Key%20Structure :default "None"))
  (:Pressed
    ;[1 1 1] Drop
    (if (Variables|Default|GetCurrentlyHoldingAnObject?)
      (Default|Pick/DropItem (Variables|Default|GetCurrentPickup) self)
      (Game|Feedback|PlayDynamicForceFeedback (Variables|Default|GetCurrentController) 0.25 0.3 false true false true))))

(event Input|ActionEvents|InputActionUse
  (params (Key :type Key%20Structure :default "None"))
  (bind _currentpickup (Variables|Default|GetCurrentPickup))
  (:Pressed
    (if (Variables|Default|GetCurrentlyUsingA%20Post?)
      ;[1 1 1] Use Station
      (Default|Use (Variables|Default|GetCurrentPost))
      (else
        ;[1 1 1] Grab
        (if (Variables|Default|GetCurrentlyHoldingAnObject?)
          ;[1 1 1] Drop
          (if (!= (Utilities|GetClass _currentpickup) "/Game/Thibaud/Blueprints/Player/Post/FireFunctionality/BPA_Kits_Extinguisher.BPA_Kits_Extinguisher_C")
            (Default|Pick/DropItem _currentpickup self)
            (Game|Feedback|PlayDynamicForceFeedback (Variables|Default|GetCurrentController) 0.25 0.3 false true false true))
          (else
            (bind (_nearest_pickup _nearenough_) (CallFunction|FindClosestPickupItem))
            (if (and _nearenough_ (Utilities|IsValid _nearest_pickup))
              (Default|Pick/DropItem _nearest_pickup self)
              (Game|Feedback|PlayDynamicForceFeedback (Variables|Default|GetCurrentController) 0.2 0.2 false true false true :!label _label)
              (else
                ;[1 1 1] Spawn Kit
                (bind _returnvalue (Actor|GetActorOfClass "/Game/Thibaud/Blueprints/Player/Post/BPA_Post_Logistics.BPA_Post_Logistics_C"))
                (if (< (Math|Vector|VectorLength (- (Transformation|GetWorldLocation (Variables|/Script/Engine.Actor|GetRootComponent _returnvalue)) (Transformation|GetActorLocation self))) (Variables|Default|GetPostActivationDistance))
                  (Default|SpawnIteminHand _returnvalue self)
                  (Variables|Default|SetCurrentPost _returnvalue)
                  (CallFunction|MovetoPost)
                  (goto _label)
                  (else
                    ;[1 1 1] Taunt
                    (if (< (/ (Math|Vector|VectorLength (Transformation|GetVelocity)) (Variables|/Script/Engine.CharacterMovementComponent|GetMaxWalkSpeed (Variables|Character|GetCharacterMovement))) 0.01)
                      (Utilities|FlowControl|Sequence
                        (:then_0
                          (Game|Feedback|PlayDynamicForceFeedback (Variables|Default|GetCurrentController) 0.08 3.0 true true true true :!label _label_2))
                        (:then_1
                          (Variables|Default|SetTauntOn? true)
                          (Utilities|FlowControl|Delay 3.0)
                          (CallFunction|StopTaunt)))))))))))))
  (:Released
    (Utilities|FlowControl|Sequence
      (:then_0
        (Variables|Default|SetTauntOn? false)
        (goto _label_2 Stop))
      (:then_1
        (if (Variables|Default|GetCurrentlyUsingA%20Post?)
          (Default|Release (Variables|Default|GetCurrentPost)))))))

(event Input|AxisEvents|InputAxisAcceleration
  (params (AxisValue :type Float%20%28single-precision%29))
  ;[1 1 1] Acceleration ship
  (if (and (Variables|Default|GetIsCurrentlyPilot) (Variables|Default|GetCurrentlyUsingA%20Post?))
    (bind _returnvalue (Actor|GetActorOfClass "/Game/Thibaud/Blueprints/Player/Post/BPA_Post_Piloting.BPA_Post_Piloting_C"))
    (Default|Acceleration _returnvalue AxisValue)))

(event Input|AxisEvents|InputAxisDeceleration
  (params (AxisValue :type Float%20%28single-precision%29))
  ;[1 1 1] Acceleration ship
  (if (and (Variables|Default|GetIsCurrentlyPilot) (Variables|Default|GetCurrentlyUsingA%20Post?))
    (bind _returnvalue (Actor|GetActorOfClass "/Game/Thibaud/Blueprints/Player/Post/BPA_Post_Piloting.BPA_Post_Piloting_C"))
    (Default|Deceleration _returnvalue AxisValue)))

(event Input|AxisEvents|InputAxisTurn_X
  (params (AxisValue :type Float%20%28single-precision%29))
  ;[1 1 1] Rotation
  (if (Variables|Default|GetCurrentlyUsingA%20Post?)
    (Default|RotatePost (Variables|Default|GetCurrentPost) AxisValue (stale Input|AxisEvents|InputAxisTurn_Y AxisValue))))

(event Input|AxisEvents|InputAxisTurn_Y
  (params (AxisValue :type Float%20%28single-precision%29))
  ;[1 1 1] Rotation
  (if (Variables|Default|GetCurrentlyUsingA%20Post?)
    (Default|RotatePost (Variables|Default|GetCurrentPost) (stale Input|AxisEvents|InputAxisTurn_X AxisValue) AxisValue)))

(event Input|AxisEvents|InputAxisMoveForward
  (params (AxisValue :type Float%20%28single-precision%29))
  ;[1 1 1] CHARACTER MOVEMENT
  (if (not (Variables|Default|GetCurrentlyUsingA%20Post?))
    (Pawn|Input|AddMovementInput (Math|Vector|GetForwardVector (Math|Rotator|MakeRotator 0.0 0.0 (.Yaw (Math|Rotator|BreakRotator "0, 0, 0")))) AxisValue false)
    (if (or (!= AxisValue 0.0) (!= (stale Input|AxisEvents|InputAxisMoveRight AxisValue) 0.0))
      (CallFunction|StopTaunt))))

(event Input|AxisEvents|InputAxisMoveRight
  (params (AxisValue :type Float%20%28single-precision%29))
  ;[1 1 1] CHARACTER MOVEMENT
  (if (not (Variables|Default|GetCurrentlyUsingA%20Post?))
    (Pawn|Input|AddMovementInput (Math|Vector|GetRightVector (Math|Rotator|MakeRotator 0.0 0.0 (.Yaw (Math|Rotator|BreakRotator "0, 0, 0")))) AxisValue false)
    (if (or (!= (stale Input|AxisEvents|InputAxisMoveForward AxisValue) 0.0) (!= AxisValue 0.0))
      (CallFunction|StopTaunt))))

(event Input|KeyboardEvents|O
  (params (Key :type Key%20Structure :default "None"))
  (:Pressed
    ;[1 0 0] DEBUG FIRE
    (bind _returnvalue (Actor|GetActorOfClass "/Game/Thibaud/Blueprints/Player/Bp_Starship.Bp_Starship_C"))
    (Default|DamageStack _returnvalue 2.5e+02)))

(fn ConstructionScript)

(fn FindClosestPickupItem
  (Variables|Default|SetCurrentPickup 0)
  (Variables|Default|SetClosestPickupObject 999999.0)
  (bind _outactors (Actor|GetAllActorsOfClass "/Game/Thibaud/Blueprints/Kits/BPA_Kit_Parent.BPA_Kit_Parent_C"))
  (for _array_element _outactors
    (if (Math|Boolean|ANDBoolean (< (Math|Vector|VectorLength (- (Transformation|GetWorldLocation (Variables|/Game/Thibaud/Blueprints/Kits/BPA_Kit_Parent.BPA_Kit_Parent_C|GetHolder _array_element)) (Transformation|GetActorLocation self))) (Variables|Default|GetGrabbingDistance)) (< (Math|Vector|VectorLength (- (Transformation|GetWorldLocation (Variables|/Game/Thibaud/Blueprints/Kits/BPA_Kit_Parent.BPA_Kit_Parent_C|GetHolder _array_element)) (Transformation|GetActorLocation self))) (Variables|Default|GetClosestPickupObject)) (not (Variables|/Game/Thibaud/Blueprints/Kits/BPA_Kit_Parent.BPA_Kit_Parent_C|GetIsBeingCarried? _array_element)))
      (Variables|Default|SetClosestPickupObject (Math|Vector|VectorLength (- (Transformation|GetWorldLocation (Variables|/Game/Thibaud/Blueprints/Kits/BPA_Kit_Parent.BPA_Kit_Parent_C|GetHolder _array_element)) (Transformation|GetActorLocation self))))
      (bind _output_get (Variables|Default|SetCurrentPickup _array_element))))
  (if (!= _output_get 0)
    (return _output_get (< (Math|Vector|VectorLength (- (Transformation|GetWorldLocation (Variables|/Game/Thibaud/Blueprints/Kits/BPA_Kit_Parent.BPA_Kit_Parent_C|GetHolder _output_get)) (Transformation|GetActorLocation self))) (Variables|Default|GetGrabbingDistance)))
    (else
      (return 0 false))))

(fn FindNearestPost->SettoCurrentPostifinDistance
  (bind _outactors (Actor|GetAllActorsOfClass "/Game/Thibaud/Blueprints/Player/Post/BPA_Post_Parent.BPA_Post_Parent_C"))
  (for (_array_element _array_index) _outactors
    (if (> _array_index 0)
      (bind _isless_ (CallFunction|CheckDistance (Transformation|GetWorldLocation (Variables|/Game/Thibaud/Blueprints/Player/Post/BPA_Post_Parent.BPA_Post_Parent_C|GetDefaultSceneRoot (Variables|Default|GetCurrentPost))) (Transformation|GetWorldLocation (Variables|Collision|GetCapsuleComponent self)) (Variables|Default|GetPostActivationDistance)))
      ;[1 1 1] THIS WORKS BC THERE CAN BE ONLY ONE POST WITHIN POST ACTIVATION DISTANCE
      (if _isless_
        _
        (else
          (Variables|Default|SetCurrentPost _array_element)))
      (bind _isless__2 (CallFunction|CheckDistance (Transformation|GetWorldLocation (Variables|/Game/Thibaud/Blueprints/Player/Post/BPA_Post_Parent.BPA_Post_Parent_C|GetDefaultSceneRoot (Variables|Default|GetCurrentPost))) (Transformation|GetWorldLocation (Variables|Collision|GetCapsuleComponent self)) (Variables|Default|GetPostActivationDistance)))
      (else
        (Variables|Default|SetCurrentPost _array_element))))
  (return _isless__2 (Variables|Default|GetCurrentPost)))

(fn ChangePostColor
  (params (Post :type BPA%20Post%20Parent%20Object%20Reference)))

(fn CheckDistance
  (params (Actor%201%20pos :type Vector) (Actor%202%20pos :type Vector) (Less%20then :type Float%20%28single-precision%29))
  (bind _returnvalue (- Actor%201%20pos Actor%202%20pos))
  (bind _returnvalue_2 (Math|Vector|VectorLength _returnvalue))
  (return (< _returnvalue_2 Less%20then) _returnvalue_2))