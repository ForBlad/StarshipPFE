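; AI-driven player character that seeks and mans combat posts aboard the ship, while keeping aligned with the tilting hull.
; BeginPlay lists combat posts; Tick picks the closest free one once, re-armed after a steal briefly disables input.
; It steers by turning the screen-projected offset to that post into movement input, mimicking a stick.
; Overlapping a free combat post triggers interaction, which activates or leaves the current post; LookForClosestEnemy is empty.
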(event OnComponentBeginOverlap(PostCollision)
  (params (OverlappedComponent :type Primitive%20Component%20Object%20Reference) (OtherActor :type Actor%20Object%20Reference) (OtherComp :type Primitive%20Component%20Object%20Reference) (OtherBodyIndex :type Integer) (bFromSweep :type Boolean) (SweepResult :type Hit%20Result%20Structure%20%28by%20ref%29))
  (bind _asbpa_post_parent (Utilities|Casting|CastToBPA_Post_Parent OtherActor))
  (if (and (not (Variables|/Game/Thibaud/Blueprints/Player/Post/BPA_Post_Parent.BPA_Post_Parent_C|GetIsOccupied? _asbpa_post_parent)) (Variables|/Game/Thibaud/Blueprints/Player/Post/BPA_Post_Parent.BPA_Post_Parent_C|GetIsCombatPost? _asbpa_post_parent))
    (CallFunction|EventInteraction)
    (else
      (Development|PrintString "FALSE"))))

(event Custom|Event%20Interaction
  (bind _self self)
  (bind _currentpost (Variables|Default|GetCurrentPost))
  (bind _currentpost_2 (Variables|Default|GetCurrentPost))
  (bind _currentpickup (Variables|Default|GetCurrentPickup))
  (Development|PrintString "Hello")
  (if (Variables|Default|GetCurrentlyUsingA%20Post?)
    (Default|PostDeactivate _currentpost_2 _self)
    (elif (not (Variables|/Game/Thibaud/Blueprints/Player/Post/BPA_Post_Parent.BPA_Post_Parent_C|GetIsOnFire? _currentpost))
      (if (not (Variables|/Game/Thibaud/Blueprints/Player/Post/BPA_Post_Parent.BPA_Post_Parent_C|GetIsOccupied? _currentpost))
        (Default|PostActivate _currentpost_2 _self)
        (Utilities|FlowControl|Sequence
          (:then_0
            (if (Variables|/Game/Thibaud/Blueprints/Player/Post/BPA_Post_Parent.BPA_Post_Parent_C|GetIsSecondaryPost? _currentpost_2)
              ;[1 1 1] Secondary stations on Y
              (Utilities|FlowControl|Sequence
                (:then_0
                  (bind _asbpa_power (Utilities|Casting|CastToBPA_Power _currentpost))
                  (Default|UsePower _asbpa_power self)
                  (CallFunction|MovetoPost :!label _label))
                (:then_1
                  (if (not (Variables|Default|GetCurrentlyHoldingAnObject?))
                    (bind _asbpa_post_logistics (Utilities|Casting|CastToBPA_Post_Logistics _currentpost))
                    (Default|SpawnIteminHand _asbpa_post_logistics self)
                    (goto _label))))
              (else
                (CallFunction|MovetoPost)
                (Variables|Default|SetTauntOn? false)
                (if (Variables|Default|GetCurrentlyHoldingAnObject?)
                  (Default|Pick/DropItem _currentpickup self 0.0)
                  (bind _asbpa_kits_extinguisher (Utilities|Casting|CastToBPA_Kits_Extinguisher _currentpickup))
                  (Default|StopExtinguishing _asbpa_kits_extinguisher)))))
          (:then_1
            (Development|PrintString "rhis happening?")))))))

(event Custom|Stolen%20Input
  (Variables|Default|SetInputDisabled? true)
  (Utilities|FlowControl|Delay 0.9)
  (Variables|Default|SetInputDisabled? false)
  (Utilities|FlowControl|DoOnce false) ; enters at Reset
)

(event EventBeginPlay
  (CallFunction|PlayerInit)
  (CallFunction|ListCombatPosts)
  (bind _output_get (Variables|Default|SetCurrentPost (Utilities|Array|Get(acopy) (Variables|Default|GetCombatPosts))))
  (Development|PrintString (Utilities|GetDisplayName _output_get))
  (Variables|Default|SetPlayerNumber 3))

(event Collision|EventActorBeginOverlap
  (params (OtherActor :type Actor%20Object%20Reference)))

(event EventStealDelay
  (Development|PrintString "STOLEN")
  (CallFunction|StolenInput))

(event EventForceFeedback
  (params (Intensity :type Float%20%28single-precision%29) (Duration :type Float%20%28single-precision%29) (LargeOn? :type Boolean)))

(event EventTick
  (params (DeltaSeconds :type Float%20%28single-precision%29))
  (bind _yaw (Math|Rotator|BreakRotator "0, 0, 0"))
  (bind _returnvalue (Game|GetPlayerController 0))
  (bind _self self)
  (bind _rootcomponent (Variables|Transformation|GetRootComponent))
  (bind _bpa_vaisseau (Variables|Default|GetBPA%20Vaisseau))
  (bind _currentpost (Variables|Default|GetCurrentPost))
  (bind _returnvalue_2 (Math|Rotator|MakeRotator 0.0 0.0 _yaw))
  (bind _returnvalue_3 (Transformation|GetWorldRotation _rootcomponent))
  (bind _ship_hull (Variables|/Game/Thibaud/Blueprints/Player/Bp_Starship.Bp_Starship_C|GetShip%20Hull _bpa_vaisseau))
  (bind _capsulecomponent (Variables|Default|GetCapsuleComponent _self))
  (bind _rootcomponent_2 (Variables|/Script/Engine.Actor|GetRootComponent _currentpost))
  (bind _returnvalue_4 (Transformation|GetWorldLocation _rootcomponent_2))
  (bind _returnvalue_5 (Transformation|GetWorldLocation _capsulecomponent))
  (bind _returnvalue_6 (Transformation|GetWorldRotation _ship_hull))
  (bind _returnvalue_7 (Transformation|GetWorldRotation _ship_hull))
  (bind _screenlocation (Class|PlayerController|ProjectWorldLocationtoScreen _returnvalue _returnvalue_4 false))
  (bind _screenlocation_2 (Class|PlayerController|ProjectWorldLocationtoScreen _returnvalue _returnvalue_5 false))
  (bind _returnvalue_8 (Class|KismetMathLibrary|NegateRotator _returnvalue_7))
  (bind _returnvalue_9 (Math|Rotator|MakeRotator (.pitch _returnvalue_8) (.roll _returnvalue_8) (.yaw _returnvalue_3)))
  (bind _returnvalue_10 (- (.y _screenlocation) (.y _screenlocation_2)))
  (bind _returnvalue_11 (- (.x _screenlocation) (.x _screenlocation_2)))
  (bind _returnvalue_12 (Class|KismetMathLibrary|NegateRotator _returnvalue_9))
  (bind _returnvalue_13 (Class|KismetMathLibrary|VectorNormal2D (Math|Vector|MakeVector _returnvalue_11 _returnvalue_10 0.0) 0.0001))
  (bind _returnvalue_14 (Math|Float|Clamp(Float) (.x _returnvalue_13) -1.0))
  (bind _returnvalue_15 (Math|Float|Clamp(Float) (.y _returnvalue_13) -1.0))
  (if (Variables|Default|GetInputDisabled?)
    ;[1 1 1] Tilt with Ship Hull
    (Transformation|SetWorldRotation _rootcomponent (Math|Rotator|MakeRotator (.pitch _returnvalue_12) (.roll _returnvalue_12) (.yaw _returnvalue_3)) false false :!label _label)
    (Transformation|SetWorldRotation (Variables|Default|GetIdentity%20Circle) (Math|Rotator|MakeRotator (.roll _returnvalue_6) (.pitch _returnvalue_6) (.yaw _returnvalue_6)) false false)
    (else
      (Utilities|FlowControl|Sequence
        (:then_0
          (goto _label))
        (:then_1
          (if (not (Variables|Default|GetCurrentlyUsingA%20Post?))
            (Utilities|FlowControl|DoOnce false
              (:Completed
                (CallFunction|LookforAppropriatePost)
                (Development|PrintString "I DEED ETTT")))))
        (:then_2
          (Utilities|FlowControl|Sequence
            (:then_0
              (if (not (Variables|Default|GetCurrentlyUsingA%20Post?))
                (Pawn|Input|AddMovementInput (Math|Vector|GetForwardVector _returnvalue_2) _returnvalue_14 false)
                (if (or (!= _returnvalue_14 0.0) (!= _returnvalue_15 0.0)) :!label _label_2
                  _)))
            (:then_1
              (if (not (Variables|Default|GetCurrentlyUsingA%20Post?))
                (Pawn|Input|AddMovementInput (Math|Vector|GetRightVector _returnvalue_2) _returnvalue_15 false)
                (goto _label_2)))))))))

(event Input|ActionEvents|InputActionUse
  (params (Key :type Key%20Structure :default "None")))

(fn ConstructionScript
  (|CallParentFunction))

(fn LookforAppropriatePost
  (bind _self self)
  (bind _combatposts (Variables|Default|GetCombatPosts))
  (bind _output (Utilities|Array|Get(acopy) _combatposts))
  (Development|PrintString (Utilities|GetDisplayName _output))
  (Variables|Default|SetClosest%20Post _output)
  (for _array_element _combatposts
    (Math|Float|CompareFloat (Transformation|GetDistanceTo _array_element _self) (Transformation|GetDistanceTo (Variables|Default|GetClosest%20Post) _self)
      (:<
        (if (not (Variables|/Game/Thibaud/Blueprints/Player/Post/BPA_Post_Parent.BPA_Post_Parent_C|GetIsOccupied? _array_element))
          (Variables|Default|SetClosest%20Post _array_element)))))
  (Variables|Default|SetCurrentPost (Variables|Default|GetClosest%20Post)))

(fn ListCombatPosts
  (for _array_element (Variables|/Game/Thibaud/Blueprints/Player/Bp_Starship.Bp_Starship_C|GetAllPosts (Variables|Default|GetBPA%20Vaisseau))
    (if (Variables|/Game/Thibaud/Blueprints/Player/Post/BPA_Post_Parent.BPA_Post_Parent_C|GetIsCombatPost? _array_element)
      (Utilities|Array|Add (Variables|Default|GetCombatPosts) _array_element))))

(fn LookforClosestEnemy)