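; BP_Post_Fire is a fire actor tied to a player Post.
; On BeginPlay it attaches a looping fire sound and particle effect to its root.
; Each Extinguish call lowers Health by a fixed amount and plays an extinguisher effect, destroying the actor once Health is depleted.
; On destruction it notifies its Post through ExtinguishFire, passing itself.
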(event EventDestroyed
  (Default|ExtinguishFire (Variables|Default|GetPost) self))

(event EventBeginPlay
  (bind _defaultsceneroot (Variables|Default|GetDefaultSceneRoot))
  (Audio|SpawnSoundAttached "/Game/Assets/Audio/SOUNDBANK/SFX/SFX_SHIP/MAINSHIP/MAINSHIP_LOGISTICS/SFX_SHIP_MAINSHIP_Logistics_Station_Fire_LP.SFX_SHIP_MAINSHIP_Logistics_Station_Fire_LP" _defaultsceneroot "None" "0, 0, 0" "0, 0, 0" "KeepRelativeOffset" true 0.8 1.0 0.0 0 0)
  (Effects|SpawnEmitterAttached "/Game/Assets/Particles/P_Post_Fire2.P_Post_Fire2" _defaultsceneroot "None" "0, 0, 0" "0, 0, 0" "0.250000,0.250000,0.250000"))

(fn ConstructionScript)

(fn Extinguish
  (Variables|Default|SetHealth (- (Variables|Default|GetHealth) 2.0))
  (Effects|SpawnEmitterAttached "/Game/Assets/Particles/P_ExtinguisherStatic.P_ExtinguisherStatic" (Variables|Default|GetDefaultSceneRoot) "None" "0, 0, 0" "0, 0, 0" "0.200000,0.200000,0.200000")
  (if (<= (Variables|Default|GetHealth) 0.0)
    (Actor|DestroyActor)))