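; BP_Extinguisher is a fire extinguisher actor that sprays ExtinguisherParticle projectiles while in use.
; UseExtinguisher starts a looping timer at the RoF interval that fires Extinguish, and StopExtinguishing clears it by function name.
; Each Extinguish spawns a particle at the Arrow's location and rotation, adding the Bp_Vaisseau ship's unit forward vector to its projectile velocity.
; GibDatSpit does the same spawn without the velocity adjustment and is not called here.
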(event Custom|UseExtinguisher
  (Utilities|Time|SetTimerbyEvent (delegate Custom|Extinguish) (Variables|Default|GetRoF) true))

(event Custom|Extinguish
  (bind _arrow (Variables|Default|GetArrow))
  (bind _returnvalue (Game|SpawnActorfromClass "/Game/Thibaud/Blueprints/Player/Post/FireFunctionality/ExtinguisherParticle.ExtinguisherParticle_C" (Math|Transform|MakeTransform (Transformation|GetWorldLocation _arrow) (Transformation|GetWorldRotation _arrow) "1,1,1") "Undefined" 0 "0.000000,0.000000,0.000000" 0))
  (bind _returnvalue_2 (Actor|GetActorOfClass "/Game/Thibaud/Blueprints/Player/Bp_Vaisseau.Bp_Vaisseau_C"))
  (Variables|/Script/Engine.MovementComponent|SetVelocity (Variables|/Game/Thibaud/Blueprints/Player/Post/FireFunctionality/ExtinguisherParticle.ExtinguisherParticle_C|GetProjectileMovement _returnvalue) (+ (Variables|/Script/Engine.MovementComponent|GetVelocity (Variables|/Game/Thibaud/Blueprints/Player/Post/FireFunctionality/ExtinguisherParticle.ExtinguisherParticle_C|GetProjectileMovement _returnvalue)) (Math|Vector|GetForwardVector (Variables|/Script/Engine.Actor|GetRootComponent _returnvalue_2)))))

(event Custom|StopExtinguishing
  (Utilities|Time|ClearTimerbyFunctionName self "Extinguish"))

(event EventBeginPlay)

(event Collision|EventActorBeginOverlap
  (params (OtherActor :type Actor%20Object%20Reference)))

(event EventTick
  (params (DeltaSeconds :type Float%20%28single-precision%29)))

(fn ConstructionScript)

(fn GibDatSpit
  (bind _arrow (Variables|Default|GetArrow))
  (Game|SpawnActorfromClass "/Game/Thibaud/Blueprints/Player/Post/FireFunctionality/ExtinguisherParticle.ExtinguisherParticle_C" (Math|Transform|MakeTransform (Transformation|GetWorldLocation _arrow) (Transformation|GetWorldRotation _arrow) "1,1,1") "Undefined" 0 "0.000000,0.000000,0.000000" 0))