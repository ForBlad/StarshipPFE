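; Player starship Blueprint holding helper functions for damage, wall angles, camera shake and circling, with no event logic.
; DamageStack accumulates damage past a threshold, then tries to ignite a random post, re-rolling the index between check and ignition.
; WallDotProduct returns a signed angle from ship forward to a wall, using the right vector for sign.
; Camera shake follows the GameInstance scale, and the circling coefficient oscillates by reversing its delta beyond a limit.
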(fn ConstructionScript)

(fn DamageStack
  (params (Damage :type Float%20%28single-precision%29))
  (bind _allposts (Variables|Default|GetAllPosts))
  (bind _returnvalue (Utilities|Array|Length _allposts))
  (bind _returnvalue_2 (- _returnvalue 1))
  (bind _returnvalue_3 (Math|Random|RandomIntegerinRange 0 _returnvalue_2))
  (bind _output (Utilities|Array|Get(acopy) _allposts _returnvalue_3))
  (Variables|Default|SetAccumulatedDamage (+ (Variables|Default|GetAccumulatedDamage) Damage))
  (if (> (Variables|Default|GetAccumulatedDamage) 2e+02)
    (if (not (Variables|/Game/Thibaud/Blueprints/Player/Post/BPA_Post_Parent.BPA_Post_Parent_C|GetIsOnFire? _output))
      (Default|SetPostonFire _output)
      (Variables|Default|SetAccumulatedDamage 0.0))))

(fn WallDotProduct
  (params (WallLocation :type Vector))
  (bind _returnvalue (Transformation|GetActorLocation))
  (bind _returnvalue_2 (Transformation|GetActorForwardVector))
  (bind _returnvalue_3 (- WallLocation _returnvalue))
  (bind _returnvalue_4 (Math|Vector|Normalize _returnvalue_2))
  (bind _returnvalue_5 (Math|Vector|Normalize _returnvalue_3))
  (bind _returnvalue_6 (Math|Vector|DotProduct _returnvalue_5 _returnvalue_4))
  (bind _returnvalue_7 (Class|KismetMathLibrary|DegAcos _returnvalue_6))
  (if (> (Math|Float|Sign(Float) (Math|Vector|DotProduct (Math|Vector|Normalize _returnvalue_3) (Math|Vector|Normalize (Transformation|GetActorRightVector)))) 0.0)
    (return (* 1 _returnvalue_7))
    (else
      (return (* -1 _returnvalue_7)))))

(fn CameraShake
  (params (Scale :type Float%20%28single-precision%29) (Shake :type Camera%20Shake%20Class%20Reference))
  (Class|PlayerController|ClientPlayCameraShake (Game|GetPlayerController 0) Shake (* Scale (Variables|/Game/Blueprints/StarshipInstance.StarshipInstance_C|GetCameraShakeScale (Variables|Default|GetGameInstance))) "CameraLocal" "0, 0, 0"))

(fn SetCirclingCoefficient
  (params (MinSpeed :type Float%20%28single-precision%29) (MaxSpeed :type Float%20%28single-precision%29) (TurnpointMargin :type Float%20%28single-precision%29) (TimesDeltaPerTick :type Float%20%28single-precision%29) (DeltaTime :type Float%20%28single-precision%29))
  (if (> (Math|Float|Absolute(Float) (Variables|Default|GetCirclingCoefficientGlobal)) (+ MaxSpeed TurnpointMargin))
    (Variables|Default|SetCirclingDeltaGlobal (* (Variables|Default|GetCirclingDeltaGlobal) -1.0))
    (else
      (bind _output_get (Variables|Default|SetCirclingDeltaGlobal (* TimesDeltaPerTick DeltaTime (Math|Float|Sign(Float) (Variables|Default|GetCirclingDeltaGlobal)))))))
  (Variables|Default|SetCirclingCoefficientGlobal (+ _output_get (Variables|Default|GetCirclingCoefficientGlobal))))