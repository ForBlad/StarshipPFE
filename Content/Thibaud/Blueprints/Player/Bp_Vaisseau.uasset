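; Player starship pawn shared by multiple crew: registers with the game instance, creates the HUD and colors players.
; Handles thrust, braking, speed-based hull tilt and spawning of weapon kits.
; Impacts and damage trigger shake and drain Life until explosion and main menu; DamageStack ignites random posts past a decaying threshold.
; Timelines zoom the camera by weapon-post count, with boss variants; old turret, shield and firing logic is disabled.
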(event OnComponentHit(Sphere)
  (params (HitComponent :type Primitive%20Component%20Object%20Reference) (OtherActor :type Actor%20Object%20Reference) (OtherComp :type Primitive%20Component%20Object%20Reference) (NormalImpulse :type Vector :default "0, 0, 0") (Hit :type Hit%20Result%20Structure%20%28by%20ref%29))
  (bind _returnvalue (Transformation|GetVelocity))
  (bind _returnvalue_2 (Transformation|GetVelocity))
  (bind _impactnormal (Collision|BreakHitResult Hit))
  (bind _returnvalue_3 (Math|Vector|VectorLength _returnvalue))
  (bind _returnvalue_4 (Math|Vector|Normalize _impactnormal))
  (bind _returnvalue_5 (Math|Vector|Normalize _returnvalue_2))
  (bind _returnvalue_6 (Math|Vector|RotateVector _returnvalue_5 "0,-90.000000, 0"))
  (bind _returnvalue_7 (Math|Vector|DotProduct _returnvalue_4 _returnvalue_6))
  (bind _returnvalue_8 (Class|KismetMathLibrary|DegAcos _returnvalue_7))
  ;[1 1 1] Wall Impact
  (if (Math|Boolean|ANDBoolean (< _returnvalue_8 135.0) (> _returnvalue_8 45.0) (> _returnvalue_3 (* (Class|MovementComponent|GetMaxSpeed (Variables|Default|GetShip%20Movement)) 0.7)))
    (Utilities|FlowControl|DoOnce false :!label _label
      (:Completed
        (Camera|PlayWorldCameraShake "/Game/Blueprints/CS_Wall_Impact.CS_Wall_Impact_C" (Transformation|GetWorldLocation (Variables|Default|GetCamera1)) 6e+06 9e+06)
        (bind _outactors (Actor|GetAllActorsOfClass "/Script/Engine.Controller"))
        (for _array_element _outactors
          (bind _asplayer_controller (Utilities|Casting|CastToPlayerController _array_element))
          (Game|Feedback|PlayDynamicForceFeedback _asplayer_controller (* _returnvalue_3 0.001) 0.4 true true true true))
        (Audio|PlaySound2D "/Game/Assets/Audio/SoundCues/SC_HittingWall.SC_HittingWall" 1.0 1.0 0.0 0 0)
        (Game|Damage|ApplyDamage self (* _returnvalue_3 0.1) 0 0)
        (Components|Movement|StopMovementImmediately (Variables|Default|GetShip%20Movement))
        (Utilities|FlowControl|Delay 2.0)
        (goto _label Reset)))
    (else
      (bind _outactors_2 (Actor|GetAllActorsOfClass "/Script/Engine.Controller"))
      (for _array_element_2 _outactors_2
        (bind _asplayer_controller_2 (Utilities|Casting|CastToPlayerController _array_element_2))
        (Utilities|FlowControl|Sequence
          (:then_0
            (Game|Feedback|PlayDynamicForceFeedback _asplayer_controller_2 (* _returnvalue_3 0.0003) 0.4 true true true true))
          (:then_1
            (Utilities|FlowControl|DoOnce false :!label _label_2
              (:Completed
                (Class|PlayerController|ClientPlayCameraShake (Game|GetPlayerController 0) "/Game/Blueprints/CS_Wall_Impact.CS_Wall_Impact_C" 0.1 "CameraLocal" "0, 0, 0")
                (Utilities|FlowControl|Delay 0.4)
                (goto _label_2 Reset)))))))))

(event Custom|Acceleration/Decceleration
  (params (AxisValue :type Float%20%28single-precision%29))
  ;[1 1 1] Poste - Pilotage : Mouvement Physique
  (Pawn|Input|AddMovementInput (Transformation|GetActorRightVector) (* 1e+02 AxisValue) true))

(event Custom|BackWard%20Trust
  (params (AxisValue :type Float%20%28single-precision%29))
  (bind _ship_movement (Variables|Default|GetShip%20Movement))
  ;[1 1 1] Poste - Pilotage : Mouvement Physique
  (if (!= AxisValue 0.0)
    (if (>= (Class|KismetMathLibrary|DegAcos (Math|Vector|DotProduct (Math|Vector|Normalize (Variables|/Script/Engine.MovementComponent|GetVelocity _ship_movement)) (Math|Vector|Normalize (Transformation|GetActorRightVector)))) 45.0)
      (if (<= (/ (Math|Vector|VectorLength (Variables|/Script/Engine.MovementComponent|GetVelocity _ship_movement)) (Class|MovementComponent|GetMaxSpeed _ship_movement)) 0.25)
        (Pawn|Input|AddMovementInput (Transformation|GetActorRightVector) (* -1e+01 AxisValue) true))
      (else
        (Variables|/Script/Engine.MovementComponent|SetVelocity (Variables|Default|GetShip%20Movement) (* (Variables|/Script/Engine.MovementComponent|GetVelocity _ship_movement) 0.99))))))

(event Custom|FireCycleAll
  ;[1 1 1] OBSOLETE
  ;;[1 1 1] FIRE SIDE GUNS
  (Development|PrintString "Hello")
  (if (not (<= (Variables|/Game/Thibaud/Blueprints/Player/Post/BPA_Post_Parent.BPA_Post_Parent_C|GetAmmo (stale Custom|Fire/Accelerate Post)) 0.0))
    (Game|SpawnActorfromClass "/Game/Blueprints/Projectiles/BP_ProjectilePlayerSecondary.BP_ProjectilePlayerSecondary_C" (Transformation|GetWorldTransform (Variables|Default|GetS_Post_Arrow)) "AlwaysSpawn" 0 "(R=10.000000,G=0.706065,B=0.000000,A=1.000000)" 0)
    (Variables|/Game/Thibaud/Blueprints/Player/Post/BPA_Post_Parent.BPA_Post_Parent_C|SetAmmo (stale Custom|Fire/Accelerate Post) (- (Variables|/Game/Thibaud/Blueprints/Player/Post/BPA_Post_Parent.BPA_Post_Parent_C|GetAmmo (stale Custom|Fire/Accelerate Post)) 0.0))))

(event Custom|FirecycleRight
  (bind _gmi_starship (Variables|Default|GetGMI_Starship))
  ;[1 1 1] Poste - Arme Auxilliaire : Droite
  (if (not (<= (Variables|/Game/Thibaud/Blueprints/BP_Diverses/BPI_Starship.BPI_Starship_C|GetBullets_Right_wpn (Variables|Default|GetGMI_Starship)) 0.0))
    (Game|SpawnActorfromClass "/Game/Blueprints/Projectiles/BP_ProjectilePlayerSecondary.BP_ProjectilePlayerSecondary_C" (Transformation|GetWorldTransform) "Undefined" 0 "(R=10.000000,G=0.706065,B=0.000000,A=1.000000)" 0)
    (Variables|/Game/Thibaud/Blueprints/BP_Diverses/BPI_Starship.BPI_Starship_C|SetBullets_Right_wpn _gmi_starship (- (Variables|/Game/Thibaud/Blueprints/BP_Diverses/BPI_Starship.BPI_Starship_C|GetBullets_Right_wpn _gmi_starship) 1.0))))

(event Custom|TiltAccordingVelocity
  (bind _ship_hull (Variables|Default|GetShip%20Hull))
  (bind _relativerotation (Variables|/Script/Engine.SceneComponent|GetRelativeRotation _ship_hull))
  (Transformation|SetRelativeRotation _ship_hull (Math|Rotator|MakeRotator (/ (Math|Vector|VectorLength (Variables|/Script/Engine.MovementComponent|GetVelocity (Variables|Default|GetShip%20Movement))) 1.5e+02) (.pitch _relativerotation) (.yaw _relativerotation)) false false))

(event Custom|Fire%20Gatling%20Left
  ;[1 1 1] Poste - Arme Auxilliaire : Gauche
  (Utilities|Time|SetTimerbyEvent (delegate Custom|Firecycle) 0.1 true))

(event Custom|Firecycle
  (bind _gmi_starship (Variables|Default|GetGMI_Starship))
  ;[1 1 1] Poste - Arme Auxilliaire : Gauche
  (if (not (<= (Variables|/Game/Thibaud/Blueprints/BP_Diverses/BPI_Starship.BPI_Starship_C|GetBullets_Left_wpn (Variables|Default|GetGMI_Starship)) 0.0))
    (Game|SpawnActorfromClass "/Game/Blueprints/Projectiles/BP_ProjectilePlayerSecondary.BP_ProjectilePlayerSecondary_C" (Transformation|GetWorldTransform) "Undefined" 0 "(R=10.000000,G=0.706065,B=0.000000,A=1.000000)" 0)
    (Variables|/Game/Thibaud/Blueprints/BP_Diverses/BPI_Starship.BPI_Starship_C|SetBullets_Left_wpn _gmi_starship (- (Variables|/Game/Thibaud/Blueprints/BP_Diverses/BPI_Starship.BPI_Starship_C|GetBullets_Left_wpn _gmi_starship) 1.0))))

(event Custom|LowerDamageStack
  (if (> (Variables|Default|GetAccumulatedDamage) 0.0)
    (Variables|Default|SetAccumulatedDamage (- (Variables|Default|GetAccumulatedDamage) 1.0))))

(event Custom|Create%20Flamethrower%20Kit
  ;[1 0.9163 0.04337] Weapon Creation
  (Game|SpawnActorfromClass "/Game/Thibaud/Blueprints/Kits/BPA_Kits_Flamethrower.BPA_Kits_Flamethrower_C" (Math|Transform|MakeTransform (Transformation|GetWorldLocation (Variables|Default|GetBOX%20SPAWNER)) "0, 0, 0" "1,1,1") "Undefined" 0 0))

(event Custom|Create%20Gatling
  ;[1 0.9163 0.04337] Weapon Creation
  (Game|SpawnActorfromClass "/Game/Thibaud/Blueprints/Kits/BPA_Kits_Gatling.BPA_Kits_Gatling_C" (Math|Transform|MakeTransform (Transformation|GetWorldLocation (Variables|Default|GetBOX%20SPAWNER)) "0, 0, 0" "1,1,1") "Undefined" 0 0))

(event Custom|Create%20Missile
  ;[1 0.9163 0.04337] Weapon Creation
  (Game|SpawnActorfromClass "/Game/Thibaud/Blueprints/Kits/BPA_Kits_Missile.BPA_Kits_Missile_C" (Math|Transform|MakeTransform (Transformation|GetWorldLocation (Variables|Default|GetBOX%20SPAWNER)) "0, 0, 0" "1,1,1") "Undefined" 0 0))

(event Custom|TurnLeft
  (params (AxisValue :type Float%20%28single-precision%29)))

(event Custom|TurnShield
  (params (AxisValue :type Float%20%28single-precision%29))
  ;[1 1 1] Poste - Bouclier
  (if (== AxisValue -1.0)
    (Transformation|AddLocalRotation "0,-1.000000, 0" false false)
    (elif (== AxisValue 1.0)
      (Transformation|AddLocalRotation "0,1.000000, 0" false false))))

(event Custom|Rotate%20Post
  (params (Turn_X :type Float%20%28single-precision%29) (Turn_Y :type Float%20%28single-precision%29) (Post :type BPA%20Post%20Parent%20Object%20Reference))
  (bind _returnvalue (* Turn_X -1.0))
  (bind _returnvalue_2 (* Turn_Y -1.0))
  (bind _returnvalue_3 (* Turn_X 1.0))
  (bind _returnvalue_4 (* Turn_Y -1.0))
  (bind _returnvalue_5 (Math|Vector|MakeVector _returnvalue_3 _returnvalue_4 0.0))
  (bind _returnvalue_6 (Math|Vector|MakeVector _returnvalue_2 _returnvalue 0.0))
  ;[1 1 1] Old & Obsolete
  ;;[1 1 1] assigning mesh to rotate
  (switch int (Variables|/Game/Thibaud/Blueprints/Player/Post/BPA_Post_Parent.BPA_Post_Parent_C|GetPostNumber Post)
    (:0
      ;;[1 1 1] ROTATE SHIP
      (CallFunction|TurnLeft Turn_X))
    (:1
      (Variables|Default|SetS_Post_Mesh 0)
      ;;[1 1 1] ROTATE POST
      (if (and (>= (.Yaw (Math|Rotator|BreakRotator (Variables|/Script/Engine.SceneComponent|GetRelativeRotation (Variables|Default|GetS_Post_Mesh)))) (Variables|/Game/Thibaud/Blueprints/Player/Post/BPA_Post_Parent.BPA_Post_Parent_C|GetMinRotValue Post)) (<= (.Yaw (Math|Rotator|BreakRotator (Variables|/Script/Engine.SceneComponent|GetRelativeRotation (Variables|Default|GetS_Post_Mesh)))) (Variables|/Game/Thibaud/Blueprints/Player/Post/BPA_Post_Parent.BPA_Post_Parent_C|GetMaxRotValue Post))) :!label _label
        (bind _output_get (Variables|/Game/Thibaud/Blueprints/Player/Post/BPA_PostGatlineLeft.BPA_PostGatlineLeft_C|SetLastValidRotation Post (Transformation|GetWorldRotation (Variables|Default|GetS_Post_Mesh))))
        (if (> (Math|Vector|VectorLength _returnvalue_6) 0.2)
          (bind _newtrack_0 (Timeline|TimelineRotatePost PlayFromStart)
            (:Update
              (if (and (>= (.Yaw (Math|Rotator|BreakRotator (Variables|/Script/Engine.SceneComponent|GetRelativeRotation (Variables|Default|GetS_Post_Mesh)))) (Variables|/Game/Thibaud/Blueprints/Player/Post/BPA_Post_Parent.BPA_Post_Parent_C|GetMinRotValue Post)) (<= (.Yaw (Math|Rotator|BreakRotator (Variables|/Script/Engine.SceneComponent|GetRelativeRotation (Variables|Default|GetS_Post_Mesh)))) (Variables|/Game/Thibaud/Blueprints/Player/Post/BPA_Post_Parent.BPA_Post_Parent_C|GetMaxRotValue Post)))
                (Transformation|SetWorldRotation (Variables|Default|GetS_Post_Mesh) (Math|Rotator|Lerp(Rotator) (Transformation|GetWorldRotation (Variables|Default|GetS_Post_Mesh)) (Math|Rotator|MakeRotfromX (Math|Vector|Normalize _returnvalue_6)) _newtrack_0 true) false false)
                (Development|PrintString (Utilities|String|ToString(Float) (.Yaw (Math|Rotator|BreakRotator (Variables|/Script/Engine.SceneComponent|GetRelativeRotation (Variables|Default|GetS_Post_Mesh))))))
                (else
                  (Transformation|SetWorldRotation (Variables|Default|GetS_Post_Mesh) _output_get false false)))))
          (else
            (Timeline|TimelineRotatePost Stop)))))
    (:2
      (Variables|Default|SetS_Post_Mesh 0)
      (goto _label))
    (:3
      (Variables|Default|SetS_Post_Mesh 0)
      (goto _label))
    (:4
      ;;[1 1 1] SPECIAL CASE FOR SHIELD
      (Variables|Default|SetS_Post_Mesh 0)
      (if (> (Math|Vector|VectorLength _returnvalue_5) 0.2)
        (bind _newtrack_0_2 (Timeline|Timeline_0 PlayFromStart)
          (:Update
            (Transformation|SetWorldRotation (Variables|Default|GetS_Post_Mesh) (Math|Rotator|MakeRotator 0.0 0.0 (+ (.yaw (Math|Rotator|Lerp(Rotator) (Transformation|GetWorldRotation (Variables|Default|GetS_Post_Mesh)) (Math|Rotator|MakeRotfromX (Math|Vector|Normalize _returnvalue_5)) _newtrack_0_2 true)) 0.5)) false false)
            (Development|PrintString (Utilities|String|ToString(Float) _returnvalue_3) true true "(R=0.000000,G=0.660000,B=1.000000,A=1.000000)" _returnvalue_3)))
        (else
          (Timeline|Timeline_0 Stop))))))

(event Custom|TurnRightRotation_GatlineRight
  (params (AxisValue :type Float%20%28single-precision%29))
  (bind _relativerotation (Variables|Default|GetRelativeRotation))
  (bind _yaw (Math|Rotator|BreakRotator _relativerotation))
  ;[1 1 1] Poste - Arme Auxilliaire : Droite
  (Development|PrintString (Utilities|String|ToString(Float) _yaw))
  (if (== AxisValue -1.0)
    (if (or (>= _yaw 3.0) false)
      (Transformation|AddLocalRotation "0,-1.000000, 0" false false))
    (elif (== AxisValue 1.0)
      (if (or false (<= _yaw 1.1e+02))
        (Transformation|AddLocalRotation "0,1.000000, 0" false false)))))

(event Custom|LaserTurn
  (bind _gmi_starship (Variables|Default|GetGMI_Starship))
  ;[1 1 1] Poste - Arme Principale
  (if (not (<= (Variables|/Game/Thibaud/Blueprints/BP_Diverses/BPI_Starship.BPI_Starship_C|GetAmmo_left_main_wpn (Variables|Default|GetGMI_Starship)) 0.0))
    (if (not (Variables|Default|GetCanFire?))
      (Game|SpawnActorfromClass "/Game/Blueprints/Projectiles/BP_ProjectilePlayerPrimary.BP_ProjectilePlayerPrimary_C" (Transformation|GetWorldTransform) "Undefined" 0 "(R=0.029012,G=0.850141,B=1.000000,A=0.000000)" 0)
      (Variables|Default|SetCanFire? true)
      (Variables|/Game/Thibaud/Blueprints/BP_Diverses/BPI_Starship.BPI_Starship_C|SetAmmo_left_main_wpn _gmi_starship (- (Variables|/Game/Thibaud/Blueprints/BP_Diverses/BPI_Starship.BPI_Starship_C|GetAmmo_left_main_wpn _gmi_starship) 1.0))
      (Utilities|FlowControl|Delay 0.1)
      (Variables|Default|SetCanFire? false))))

(event Custom|TurnLaser
  (params (AxisValue :type Float%20%28single-precision%29))
  ;[1 1 1] Poste - Arme Principale
  (if (== AxisValue 1.0)
    (Transformation|AddLocalRotation "0,-1.000000, 0" false false)
    (elif (== AxisValue -1.0)
      (Transformation|AddLocalRotation "0,1.000000, 0" false false))))

(event Custom|TurnLeftRotation_GatlineLeft
  (params (AxisValue :type Float%20%28single-precision%29))
  (bind _relativerotation (Variables|Default|GetRelativeRotation))
  (bind _yaw (Math|Rotator|BreakRotator _relativerotation))
  ;[1 1 1] Poste - Arme Auxilliaire : Gauche
  (if (== AxisValue -1.0)
    (if (>= _yaw -9e+01)
      (Transformation|AddLocalRotation "0,-1.000000, 0" false false))
    (elif (== AxisValue 1.0)
      (if (<= _yaw 6.0)
        (Transformation|AddLocalRotation "0,1.000000, 0" false false)))))

(event Custom|Fire/Accelerate
  (params (Post :type BPA%20Post%20Parent%20Object%20Reference))
  ;[1 1 1] OBSOLETE
)

(event Custom|Fire%20Gatling%20Right
  ;[1 1 1] Poste - Arme Auxilliaire : Droite
  (Utilities|Time|SetTimerbyEvent (delegate Custom|FirecycleRight) 0.1 true))

(event EventBeginPlay
  (Utilities|FlowControl|Sequence
    (:then_0
      ;[1 1 1] Event BeginPlay
      (bind _asbpi_starship (Utilities|Casting|CastToBPI_Starship (Game|GetGameInstance)))
      (bind _output_get (Variables|Default|SetGMI_Starship _asbpi_starship))
      (Variables|/Game/Thibaud/Blueprints/BP_Diverses/BPI_Starship.BPI_Starship_C|SetShip _output_get self)
      (Utilities|FlowControl|Sequence
        (:then_0
          (bind _returnvalue (UserInterface|CreateWidget "/Game/Thibaud/Blueprints/Widgets/WG_HUD.WG_HUD_C"))
          (UserInterface|Viewport|AddtoViewport _returnvalue 0)
          (CallFunction|StartCamera)
          (Game|Player|SetViewTargetwithBlend (Game|GetPlayerController 0) self 0.0 "VTBlend_Linear" 0.0 true))))
    (:then_1
      (Utilities|FlowControl|Delay 0.2)
      (bind _outactors (Actor|GetAllActorsOfClass "/Game/Thibaud/Blueprints/Player/BP_Player.BP_Player_C"))
      (for (_array_element _array_index) _outactors
        (bind _output_get_2 (Variables|/Game/Thibaud/Blueprints/Player/BP_Player.BP_Player_C|SetPlayerNumber _array_element _array_index))
        (Rendering|Material|SetMaterial (Variables|/Script/Engine.Character|GetMesh _array_element) 0 (Utilities|Array|Get(acopy) (Variables|/Game/Thibaud/Blueprints/Player/BP_Player.BP_Player_C|GetPlayerColors _array_element) _output_get_2))
        (Rendering|Material|SetMaterial (Variables|/Game/Thibaud/Blueprints/Player/BP_Player.BP_Player_C|GetIdentity%20Circle _array_element) 0 (Utilities|Array|Get(acopy) (Variables|/Game/Thibaud/Blueprints/Player/BP_Player.BP_Player_C|GetCircleColors _array_element) _output_get_2))))
    (:then_2
      (Utilities|Time|SetTimerbyFunctionName 0 "TiltAccordingVelocity" 0.1 true))
    (:then_3
      (Utilities|Time|SetTimerbyEvent (delegate Custom|LowerDamageStack) 0.6 true))))

(event Game|Damage|EventAnyDamage
  (params (Damage :type Float%20%28single-precision%29) (DamageType :type Damage%20Type%20Object%20Reference) (InstigatedBy :type Controller%20Object%20Reference) (DamageCauser :type Actor%20Object%20Reference))
  (bind _returnvalue (Transformation|GetActorLocation))
  ;[1 1 1] Shields
  (Audio|PlaySound2D "/Game/Assets/Audio/SoundCues/SC_HullDamages.SC_HullDamages" 1.0 1.0 0.0 0 0)
  (switch int (Math|Random|RandomInteger 2)
    (:0
      ;[1 1 1] Damages System
      (Camera|PlayWorldCameraShake "/Game/Blueprints/CS_Damage_1.CS_Damage_1_C" (Transformation|GetWorldLocation (Variables|Default|GetCamera1)) 6e+06 9e+06))
    (:1
      (Camera|PlayWorldCameraShake "/Game/Blueprints/CS_Damage_2.CS_Damage_2_C" (Transformation|GetWorldLocation (Variables|Default|GetCamera1)) 6e+06 9e+06)))
  (Variables|Default|SetLife (Math|Float|Clamp(Float) (- (Variables|Default|GetLife) Damage) 0.0 (Variables|Default|GetMax_Life)))
  (if (<= (Variables|Default|GetLife) 2e+02)
    _
    (else
      _))
  (if (<= (Variables|Default|GetLife) 0.0)
    (Effects|SpawnEmitteratLocation "/Game/InfinityBladeEffects/Effects/FX_Mobile/combat/P_Impact_Golem_Gib_Fire.P_Impact_Golem_Gib_Fire" _returnvalue "0, 0, 0" "5.000000,5.000000,5.000000")
    (Audio|PlaySoundatLocation "/Game/Assets/Audio/Explosion.Explosion" _returnvalue "0, 0, 0" 1.0 1.0 0.0 0 0 0)
    (Utilities|FlowControl|Delay 5.0)
    (Game|OpenLevel(byName) "MainMenu")))

(event Input|KeyboardEvents|T
  (params (Key :type Key%20Structure :default "None"))
  (bind _timelinerotatepost (Variables|Default|GetTimelineRotatePost))
  ;[1 1 1] Old & Obsolete
  (:Pressed
    (Utilities|FlowControl|FlipFlop
      (:A
        (Components|Timeline|SetPlayRate _timelinerotatepost 1e+01))
      (:B
        (Components|Timeline|SetPlayRate _timelinerotatepost 1.0)))))

(event Custom|Modification_Camera_No_Have_Weapon
  (bind _gmi_starship (Variables|Default|GetGMI_Starship))
  (bind _gmi_starship_2 (Variables|Default|GetGMI_Starship))
  ;[1 1 1] Zoom Camera
  (if (Variables|Default|GetBoss_Camera)
    (Variables|/Game/Thibaud/Blueprints/BP_Diverses/BPI_Starship.BPI_Starship_C|SetNbre_CheckPost _gmi_starship_2 (- (Variables|/Game/Thibaud/Blueprints/BP_Diverses/BPI_Starship.BPI_Starship_C|GetNbre_CheckPost _gmi_starship_2) 1))
    (if (not (>= (Variables|/Game/Thibaud/Blueprints/BP_Diverses/BPI_Starship.BPI_Starship_C|GetNbre_CheckPost (Variables|Default|GetGMI_Starship)) 1))
      (CallFunction|CameraSetupBossNoWeapon))
    (else
      (Variables|/Game/Thibaud/Blueprints/BP_Diverses/BPI_Starship.BPI_Starship_C|SetNbre_CheckPost _gmi_starship (- (Variables|/Game/Thibaud/Blueprints/BP_Diverses/BPI_Starship.BPI_Starship_C|GetNbre_CheckPost _gmi_starship) 1))
      (if (not (>= (Variables|/Game/Thibaud/Blueprints/BP_Diverses/BPI_Starship.BPI_Starship_C|GetNbre_CheckPost (Variables|Default|GetGMI_Starship)) 1))
        (if (not (Variables|Default|GetBoss_Camera))
          (bind _newtrack_0 (Timeline|Zoom/Dezoom Reverse)
            (:Update
              (Transformation|SetRelativeLocation (Variables|Default|GetCamera1) _newtrack_0 false false))))))))

(event Custom|Modification_Camera_Have_Weapon
  (bind _gmi_starship (Variables|Default|GetGMI_Starship))
  (bind _gmi_starship_2 (Variables|Default|GetGMI_Starship))
  ;[1 1 1] Dezoom_Camera
  (if (Variables|Default|GetBoss_Camera)
    (Variables|/Game/Thibaud/Blueprints/BP_Diverses/BPI_Starship.BPI_Starship_C|SetNbre_CheckPost _gmi_starship (+ (Variables|/Game/Thibaud/Blueprints/BP_Diverses/BPI_Starship.BPI_Starship_C|GetNbre_CheckPost _gmi_starship) 1))
    (if (== (Variables|/Game/Thibaud/Blueprints/BP_Diverses/BPI_Starship.BPI_Starship_C|GetNbre_CheckPost (Variables|Default|GetGMI_Starship)) 1)
      (CallFunction|CameraSetupBoss))
    (else
      (Variables|/Game/Thibaud/Blueprints/BP_Diverses/BPI_Starship.BPI_Starship_C|SetNbre_CheckPost _gmi_starship_2 (+ (Variables|/Game/Thibaud/Blueprints/BP_Diverses/BPI_Starship.BPI_Starship_C|GetNbre_CheckPost _gmi_starship_2) 1))
      (if (not (Variables|Default|GetBoss_Camera))
        (bind _newtrack_0 (Timeline|Zoom/Dezoom Play)
          (:Update
            (Transformation|SetRelativeLocation (Variables|Default|GetCamera1) _newtrack_0 false false)))))))

(event Custom|Start_Camera
  (bind _newtrack_0 (Timeline|Zoom/Dezoom Reverse)
    (:Update
      (Transformation|SetRelativeLocation (Variables|Default|GetCamera1) _newtrack_0 false false))))

(event Custom|Camera%20Setup%20Boss
  (bind _camera1 (Variables|Default|GetCamera1))
  ;[1 1 1] Boss Camera
  (if (Variables|Default|GetSetup%20Camera%20Start)
    (bind _newtrack_0 (Timeline|Timeline_3 PlayFromStart)
      (:Update
        (Transformation|SetRelativeLocation _camera1 _newtrack_0 false false)))
    (else
      (Variables|Default|SetSetup%20Camera%20Start true)
      (bind _newtrack_0_2 (Timeline|Timeline_1 Play)
        (:Update
          (Transformation|SetRelativeLocation _camera1 _newtrack_0_2 false false))))))

(event Custom|Camera%20Setup%20Boss%20No%20Weapon
  ;[1 1 1] Boss Camera
  (bind _newtrack_0 (Timeline|Timeline_2 PlayFromStart)
    (:Update
      (Transformation|SetRelativeLocation (Variables|Default|GetCamera1) _newtrack_0 false false))))

(fn ConstructionScript)

(fn DamageStack
  (params (Damage :type Float%20%28single-precision%29))
  (Variables|Default|SetAccumulatedDamage (+ (Variables|Default|GetAccumulatedDamage) Damage))
  (if (> (Variables|Default|GetAccumulatedDamage) 2e+02)
    (bind _returnvalue (Actor|GetActorOfClass "/Game/Thibaud/Blueprints/Player/BP_Player.BP_Player_C" :!label _label))
    (if (Variables|/Game/Thibaud/Blueprints/Player/Post/BPA_Post_Parent.BPA_Post_Parent_C|GetIsOnFire? (Utilities|Array|Get(acopy) (Variables|/Game/Thibaud/Blueprints/Player/BP_Player.BP_Player_C|GetAllPosts _returnvalue) (Math|Random|RandomIntegerinRange 0 (- (Utilities|Array|Length (Variables|/Game/Thibaud/Blueprints/Player/BP_Player.BP_Player_C|GetAllPosts _returnvalue)) 1))))
      (goto _label)
      (else
        (Default|SetPostonFire (Utilities|Array|Get(acopy) (Variables|/Game/Thibaud/Blueprints/Player/BP_Player.BP_Player_C|GetAllPosts _returnvalue) (Math|Random|RandomIntegerinRange 0 (- (Utilities|Array|Length (Variables|/Game/Thibaud/Blueprints/Player/BP_Player.BP_Player_C|GetAllPosts _returnvalue)) 1))))
        (Variables|Default|SetAccumulatedDamage 0.0)))))

(fn WallDotProduct
  (params (WallLocation :type Vector))
  (bind _returnvalue (Transformation|GetActorLocation))
  (bind _returnvalue_2 (Transformation|GetActorForwardVector))
  (bind _returnvalue_3 (- WallLocation _returnvalue))
  (bind _returnvalue_4 (Math|Vector|Normalize _returnvalue_2))
  (bind _returnvalue_5 (Math|Vector|Normalize _returnvalue_3))
  (bind _returnvalue_6 (Math|Vector|DotProduct _returnvalue_5 _returnvalue_4))
  (bind _returnvalue_7 (Class|KismetMathLibrary|DegAcos _returnvalue_6))
  (if (> (Math|Float|Sign(Float) (Math|Vector|DotProduct (Math|Vector|Normalize _returnvalue_3) (Math|Vector|Normalize (Transformation|GetActorRightVector)))) 0.0)
    (return (* 1 _returnvalue_7))
    (else
      (return (* -1 _returnvalue_7)))))