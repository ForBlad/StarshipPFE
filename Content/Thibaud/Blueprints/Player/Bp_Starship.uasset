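; Player starship pawn with crewed stations: handles piloting input, damage, camera and upgrade kit spawning.
; A looping timer tilts the hull and widens FOV with speed, while fast angled wall hits cause self-damage, shake and pilot rumble.
; Damage drains Life until explosion and return to MainMenu; a separate decaying DamageStack sets random posts on fire past a threshold.
; Station occupancy drives timeline camera zooms, with alternate boss framing.
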(event OnComponentHit(Collision_Ship)
  (params (HitComponent :type Primitive%20Component%20Object%20Reference) (OtherActor :type Actor%20Object%20Reference) (OtherComp :type Primitive%20Component%20Object%20Reference) (NormalImpulse :type Vector :default "0, 0, 0") (Hit :type Hit%20Result%20Structure%20%28by%20ref%29))
  (bind _returnvalue (Transformation|GetVelocity))
  (bind _returnvalue_2 (Transformation|GetVelocity))
  (bind _impactnormal (Collision|BreakHitResult Hit))
  (bind _returnvalue_3 (Math|Vector|VectorLength _returnvalue))
  (bind _returnvalue_4 (Math|Vector|Normalize _impactnormal))
  (bind _returnvalue_5 (Math|Vector|Normalize _returnvalue_2))
  (bind _returnvalue_6 (Math|Vector|RotateVector _returnvalue_5 "0,-90.000000, 0"))
  (bind _returnvalue_7 (Math|Vector|DotProduct _returnvalue_4 _returnvalue_6))
  (bind _returnvalue_8 (Class|KismetMathLibrary|DegAcos _returnvalue_7))
  ;[1 1 1] Piloting - Wall Impact
  (Utilities|Casting|CastToStaticMeshActor OtherActor)
  (if (Math|Boolean|ANDBoolean (< _returnvalue_8 135.0) (> _returnvalue_8 45.0) (> _returnvalue_3 (* (Class|MovementComponent|GetMaxSpeed (Variables|Default|GetShip%20Movement)) 0.7)))
    (Utilities|FlowControl|DoOnce false :!label _label
      (:Completed
        (Class|PlayerController|ClientPlayCameraShake (Game|GetPlayerController 0) "/Game/Blueprints/CS_Wall_Impact.CS_Wall_Impact_C" 1.0 "CameraLocal" "0, 0, 0")
        (Audio|PlaySound2D "/Game/Assets/Audio/SoundCues/SC_HittingWall.SC_HittingWall" 1.0 1.0 0.0 0 0)
        (Game|Damage|ApplyDamage self (* _returnvalue_3 0.1) 0 0)
        (bind _outactors (Actor|GetAllActorsOfClass "/Game/Thibaud/Blueprints/Player/BP_Player.BP_Player_C"))
        (for _array_element _outactors
          (if (Variables|/Game/Thibaud/Blueprints/Player/BP_Player.BP_Player_C|GetIsCurrentlyPilot _array_element)
            (bind _asplayer_controller (Utilities|Casting|CastToPlayerController (Pawn|GetController _array_element)))
            (Game|Feedback|PlayDynamicForceFeedback _asplayer_controller (* _returnvalue_3 0.001) 0.4 true true true true)))
        (Components|Movement|StopMovementImmediately (Variables|Default|GetShip%20Movement))
        (Utilities|FlowControl|Delay 2.0)
        (goto _label Reset)))
    (else
      (Utilities|FlowControl|Sequence
        (:then_0
          (bind _outactors_2 (Actor|GetAllActorsOfClass "/Game/Thibaud/Blueprints/Player/BP_Player.BP_Player_C"))
          (for _array_element_2 _outactors_2
            (if (Variables|/Game/Thibaud/Blueprints/Player/BP_Player.BP_Player_C|GetIsCurrentlyPilot _array_element_2)
              (bind _asplayer_controller_2 (Utilities|Casting|CastToPlayerController (Pawn|GetController _array_element_2)))
              (Game|Feedback|PlayDynamicForceFeedback _asplayer_controller_2 (* _returnvalue_3 0.0003) 0.4 true true true true))))
        (:then_1
          (Utilities|FlowControl|DoOnce false :!label _label_2
            (:Completed
              (Class|PlayerController|ClientPlayCameraShake (Game|GetPlayerController 0) "/Game/Blueprints/CS_Wall_Impact.CS_Wall_Impact_C" 0.1 "CameraLocal" "0, 0, 0")
              (Utilities|FlowControl|Delay 0.4)
              (goto _label_2 Reset))))))))

(event Custom|Acceleration/Decceleration
  (params (AxisValue :type Float%20%28single-precision%29))
  ;[1 1 1] Piloting - Accelerations
  (if (== (stale Custom|BackWard%20Trust AxisValue) 0.0)
    (Pawn|Input|AddMovementInput (Transformation|GetActorRightVector) (* 1e+02 AxisValue) true)))

(event Custom|BackWard%20Trust
  (params (AxisValue :type Float%20%28single-precision%29))
  (bind _ship_movement (Variables|Default|GetShip%20Movement))
  ;[1 1 1] Piloting - Accelerations
  (if (== (stale Custom|Acceleration/Decceleration AxisValue) 0.0)
    (if (!= AxisValue 0.0)
      (if (>= (Class|KismetMathLibrary|DegAcos (Math|Vector|DotProduct (Math|Vector|Normalize (Variables|/Script/Engine.MovementComponent|GetVelocity _ship_movement)) (Math|Vector|Normalize (Transformation|GetActorRightVector)))) 45.0)
        (if (<= (/ (Math|Vector|VectorLength (Variables|/Script/Engine.MovementComponent|GetVelocity _ship_movement)) (Class|MovementComponent|GetMaxSpeed _ship_movement)) 0.25)
          (Pawn|Input|AddMovementInput (Transformation|GetActorRightVector) (* -1e+01 AxisValue) true))
        (else
          (Variables|/Script/Engine.MovementComponent|SetVelocity (Variables|Default|GetShip%20Movement) (* (Variables|/Script/Engine.MovementComponent|GetVelocity _ship_movement) 0.99)))))))

(event Custom|TiltAccordingVelocity
  (bind _ship_hull (Variables|Default|GetShip%20Hull))
  (bind _ship_movement (Variables|Default|GetShip%20Movement))
  (bind _returnvalue (Class|MovementComponent|GetMaxSpeed _ship_movement))
  (bind _velocity (Variables|/Script/Engine.MovementComponent|GetVelocity _ship_movement))
  (bind _relativerotation (Variables|/Script/Engine.SceneComponent|GetRelativeRotation _ship_hull))
  (bind _returnvalue_2 (Math|Vector|VectorLength _velocity))
  (bind _returnvalue_3 (/ _returnvalue_2 _returnvalue))
  ;[1 1 1] Piloting - Tilt & FoV change by velocity
  (Transformation|SetRelativeRotation _ship_hull (Math|Rotator|MakeRotator (* _returnvalue_3 3.5) (.pitch _relativerotation) (.yaw _relativerotation)) false false)
  (Camera|SetFieldOfView (Variables|Default|GetCamera1) (+ (* _returnvalue_3 15.0) 1e+02)))

(event Custom|LowerDamageStack
  (if (> (Variables|Default|GetAccumulatedDamage) 0.0)
    (Variables|Default|SetAccumulatedDamage (- (Variables|Default|GetAccumulatedDamage) 1.0))))

(event Custom|Create%20Flamethrower%20Kit
  ;[1 0.9163 0.04337] Spawn upgrade Kits
  (Game|SpawnActorfromClass "/Game/Thibaud/Blueprints/Kits/BPA_Kits_Flamethrower.BPA_Kits_Flamethrower_C" (Math|Transform|MakeTransform (Transformation|GetWorldLocation (Variables|Default|GetRespawn_Position)) "0, 0, 0" "1,1,1") "Undefined" 0 0))

(event Custom|Create%20Gatling
  ;[1 0.9163 0.04337] Spawn upgrade Kits
  (Game|SpawnActorfromClass "/Game/Thibaud/Blueprints/Kits/BPA_Kits_Gatling.BPA_Kits_Gatling_C" (Math|Transform|MakeTransform (Transformation|GetWorldLocation (Variables|Default|GetRespawn_Position)) "0, 0, 0" "1,1,1") "Undefined" 0 0))

(event Custom|Create%20Missile
  ;[1 0.9163 0.04337] Spawn upgrade Kits
  (Game|SpawnActorfromClass "/Game/Thibaud/Blueprints/Kits/BPA_Kits_Missile.BPA_Kits_Missile_C" (Math|Transform|MakeTransform (Transformation|GetWorldLocation (Variables|Default|GetRespawn_Position)) "0, 0, 0" "1,1,1") "Undefined" 0 0))

(event EventBeginPlay
  (Utilities|FlowControl|Sequence
    (:then_0
      ;[1 1 1] Event BeginPlay
      (bind _returnvalue (UserInterface|CreateWidget "/Game/Thibaud/Blueprints/Widgets/WG_HUD.WG_HUD_C"))
      (UserInterface|Viewport|AddtoViewport _returnvalue 0)
      (CallFunction|StartCamera)
      (Game|Player|SetViewTargetwithBlend (Game|GetPlayerController 0) self 0.0 "VTBlend_Linear" 0.0 true))
    (:then_1
      (Utilities|Time|SetTimerbyFunctionName 0 "TiltAccordingVelocity" 0.01 true)
      (Utilities|Time|SetTimerbyEvent (delegate Custom|LowerDamageStack) 0.6 true))))

(event Game|Damage|EventAnyDamage
  (params (Damage :type Float%20%28single-precision%29) (DamageType :type Damage%20Type%20Object%20Reference) (InstigatedBy :type Controller%20Object%20Reference) (DamageCauser :type Actor%20Object%20Reference))
  (bind _returnvalue (Transformation|GetActorLocation))
  (bind _camera1 (Variables|Default|GetCamera1))
  (bind _returnvalue_2 (Transformation|GetWorldLocation _camera1))
  ;[1 1 1] Damage System
  (Audio|PlaySound2D "/Game/Assets/Audio/SoundCues/SC_HullDamages.SC_HullDamages" 1.0 1.0 0.0 0 0)
  (switch int (Math|Random|RandomInteger 2)
    (:0
      (Camera|PlayWorldCameraShake "/Game/Blueprints/CS_Damage_1.CS_Damage_1_C" _returnvalue_2 6e+06 9e+06))
    (:1
      (Camera|PlayWorldCameraShake "/Game/Blueprints/CS_Damage_2.CS_Damage_2_C" _returnvalue_2 6e+06 9e+06)))
  (Variables|Default|SetLife (Math|Float|Clamp(Float) (- (Variables|Default|GetLife) Damage) 0.0 (Variables|Default|GetMax_Life)))
  (if (<= (Variables|Default|GetLife) 0.0)
    (Effects|SpawnEmitteratLocation "/Game/InfinityBladeEffects/Effects/FX_Mobile/combat/P_Impact_Golem_Gib_Fire.P_Impact_Golem_Gib_Fire" _returnvalue "0, 0, 0" "5.000000,5.000000,5.000000")
    (Audio|PlaySoundatLocation "/Game/Assets/Audio/Explosion.Explosion" _returnvalue "0, 0, 0" 1.0 1.0 0.0 0 0 0)
    (Utilities|FlowControl|Delay 5.0)
    (Game|OpenLevel(byName) "MainMenu")))

(event Custom|StationsManned--
  (bind _stationsinuse (Variables|Default|GetStationsInUse))
  ;[1 1 1] Player Left Station
  (Math|Integer|DecrementInt _stationsinuse
    (:%20%20
      (if (not (> _stationsinuse 0))
        (if (Variables|Default|GetBoss_Camera)
          ;[1 1 1] Boss Camera
          (bind _newtrack_0 (Timeline|Timeline_2 Play)
            (:Update
              (Transformation|SetRelativeLocation (Variables|Default|GetCamera1) _newtrack_0 false false)))
          (else
            ;[1 1 1] Standard Camera
            (bind _newtrack_0_2 (Timeline|Zoom/Dezoom Reverse)
              (:Update
                (Transformation|SetRelativeLocation (Variables|Default|GetCamera1) _newtrack_0_2 false false)))))))))

(event Custom|StationsManned++
  (bind _stationsinuse (Variables|Default|GetStationsInUse))
  (bind _camera1 (Variables|Default|GetCamera1))
  ;[1 1 1] Player Entered Station
  (Math|Integer|IncrementInt _stationsinuse
    (:%20%20
      (if (Variables|Default|GetBoss_Camera)
        (if (== _stationsinuse 1)
          (if (Variables|Default|GetSetup%20Camera%20Start)
            ;[1 1 1] Boss Camera
            (bind _newtrack_0 (Timeline|Timeline_3 PlayFromStart)
              (:Update
                (Transformation|SetRelativeLocation _camera1 _newtrack_0 false false)))
            (else
              (Variables|Default|SetSetup%20Camera%20Start true)
              (bind _newtrack_0_2 (Timeline|Timeline_1 Play)
                (:Update
                  (Transformation|SetRelativeLocation _camera1 _newtrack_0_2 false false))))))
        (else
          ;[1 1 1] Standard Camera
          (bind _newtrack_0_3 (Timeline|Zoom/Dezoom Play)
            (:Update
              (Transformation|SetRelativeLocation (Variables|Default|GetCamera1) _newtrack_0_3 false false))))))))

(event Custom|Start_Camera
  ;[1 1 1] Game Start
  ;[1 1 1] Standard Camera
  (bind _newtrack_0 (Timeline|Zoom/Dezoom ReverseFromEnd)
    (:Update
      (Transformation|SetRelativeLocation (Variables|Default|GetCamera1) _newtrack_0 false false))))

(fn ConstructionScript)

(fn DamageStack
  (params (Damage :type Float%20%28single-precision%29))
  (Variables|Default|SetAccumulatedDamage (+ (Variables|Default|GetAccumulatedDamage) Damage))
  (if (> (Variables|Default|GetAccumulatedDamage) 2e+02)
    (bind _returnvalue (Actor|GetActorOfClass "/Game/Thibaud/Blueprints/Player/BP_Player.BP_Player_C" :!label _label))
    (if (Variables|/Game/Thibaud/Blueprints/Player/Post/BPA_Post_Parent.BPA_Post_Parent_C|GetIsOnFire? (Utilities|Array|Get(acopy) (Variables|/Game/Thibaud/Blueprints/Player/BP_Player.BP_Player_C|GetAllPosts _returnvalue) (Math|Random|RandomIntegerinRange 0 (- (Utilities|Array|Length (Variables|/Game/Thibaud/Blueprints/Player/BP_Player.BP_Player_C|GetAllPosts _returnvalue)) 1))))
      (goto _label)
      (else
        (Default|SetPostonFire (Utilities|Array|Get(acopy) (Variables|/Game/Thibaud/Blueprints/Player/BP_Player.BP_Player_C|GetAllPosts _returnvalue) (Math|Random|RandomIntegerinRange 0 (- (Utilities|Array|Length (Variables|/Game/Thibaud/Blueprints/Player/BP_Player.BP_Player_C|GetAllPosts _returnvalue)) 1))))
        (Variables|Default|SetAccumulatedDamage 0.0)))))

(fn WallDotProduct
  (params (WallLocation :type Vector))
  (bind _returnvalue (Transformation|GetActorLocation))
  (bind _returnvalue_2 (Transformation|GetActorForwardVector))
  (bind _returnvalue_3 (- WallLocation _returnvalue))
  (bind _returnvalue_4 (Math|Vector|Normalize _returnvalue_2))
  (bind _returnvalue_5 (Math|Vector|Normalize _returnvalue_3))
  (bind _returnvalue_6 (Math|Vector|DotProduct _returnvalue_5 _returnvalue_4))
  (bind _returnvalue_7 (Class|KismetMathLibrary|DegAcos _returnvalue_6))
  (if (> (Math|Float|Sign(Float) (Math|Vector|DotProduct (Math|Vector|Normalize _returnvalue_3) (Math|Vector|Normalize (Transformation|GetActorRightVector)))) 0.0)
    (return (* 1 _returnvalue_7))
    (else
      (return (* -1 _returnvalue_7)))))