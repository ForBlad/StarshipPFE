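; Player starship pawn with stations for piloting, a main laser, two auxiliary gatlings and a rotatable shield.
; Inputs move and rotate the ship and turrets; the delay-gated laser and timer-looped gatlings spawn projectiles using ammo stored in the BPI_Starship game instance.
; Damage shakes the camera and lowers Life; a destruction event explodes the ship and loads MainMenu.
; An occupied-post counter drives timeline camera zooms, with separate boss framing.
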(event Custom|Acceleration/Decceleration
  (params (AxisValue :type Float%20%28single-precision%29))
  ;[1 1 1] Poste - Pilotage : Mouvement Physique
  (Pawn|Input|AddMovementInput (Transformation|GetActorRightVector) AxisValue true))

(event Custom|BackWard%20Trust
  (params (Axis%20Value :type Float%20%28single-precision%29))
  ;[1 1 1] Poste - Pilotage : Mouvement Physique
  (Pawn|Input|AddMovementInput (Transformation|GetActorRightVector) Axis%20Value true))

(event Custom|FirecycleRight
  (bind _wpn_right_prjctls_spawn (Variables|Default|GetWpn_right_prjctls_spawn))
  (bind _gmi_starship (Variables|Default|GetGMI_Starship))
  ;[1 1 1] Poste - Arme Auxilliaire : Droite
  (if (<= (Variables|/Game/Thibaud/Blueprints/BP_Diverses/BPI_Starship.BPI_Starship_C|GetBullets_Right_wpn (Variables|Default|GetGMI_Starship)) 0.0)
    (Utilities|Time|ClearTimerbyFunctionName 0 "FirecycleRight")
    (else
      (Effects|SpawnEmitterAttached "/Game/InfinityBladeEffects/Effects/FX_Monsters/FX_Monster_Gruntling/Master/P_BackPack_MuzzleFlash.P_BackPack_MuzzleFlash" _wpn_right_prjctls_spawn "None" "0, 0, 0" "0, 0, 0" "0.300000,0.300000,0.300000")
      (Game|SpawnActorfromClass "/Game/Thibaud/Blueprints/Player/Balles/BPA_Balles.BPA_Balles_C" (Transformation|GetWorldTransform _wpn_right_prjctls_spawn) "Undefined" 0 0)
      (Audio|PlaySoundatLocation "/Game/Assets/Audio/EnemyShot.EnemyShot" "0, 0, 0" "0, 0, 0" 1.0 1.0 0.0 0 0 0)
      (Variables|/Game/Thibaud/Blueprints/BP_Diverses/BPI_Starship.BPI_Starship_C|SetBullets_Right_wpn _gmi_starship (- (Variables|/Game/Thibaud/Blueprints/BP_Diverses/BPI_Starship.BPI_Starship_C|GetBullets_Right_wpn _gmi_starship) 1.0)))))

(event Custom|Fire%20Gatling%20Left
  ;[1 1 1] Poste - Arme Auxilliaire : Gauche
  (Utilities|Time|SetTimerbyEvent (delegate Custom|Firecycle) 0.1 true))

(event Custom|Firecycle
  (bind _wpn_left_prjctls_spawn (Variables|Default|GetWpn_left_prjctls_spawn))
  (bind _gmi_starship (Variables|Default|GetGMI_Starship))
  ;[1 1 1] Poste - Arme Auxilliaire : Gauche
  (if (<= (Variables|/Game/Thibaud/Blueprints/BP_Diverses/BPI_Starship.BPI_Starship_C|GetBullets_Left_wpn (Variables|Default|GetGMI_Starship)) 0.0)
    (Utilities|Time|ClearTimerbyFunctionName 0 "Firecycle")
    (else
      (Effects|SpawnEmitterAttached "/Game/InfinityBladeEffects/Effects/FX_Monsters/FX_Monster_Gruntling/Master/P_BackPack_MuzzleFlash.P_BackPack_MuzzleFlash" _wpn_left_prjctls_spawn "None" "0, 0, 0" "0, 0, 0" "0.300000,0.300000,0.300000")
      (Game|SpawnActorfromClass "/Game/Blueprints/Projectiles/BP_ProjectilePlayerSecondary.BP_ProjectilePlayerSecondary_C" (Transformation|GetWorldTransform _wpn_left_prjctls_spawn) "Undefined" 0 "(R=10.000000,G=0.706065,B=0.000000,A=1.000000)" 0)
      (Audio|PlaySoundatLocation "/Game/Assets/Audio/EnemyShot.EnemyShot" "0, 0, 0" "0, 0, 0" 1.0 1.0 0.0 0 0 0)
      (Variables|/Game/Thibaud/Blueprints/BP_Diverses/BPI_Starship.BPI_Starship_C|SetBullets_Left_wpn _gmi_starship (- (Variables|/Game/Thibaud/Blueprints/BP_Diverses/BPI_Starship.BPI_Starship_C|GetBullets_Left_wpn _gmi_starship) 1.0)))))

(event Custom|TurnLeft
  (params (AxisValue :type Float%20%28single-precision%29))
  (bind _returnvalue (>= AxisValue 0.1))
  ;[1 1 1] Poste - Pilotage : Rotation
  (if _returnvalue
    (Transformation|AddActorLocalRotation "0,-1.000000,0.000000" false false)
    (else
      (Utilities|Time|ClearTimerbyFunctionName 0 "ShipRollLeft")
      (if (not _returnvalue)
        (Transformation|AddActorLocalRotation "0,1.000000, 0" false false)))))

(event Custom|TurnShield
  (params (AxisValue :type Float%20%28single-precision%29))
  (bind _shield_active (Variables|Default|GetShield_active))
  ;[1 1 1] Poste - Bouclier
  (if (== AxisValue -1.0)
    (Transformation|AddLocalRotation _shield_active "0,-1.000000, 0" false false)
    (elif (== AxisValue 1.0)
      (Transformation|AddLocalRotation _shield_active "0,1.000000, 0" false false))))

(event Custom|TurnRightRotation_GatlineRight
  (params (AxisValue :type Float%20%28single-precision%29))
  (bind _wpn_right_gatling (Variables|Default|GetWpn_right_gatling))
  (bind _relativerotation (Variables|/Script/Engine.SceneComponent|GetRelativeRotation _wpn_right_gatling))
  (bind _yaw (Math|Rotator|BreakRotator _relativerotation))
  ;[1 1 1] Poste - Arme Auxilliaire : Droite
  (if (== AxisValue -1.0)
    (if (or (>= _yaw 3.0) (<= _yaw 0.0))
      (Transformation|AddLocalRotation (Variables|Default|GetWpn_right_gatling) "0,-1.000000, 0" false false))
    (elif (== AxisValue 1.0)
      (if (or false (<= _yaw 1.1e+02))
        (Transformation|AddLocalRotation (Variables|Default|GetWpn_right_gatling) "0,1.000000, 0" false false)))))

(event Custom|LaserTurn
  (bind _gmi_starship (Variables|Default|GetGMI_Starship))
  (bind _wpn_main_prjctls_spawn (Variables|Default|GetWpn_main_prjctls_spawn))
  ;[1 1 1] Poste - Arme Principale
  (if (not (<= (Variables|/Game/Thibaud/Blueprints/BP_Diverses/BPI_Starship.BPI_Starship_C|GetAmmo_left_main_wpn (Variables|Default|GetGMI_Starship)) 0.0))
    (if (not (Variables|Default|GetCanFire?))
      (Game|SpawnActorfromClass "/Game/Thibaud/Blueprints/Player/Balles/BPA_Balles_Laser.BPA_Balles_Laser_C" (Transformation|GetWorldTransform _wpn_main_prjctls_spawn) "Undefined" 0 0)
      (Effects|SpawnEmitteratLocation "/Game/Léa/FX/Particle/P_Muzzle_laser.P_Muzzle_laser" (Transformation|GetWorldLocation _wpn_main_prjctls_spawn))
      (Variables|Default|SetCanFire? true)
      (Variables|/Game/Thibaud/Blueprints/BP_Diverses/BPI_Starship.BPI_Starship_C|SetAmmo_left_main_wpn _gmi_starship (- (Variables|/Game/Thibaud/Blueprints/BP_Diverses/BPI_Starship.BPI_Starship_C|GetAmmo_left_main_wpn _gmi_starship) 1.0))
      (Utilities|FlowControl|Delay 1.0)
      (Variables|Default|SetCanFire? false))))

(event Custom|TurnLaser
  (params (AxisValue :type Float%20%28single-precision%29))
  ;[1 1 1] Poste - Arme Principale
  (if (== AxisValue 1.0)
    (Transformation|AddLocalRotation (Variables|Default|GetWpn_main_lasgun) "0,-1.000000, 0" false false)
    (elif (== AxisValue -1.0)
      (Transformation|AddLocalRotation (Variables|Default|GetWpn_main_lasgun) "0,1.000000, 0" false false))))

(event Custom|TurnLeftRotation_GatlineLeft
  (params (AxisValue :type Float%20%28single-precision%29))
  (bind _wpn_left_gatling (Variables|Default|GetWpn_left_gatling))
  (bind _relativerotation (Variables|/Script/Engine.SceneComponent|GetRelativeRotation _wpn_left_gatling))
  (bind _yaw (Math|Rotator|BreakRotator _relativerotation))
  ;[1 1 1] Poste - Arme Auxilliaire : Gauche
  (if (== AxisValue -1.0)
    (if (>= _yaw -9e+01)
      (Transformation|AddLocalRotation (Variables|Default|GetWpn_left_gatling) "0,-1.000000, 0" false false))
    (elif (== AxisValue 1.0)
      (if (<= _yaw 5.0)
        (Transformation|AddLocalRotation (Variables|Default|GetWpn_left_gatling) "0,1.000000, 0" false false)))))

(event Custom|Destroy_Vaisseau
  (bind _returnvalue (Transformation|GetActorLocation))
  ;[1 1 1] Damages System
  (if (<= (Variables|Default|GetLife) 0.0)
    (Effects|SpawnEmitteratLocation "/Game/InfinityBladeEffects/Effects/FX_Mobile/combat/P_Impact_Golem_Gib_Fire.P_Impact_Golem_Gib_Fire" _returnvalue "0, 0, 0" "5.000000,5.000000,5.000000")
    (Audio|PlaySoundatLocation "/Game/Assets/Audio/Explosion.Explosion" _returnvalue "0, 0, 0" 1.0 1.0 0.0 0 0 0)
    (Variables|Default|SetDeath true)
    (Utilities|FlowControl|Delay 5.0)
    (Game|OpenLevel(byName) "MainMenu")))

(event Custom|Fire%20Gatling%20Right
  ;[1 1 1] Poste - Arme Auxilliaire : Droite
  (Utilities|Time|SetTimerbyEvent (delegate Custom|FirecycleRight) 0.1 true))

(event EventBeginPlay
  ;[1 1 1] Event BeginPlay
  (bind _asbpi_starship (Utilities|Casting|CastToBPI_Starship (Game|GetGameInstance)))
  (Variables|Default|SetGMI_Starship _asbpi_starship)
  (bind _returnvalue (UserInterface|CreateWidget "/Game/Thibaud/Blueprints/Widgets/WG_HUD.WG_HUD_C"))
  (UserInterface|Viewport|AddtoViewport _returnvalue 0)
  (CallFunction|StartCamera)
  (Game|Player|SetViewTargetwithBlend (Game|GetPlayerController 0) self 0.0 "VTBlend_Linear" 0.0 true))

(event Game|Damage|EventAnyDamage
  (params (Damage :type Float%20%28single-precision%29) (DamageType :type Damage%20Type%20Object%20Reference) (InstigatedBy :type Controller%20Object%20Reference) (DamageCauser :type Actor%20Object%20Reference))
  ;[1 1 1] Shields
  (Audio|PlaySoundatLocation "/Game/Assets/Audio/impact-laser-free-sound-effect-_AudioTrimmer_com_-_AudioTrimmer_com_.impact-laser-free-sound-effect-_AudioTrimmer_com_-_AudioTrimmer_com_" "0, 0, 0" "0, 0, 0" 1.0 1.0 0.0 0 0 0)
  (switch int (Math|Random|RandomInteger 2)
    (:0
      ;[1 1 1] Damages System
      (Camera|PlayWorldCameraShake "/Game/Blueprints/Camera_Shake1.Camera_Shake1_C" (Transformation|GetWorldLocation (Variables|Default|GetCamera1)) 6e+06 9e+06))
    (:1
      (Camera|PlayWorldCameraShake "/Game/Blueprints/Camera_Shake2.Camera_Shake2_C" (Transformation|GetWorldLocation (Variables|Default|GetCamera1)) 6e+06 9e+06)))
  (Variables|Default|SetLife (Math|Float|Clamp(Float) (- (Variables|Default|GetLife) Damage) 0.0 (Variables|Default|GetMax_Life))))

(event Custom|Modification_Camera_No_Have_Weapon
  (bind _gmi_starship (Variables|Default|GetGMI_Starship))
  (bind _gmi_starship_2 (Variables|Default|GetGMI_Starship))
  ;[1 1 1] Zoom Camera
  (Development|PrintString "Quand le joueur est sur un vaisseau")
  (if (Variables|Default|GetBoss_Camera)
    (Variables|/Game/Thibaud/Blueprints/BP_Diverses/BPI_Starship.BPI_Starship_C|SetNbre_CheckPost _gmi_starship_2 (- (Variables|/Game/Thibaud/Blueprints/BP_Diverses/BPI_Starship.BPI_Starship_C|GetNbre_CheckPost _gmi_starship_2) 1))
    (if (not (>= (Variables|/Game/Thibaud/Blueprints/BP_Diverses/BPI_Starship.BPI_Starship_C|GetNbre_CheckPost (Variables|Default|GetGMI_Starship)) 1))
      (CallFunction|CameraSetupBossNoWeapon))
    (else
      (Variables|/Game/Thibaud/Blueprints/BP_Diverses/BPI_Starship.BPI_Starship_C|SetNbre_CheckPost _gmi_starship (- (Variables|/Game/Thibaud/Blueprints/BP_Diverses/BPI_Starship.BPI_Starship_C|GetNbre_CheckPost _gmi_starship) 1))
      (if (not (>= (Variables|/Game/Thibaud/Blueprints/BP_Diverses/BPI_Starship.BPI_Starship_C|GetNbre_CheckPost (Variables|Default|GetGMI_Starship)) 1))
        (if (not (Variables|Default|GetBoss_Camera))
          (bind _newtrack_0 (Timeline|Zoom/Dezoom Reverse)
            (:Update
              (Transformation|SetRelativeLocation (Variables|Default|GetCamera1) _newtrack_0 false false))))))))

(event Custom|Modification_Camera_Have_Weapon
  (bind _gmi_starship (Variables|Default|GetGMI_Starship))
  (bind _gmi_starship_2 (Variables|Default|GetGMI_Starship))
  ;[1 1 1] Dezoom_Camera
  (if (Variables|Default|GetBoss_Camera)
    (Variables|/Game/Thibaud/Blueprints/BP_Diverses/BPI_Starship.BPI_Starship_C|SetNbre_CheckPost _gmi_starship (+ (Variables|/Game/Thibaud/Blueprints/BP_Diverses/BPI_Starship.BPI_Starship_C|GetNbre_CheckPost _gmi_starship) 1))
    (if (== (Variables|/Game/Thibaud/Blueprints/BP_Diverses/BPI_Starship.BPI_Starship_C|GetNbre_CheckPost (Variables|Default|GetGMI_Starship)) 1)
      (CallFunction|CameraSetupBoss))
    (else
      (Variables|/Game/Thibaud/Blueprints/BP_Diverses/BPI_Starship.BPI_Starship_C|SetNbre_CheckPost _gmi_starship_2 (+ (Variables|/Game/Thibaud/Blueprints/BP_Diverses/BPI_Starship.BPI_Starship_C|GetNbre_CheckPost _gmi_starship_2) 1))
      (Development|PrintString "Quand le joueur est sur un vaisseau")
      (if (not (Variables|Default|GetBoss_Camera))
        (bind _newtrack_0 (Timeline|Zoom/Dezoom Play)
          (:Update
            (Transformation|SetRelativeLocation (Variables|Default|GetCamera1) _newtrack_0 false false)))))))

(event Custom|Start_Camera
  (bind _newtrack_0 (Timeline|Zoom/Dezoom Reverse)
    (:Update
      (Transformation|SetRelativeLocation (Variables|Default|GetCamera1) _newtrack_0 false false))))

(event Custom|Camera%20Setup%20Boss
  (bind _camera1 (Variables|Default|GetCamera1))
  ;[1 1 1] Boss Camera
  (if (Variables|Default|GetSetup%20Camera%20Start)
    (bind _newtrack_0 (Timeline|Timeline_3 PlayFromStart)
      (:Update
        (Transformation|SetRelativeLocation _camera1 _newtrack_0 false false)))
    (else
      (Variables|Default|SetSetup%20Camera%20Start true)
      (bind _newtrack_0_2 (Timeline|Timeline_1 Play)
        (:Update
          (Transformation|SetRelativeLocation _camera1 _newtrack_0_2 false false))))))

(event Custom|Camera%20Setup%20Boss%20No%20Weapon
  ;[1 1 1] Boss Camera
  (bind _newtrack_0 (Timeline|Timeline_2 PlayFromStart)
    (:Update
      (Transformation|SetRelativeLocation (Variables|Default|GetCamera1) _newtrack_0 false false))))

(fn ConstructionScript)