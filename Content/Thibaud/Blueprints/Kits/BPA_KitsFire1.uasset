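; BPA_KitsFire1 is a fire extinguisher pickup that BP_Player can carry, drop and spray to put out BPA_Fire actors.
; Items alternates via FlipFlop between attaching the mesh to the player's Pickup without physics and releasing it with physics.
; UseItems starts a looping timer that, while UseFireExtinc holds, drains Stock and sphere-traces a short distance forward, calling Elimination on fires hit.
; The actor destroys itself once Stock runs out.
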(event Custom|Delete
  (if (== (Variables|Default|GetStock) 0.0)
    (Actor|DestroyActor)))

(event Custom|UseFireExtinceur
  (bind _scene1 (Variables|Default|GetScene1))
  (bind _returnvalue (Transformation|GetWorldLocation _scene1))
  (if (Variables|/Game/Thibaud/Blueprints/Player/BP_Player.BP_Player_C|GetUseFireExtinc (stale EventUseItems _asbp_player))
    (if (<= (Variables|Default|GetStock) 0.0)
      (Actor|DestroyActor)
      (else
        (Variables|Default|SetStock (- (Variables|Default|GetStock) 1.0))
        (bind (_outhit _returnvalue_2) (Collision|SphereTraceByChannel _returnvalue (+ _returnvalue (* (Math|Vector|GetForwardVector _scene1) 5.0)) 2.0 "TraceTypeQuery1" false (Utilities|Array|MakeArray self) "ForDuration"))
        (if _returnvalue_2
          (bind _asbpa_fire (Utilities|Casting|CastToBPA_Fire (.HitActor (Collision|BreakHitResult _outhit))))
          (Default|Elimination _asbpa_fire))))
    (else
      (Utilities|Time|ClearTimerbyFunctionName self "UseFireExtinceur"))))

(event EventUseItems
  (params (Character :type Character%20Object%20Reference))
  (bind _asbp_player (Utilities|Casting|CastToBP_Player Character))
  (Utilities|Time|SetTimerbyEvent (delegate Custom|UseFireExtinceur) 0.1 true))

(event EventItems
  (params (Character :type Character%20Object%20Reference))
  (bind _sm_fire (Variables|Default|GetSM_Fire))
  (bind _sm_fire_2 (Variables|Default|GetSM_Fire))
  (bind _asbp_player (Utilities|Casting|CastToBP_Player Character))
  (Utilities|FlowControl|FlipFlop
    (:A
      (Transformation|AttachComponentToComponent (Variables|Default|GetSM_Fire) (Variables|/Game/Thibaud/Blueprints/Player/BP_Player.BP_Player_C|GetPickup _asbp_player) "None" "SnapToTarget" "SnapToTarget" "SnapToTarget" true)
      (Class|PrimitiveComponent|SetConstraintMode _sm_fire "XYPlane")
      (Physics|SetSimulatePhysics _sm_fire false)
      (Variables|/Game/Thibaud/Blueprints/Player/BP_Player.BP_Player_C|SetKitsFireExtinc? _asbp_player true))
    (:B
      (Transformation|AttachComponentToComponent (Variables|Default|GetSM_Fire) 0 "None" "SnapToTarget" "SnapToTarget" "SnapToTarget" true)
      (Class|PrimitiveComponent|SetConstraintMode _sm_fire_2 "Default")
      (Physics|SetSimulatePhysics _sm_fire_2 true)
      (Variables|/Game/Thibaud/Blueprints/Player/BP_Player.BP_Player_C|SetKitsFireExtinc? _asbp_player false))))

(event EventBeginPlay
  (Utilities|Time|SetTimerbyEvent (delegate Custom|Delete) 0.1 true))

(fn ConstructionScript)