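; Parent Blueprint for the kits (ammo, upgrade, extinguisher) that players carry around the starship.
; Pick/DropItem attaches the kit to the player's hand or throws it with a physics impulse, destroying near-empty extinguishers.
; Holder overlaps track nearby posts to toggle their hatches, and respawn upgrade and extinguisher kits that leave the ship.
; Child-specific rules live here through self-casts, alongside tooltip icon visibility and post list cleanup on destruction.
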(event OnComponentBeginOverlap(Holder)
  (params (OverlappedComponent :type Primitive%20Component%20Object%20Reference) (OtherActor :type Actor%20Object%20Reference) (OtherComp :type Primitive%20Component%20Object%20Reference) (OtherBodyIndex :type Integer) (bFromSweep :type Boolean) (SweepResult :type Hit%20Result%20Structure%20%28by%20ref%29))
  (bind _self self)
  ;[1 1 1] Ammo Hatch Animation
  (bind (_post _ispost_) (CallFunction|IsStationOfDifferentType OtherActor))
  (if _ispost_
    (Utilities|Array|Add (Variables|Default|GetOverlappedStations) _post)
    (if (and (Variables|Default|GetIsBeingCarried?) (!= (Utilities|GetClass self) "/Game/Thibaud/Blueprints/Player/Post/FireFunctionality/BPA_Kits_Extinguisher.BPA_Kits_Extinguisher_C"))
      (Utilities|Casting|CastToBPA_Kits_Ammo _self
        (:then
          (if (!= (Variables|/Game/Thibaud/Blueprints/Player/Post/BPA_Post_Parent.BPA_Post_Parent_C|GetAmmo _post) (Variables|/Game/Thibaud/Blueprints/Player/Post/BPA_Post_Parent.BPA_Post_Parent_C|GetAmmoCap _post))
            (Default|TriggerAmmoHatch _post true _self :!label _label)))
        (:CastFailed
          (goto _label))))))

(event OnComponentEndOverlap(Holder)
  (params (OverlappedComponent :type Primitive%20Component%20Object%20Reference) (OtherActor :type Actor%20Object%20Reference) (OtherComp :type Primitive%20Component%20Object%20Reference) (OtherBodyIndex :type Integer))
  (bind _self self)
  (Utilities|FlowControl|Sequence
    (:then_0
      ;[1 1 1] Ammo Hatch Animation
      (bind (_post _ispost_) (CallFunction|IsStationOfDifferentType OtherActor))
      (if _ispost_
        (Utilities|Array|RemoveItem (Variables|Default|GetOverlappedStations) _post)
        (if (!= (Utilities|GetClass self) "/Game/Thibaud/Blueprints/Player/Post/FireFunctionality/BPA_Kits_Extinguisher.BPA_Kits_Extinguisher_C")
          (Default|TriggerAmmoHatch _post false self))))
    (:then_1
      ;[1 1 1] Respawn on Falling Off
      (bind _asbp_starship (Utilities|Casting|CastToBp_Starship OtherActor))
      (Utilities|Casting|CastToBPA_Kits_Upgrade _self
        (:then
          _)
        (:CastFailed
          (Utilities|Casting|CastToBPA_Kits_Extinguisher _self)))
      (if (and (== (Variables|/Game/Thibaud/Blueprints/Player/Bp_Starship.Bp_Starship_C|GetCollision_Ship _asbp_starship) OtherComp) (not (Variables|Default|GetIsBeingCarried?)))
        (Transformation|SetWorldLocation (Variables|Default|GetHolder) (Transformation|GetWorldLocation (Variables|/Game/Thibaud/Blueprints/Player/Bp_Starship.Bp_Starship_C|GetRespawn_Position _asbp_starship)) false true)))))

(event Custom|ChildGrab
  ;[1 1 1] Parent Function
)

(event Custom|RefreshTooltip
  (bind _icon (Variables|Default|GetIcon))
  ;[1 1 1] Tooltip
  (bind _yes_ (CallFunction|PlayersNotUsingPost?))
  (if (Math|Boolean|ANDBoolean (!= (Utilities|Array|Length (Variables|Default|GetOverlappedPlayers)) 0) (not (Variables|Default|GetIsBeingCarried?)) _yes_)
    (Rendering|SetVisibility _icon true false)
    (else
      (Rendering|SetVisibility _icon false false))))

(event Custom|Pick/Drop%20Item
  (params (Character :type Character%20Object%20Reference) (Impulse :type Float%20%28single-precision%29))
  (bind _self self)
  (bind _holder (Variables|Default|GetHolder))
  ;[1 1 1] PICK/DROP
  (Variables|Default|SetImpulse Impulse)
  (bind _output_get (Variables|Default|SetCharacter Character))
  (bind _asbp_player (Utilities|Casting|CastToBP_Player _output_get))
  (Utilities|FlowControl|Sequence
    (:then_0
      ;[1 1 1] Ammo Hatch Animation
      (if (!= (Utilities|GetClass self) "/Game/Thibaud/Blueprints/Player/Post/FireFunctionality/BPA_Kits_Extinguisher.BPA_Kits_Extinguisher_C")
        (for _array_element (Variables|Default|GetOverlappedStations)
          (Utilities|Casting|CastToBPA_Kits_Ammo _self
            (:then
              (if (!= (Variables|/Game/Thibaud/Blueprints/Player/Post/BPA_Post_Parent.BPA_Post_Parent_C|GetAmmo _array_element) (Variables|/Game/Thibaud/Blueprints/Player/Post/BPA_Post_Parent.BPA_Post_Parent_C|GetAmmoCap _array_element))
                (Default|TriggerAmmoHatch _array_element (not (Variables|/Game/Thibaud/Blueprints/Player/BP_Player.BP_Player_C|GetCurrentlyHoldingAnObject? _asbp_player)) _self :!label _label)))
            (:CastFailed
              (goto _label))))))
    (:then_1
      (Audio|PlaySound2D "/Game/Assets/Audio/SoundCues/SC_GettingOnPost_v2.SC_GettingOnPost_v2" 1.0 1.0 0.0 0 0)
      (if (Variables|/Game/Thibaud/Blueprints/Player/BP_Player.BP_Player_C|GetCurrentlyHoldingAnObject? _asbp_player)
        (CallFunction|DroppedBehaviour _asbp_player)
        (Utilities|FlowControl|Sequence
          (:then_0
            (bind _asbpa_kits_extinguisher (Utilities|Casting|CastToBPA_Kits_Extinguisher self))
            (if (<= (Variables|/Game/Thibaud/Blueprints/Player/Post/FireFunctionality/BPA_Kits_Extinguisher.BPA_Kits_Extinguisher_C|GetAmmo _asbpa_kits_extinguisher) 12.5)
              (Variables|Default|SetIsBeingCarried? true)
              (Utilities|FlowControl|Delay 0.5)
              (Effects|SpawnEmitterAttached "/Game/Léa/FX/Particle/P_Smoke_puff_localspace.P_Smoke_puff_localspace" (Variables|/Game/Thibaud/Blueprints/Player/Bp_Starship.Bp_Starship_C|GetShip%20Hull (Variables|Default|GetBPA%20Vaisseau)) "None" (Transformation|GetActorLocation) "0, 0, 0" "0.100000,0.100000,0.100000" "KeepWorldPosition")
              (Actor|DestroyActor)
              (else
                (Variables|/Game/Thibaud/Blueprints/Player/Post/FireFunctionality/BPA_Kits_Extinguisher.BPA_Kits_Extinguisher_C|SetFirstSpawn _asbpa_kits_extinguisher true))))
          (:then_1
            (bind _outactors (Actor|GetAllActorsOfClass "/Game/Thibaud/Blueprints/Player/Post/BPA_Post_Parent.BPA_Post_Parent_C"))
            (for _array_element_2 _outactors
              (Default|StopUpgradeTuto _array_element_2)))
          (:then_2
            (Utilities|FlowControl|Delay 1.0)
            (Class|PrimitiveComponent|SetConstraintMode (Variables|Default|GetHolder) "Default")))
        (else
          (Transformation|AttachComponentToComponent _holder (Variables|/Script/Engine.Character|GetMesh _asbp_player) "Hand_RSocket" "SnapToTarget" "SnapToTarget" "KeepWorld" true)
          (Class|PrimitiveComponent|SetConstraintMode _holder "XYPlane")
          (Physics|SetSimulatePhysics (Variables|Default|GetHolder) false)
          (Variables|/Game/Thibaud/Blueprints/Player/BP_Player.BP_Player_C|SetCurrentlyHoldingAnObject? _asbp_player true)
          (Variables|/Game/Thibaud/Blueprints/Player/BP_Player.BP_Player_C|SetCurrentPickup _asbp_player self)
          (Variables|Default|SetIsBeingCarried? true)
          (CallFunction|ChildGrab)
          ;[1 1 1] Tooltip
          (Rendering|SetVisibility (Variables|Default|GetIcon) false false))))))

(event EventBeginPlay
  (bind _returnvalue (Actor|GetActorOfClass "/Game/Thibaud/Blueprints/Player/Bp_Starship.Bp_Starship_C"))
  (Variables|Default|SetBPA%20Vaisseau _returnvalue))

(event EventDestroyed
  ;[1 1 1] Delete oldest kit if too many
  (bind _returnvalue (Actor|GetActorOfClass "/Game/Thibaud/Blueprints/Player/Post/BPA_Post_Logistics.BPA_Post_Logistics_C"))
  (Utilities|Array|RemoveItem (Variables|/Game/Thibaud/Blueprints/Player/Post/BPA_Post_Logistics.BPA_Post_Logistics_C|GetSpawnedKits _returnvalue) self)
  (for _array_element (Variables|Default|GetOverlappedStations)
    (Utilities|Array|RemoveItem (Variables|/Game/Thibaud/Blueprints/Player/Post/BPA_Post_Parent.BPA_Post_Parent_C|GetHeldKitsNear _array_element) self)))

(fn ConstructionScript)

(fn GetMesh
  (return (Variables|Default|GetHolder)))

(fn DroppedBehaviour
  (params (Character :type Character%20Object%20Reference))
  (bind _holder (Variables|Default|GetHolder))
  (bind _impulse (Variables|Default|GetImpulse))
  (bind _asbp_player (Utilities|Casting|CastToBP_Player (Variables|Default|GetCharacter)))
  (Variables|/Game/Thibaud/Blueprints/Player/BP_Player.BP_Player_C|SetUsingExtinguisher? _asbp_player false)
  (Transformation|SetActorRotation (Math|Rotator|MakeRotator 0.0 0.0 (.yaw (Math|Rotator|CombineRotators (Transformation|GetWorldRotation (Variables|/Script/Engine.Character|GetCapsuleComponent _asbp_player)) "0,180.000000, 0"))) true)
  (Transformation|DetachFromActor self "KeepRelative" "KeepRelative" "KeepWorld")
  (Class|PrimitiveComponent|SetConstraintMode _holder "CustomPlane")
  (Physics|SetSimulatePhysics _holder true)
  (Variables|Default|SetIsBeingCarried? false)
  (Utilities|FlowControl|Sequence
    (:then_0
      (bind _asbp_player_2 (Utilities|Casting|CastToBP_Player Character))
      (Variables|/Game/Thibaud/Blueprints/Player/BP_Player.BP_Player_C|SetCurrentlyHoldingAnObject? _asbp_player_2 false)
      (Physics|AddImpulse (Variables|Default|GetHolder) (Math|Vector|MakeVector (.x (* (Math|Vector|GetForwardVector (Variables|/Script/Engine.Character|GetCapsuleComponent _asbp_player_2)) (* _impulse 1.75e+03))) (.y (* (Math|Vector|GetForwardVector (Variables|/Script/Engine.Character|GetCapsuleComponent _asbp_player_2)) (* _impulse 1.75e+03))) (* _impulse 2.5e+03)) "None" false))
    (:then_1
      (bind _asbpa_kits_extinguisher (Utilities|Casting|CastToBPA_Kits_Extinguisher self))
      (Default|StopExtinguishing _asbpa_kits_extinguisher))))

(fn IsStationOfDifferentType
  (params (Actor :type Actor%20Object%20Reference))
  (bind _asbpa_post_parent (Utilities|Casting|CastToBPA_Post_Parent Actor)
    (:then
      (bind _asbpa_kits_upgrade (Utilities|Casting|CastToBPA_Kits_Upgrade self)
        (:then
          (if (Utilities|Enum|NotEqual(Enum) (Variables|/Game/Thibaud/Blueprints/Player/Post/BPA_Post_Parent.BPA_Post_Parent_C|GetUpgradeType _asbpa_post_parent) (Variables|/Game/Thibaud/Blueprints/Kits/BPA_Kits_Upgrade.BPA_Kits_Upgrade_C|GetType _asbpa_kits_upgrade))
            (return _asbpa_post_parent true)
            (else
              _)))
        (:CastFailed
          (return _asbpa_post_parent true))))
    (:CastFailed
      _))
  (return 0 false))

(fn PlayersNotUsingPost?
  (for _array_element (Variables|Default|GetOverlappedPlayers)
    (bind _asbp_player (Utilities|Casting|CastToBP_Player _array_element))
    (if (not (Variables|/Game/Thibaud/Blueprints/Player/BP_Player.BP_Player_C|GetCurrentlyUsingA%20Post? _asbp_player))
      (return true)))
  (return false))