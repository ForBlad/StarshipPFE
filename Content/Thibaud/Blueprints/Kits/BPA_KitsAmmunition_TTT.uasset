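; Ammunition kit actor that a BP_Player can pick up and that removes itself once its stock is depleted.
; The Items event alternates via FlipFlop between attaching the battery mesh to the player's Pickup component with physics off and restoring physics through an attach call with no parent.
; A looping timer started on BeginPlay polls Stock and destroys the actor when it reaches zero or below.
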(event Custom|Delete
  ;[1 1 1] Check Munition
  (if (<= (Variables|Default|GetStock) 0.0)
    (Actor|DestroyActor)))

(event EventItems
  (params (Character :type Character%20Object%20Reference))
  (bind _sm_battery (Variables|Default|GetSM_Battery))
  (bind _sm_battery_2 (Variables|Default|GetSM_Battery))
  ;[1 1 1] Pick Up Item
  (bind _asbp_player (Utilities|Casting|CastToBP_Player Character))
  (Utilities|FlowControl|FlipFlop
    (:A
      (Transformation|AttachComponentToComponent (Variables|Default|GetSM_Battery) (Variables|/Game/Thibaud/Blueprints/Player/BP_Player.BP_Player_C|GetPickup _asbp_player) "None" "SnapToTarget" "SnapToTarget" "SnapToTarget" true)
      (Class|PrimitiveComponent|SetConstraintMode _sm_battery "XYPlane")
      (Physics|SetSimulatePhysics _sm_battery false)
      (Development|PrintString "HIT"))
    (:B
      (Transformation|AttachComponentToComponent (Variables|Default|GetSM_Battery) 0 "None" "SnapToTarget" "SnapToTarget" "SnapToTarget" true)
      (Class|PrimitiveComponent|SetConstraintMode _sm_battery_2 "Default")
      (Physics|SetSimulatePhysics _sm_battery_2 true))))

(event EventBeginPlay
  ;[1 1 1] Check Munition
  (Utilities|Time|SetTimerbyEvent (delegate Custom|Delete) 0.1 true))

(fn ConstructionScript)