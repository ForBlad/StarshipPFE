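; Gatling kit pickup that, when a player drops it near a post, upgrades that post and refills its ammo.
; The dropped-behaviour override runs the parent logic, then has the player find the nearest post and set it as current.
; If that current post is within interaction distance, the nearest post receives the blue upgrade with this kit and its ammo is set to the cap.
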(event EventBeginPlay)

(fn ConstructionScript)

(fn DroppedBehaviour
  (params (Character :type Character%20Object%20Reference))
  (|CallParentFunction Character)
  (bind _asbp_player (Utilities|Casting|CastToBP_Player Character))
  (bind _nearest_post (Default|FindNearestPost->SettoCurrentPostifinDistance _asbp_player))
  (Utilities|IsValid _nearest_post
    (:Is%20Valid
      (bind _isless_ (Default|CheckDistance _asbp_player (Transformation|GetWorldLocation (Variables|/Script/Engine.Actor|GetRootComponent _asbp_player)) (Transformation|GetWorldLocation (Variables|/Game/Thibaud/Blueprints/Player/Post/BPA_Post_Parent.BPA_Post_Parent_C|GetDefaultSceneRoot (Variables|/Game/Thibaud/Blueprints/Player/BP_Player.BP_Player_C|GetCurrentPost _asbp_player))) (Variables|Default|GetPostInteractionDistance)))
      (if _isless_
        (Default|UPGRADE!-BLUE _nearest_post self)
        (Variables|/Game/Thibaud/Blueprints/Player/Post/BPA_Post_Parent.BPA_Post_Parent_C|SetAmmo _nearest_post (Variables|/Game/Thibaud/Blueprints/Player/Post/BPA_Post_Parent.BPA_Post_Parent_C|GetAmmoCap _nearest_post))))))