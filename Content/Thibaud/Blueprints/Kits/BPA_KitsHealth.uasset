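; Health kit actor that the player can pick up and drop; it contains no healing logic yet.
; The Items event casts the interacting character to BPC_Player, then a FlipFlop alternates between carrying and releasing.
; Carrying snaps the Sphere to the player's Pickup component with physics off and prints a debug message.
; Releasing calls attach with no parent, restores the default constraint mode and re-enables physics.
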(event EventItems
  (params (Character :type Character%20Object%20Reference))
  (bind _sphere (Variables|Default|GetSphere))
  (bind _sphere_2 (Variables|Default|GetSphere))
  ;[1 1 1] Pick Up Item
  (bind _asbpc_player (Utilities|Casting|CastToBPC_Player Character))
  (Utilities|FlowControl|FlipFlop
    (:A
      (Transformation|AttachComponentToComponent (Variables|Default|GetSphere) (Variables|/Game/Thibaud/Blueprints/Player/BPC_Player.BPC_Player_C|GetPickup _asbpc_player) "None" "SnapToTarget" "SnapToTarget" "SnapToTarget" true)
      (Class|PrimitiveComponent|SetConstraintMode _sphere "XYPlane")
      (Physics|SetSimulatePhysics _sphere false)
      (Development|PrintString "HIT"))
    (:B
      (Transformation|AttachComponentToComponent (Variables|Default|GetSphere) 0 "None" "SnapToTarget" "SnapToTarget" "SnapToTarget" true)
      (Class|PrimitiveComponent|SetConstraintMode _sphere_2 "Default")
      (Physics|SetSimulatePhysics _sphere_2 true))))

(fn ConstructionScript)