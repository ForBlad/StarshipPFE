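; Fire extinguisher kit item that lets the player put out BPA_Fire actors.
; UseItems stores the BP_Player and starts a looping timer that runs while that player's UseFireExtinc flag is set.
; Each tick spends one unit of Stock and sphere-traces a short distance forward from Scene1, calling Elimination on a hit fire.
; The actor destroys itself once Stock runs out, and the trace's debug drawing is enabled.
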(event Custom|UseFireExtinceur
  (bind _scene1 (Variables|Default|GetScene1))
  (bind _returnvalue (Transformation|GetWorldLocation _scene1))
  ;[1 1 1] PUTTING FIRE OUT
  (if (Variables|/Game/Thibaud/Blueprints/Player/BP_Player.BP_Player_C|GetUseFireExtinc (stale EventUseItems _asbp_player))
    (if (<= (Variables|Default|GetStock) 0.0)
      (Actor|DestroyActor)
      (else
        (Variables|Default|SetStock (- (Variables|Default|GetStock) 1.0))
        (bind (_outhit _returnvalue_2) (Collision|SphereTraceByChannel _returnvalue (+ _returnvalue (* (Math|Vector|GetForwardVector _scene1) 5.0)) 2.0 "TraceTypeQuery1" false (Utilities|Array|MakeArray self) "ForDuration"))
        (if _returnvalue_2
          (bind _asbpa_fire (Utilities|Casting|CastToBPA_Fire (.HitActor (Collision|BreakHitResult _outhit))))
          (Default|Elimination _asbpa_fire))))
    (else
      (Utilities|Time|ClearTimerbyFunctionName self "UseFireExtinceur"))))

(event EventBeginPlay
  (Components|StaticMesh|SetStaticMesh (Variables|Default|GetHolder) "/Game/Thibaud/Blueprints/Kits/SM_Estinguisher.SM_Estinguisher"))

(event EventUseItems
  (params (Character :type Character%20Object%20Reference))
  ;[1 1 1] PUTTING FIRE OUT
  (bind _asbp_player (Utilities|Casting|CastToBP_Player Character))
  (Utilities|Time|SetTimerbyEvent (delegate Custom|UseFireExtinceur) 0.1 true))

(fn ConstructionScript)