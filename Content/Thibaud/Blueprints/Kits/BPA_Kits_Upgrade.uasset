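; Upgrade kit that a player drops near a post to upgrade it with the kit's type: Laser, Explosive, Alien or Bullet.
; The construction script colours the Holder mesh by Type.
; On drop, it runs the parent behaviour, has BP_Player find and set the nearest post, then checks the player's distance to CurrentPost.
; Within PostInteractionDistance, it passes itself and its Type to that post's KitUpgrade.
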(fn ConstructionScript
  (bind _holder (Variables|Default|GetHolder))
  (switch string (Variables|Default|GetType)
    (:laser
      (Rendering|Material|SetMaterial _holder 0 "/Game/Assets/Materials/BRILLE_blue.BRILLE_blue"))
    (:explosive
      (Rendering|Material|SetMaterial _holder 0 "/Game/Assets/Materials/BRILLE_red.BRILLE_red"))
    (:alien
      (Rendering|Material|SetMaterial _holder 0 "/Game/Assets/Materials/BRILLE_violet.BRILLE_violet"))
    (:bullet
      (Rendering|Material|SetMaterial _holder 0 "/Game/Assets/Materials/BRILLE_yellow.BRILLE_yellow"))))

(fn DroppedBehaviour
  (params (Character :type Character%20Object%20Reference))
  (|CallParentFunction Character)
  (bind _asbp_player (Utilities|Casting|CastToBP_Player Character))
  (bind _nearest_post (Default|FindNearestPost->SettoCurrentPostifinDistance _asbp_player))
  (Utilities|IsValid _nearest_post
    (:Is%20Valid
      (bind _isless_ (Default|CheckDistance _asbp_player (Transformation|GetWorldLocation (Variables|/Script/Engine.Actor|GetRootComponent _asbp_player)) (Transformation|GetWorldLocation (Variables|/Game/Thibaud/Blueprints/Player/Post/BPA_Post_Parent.BPA_Post_Parent_C|GetDefaultSceneRoot (Variables|/Game/Thibaud/Blueprints/Player/BP_Player.BP_Player_C|GetCurrentPost _asbp_player))) (Variables|Default|GetPostInteractionDistance)))
      (if _isless_
        (Default|KitUpgrade _nearest_post self (Variables|Default|GetType))))))