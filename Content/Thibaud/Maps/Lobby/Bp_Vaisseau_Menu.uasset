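; Lobby/menu variant of the starship, which creates the HUD and colors each BP_Player's mesh and identity circle by player index after a short delay.
; Left and right overlap zones consume flamethrower, missile or gatling kits, setting that side's exclusive weapon flags on the GameInstance.
; TurnLeft applies local yaw and prints its axis value, while thrust events are empty.
; The post map built at BeginPlay is marked unused and only reads the first post.
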(event OnComponentBeginOverlap(SwitchWeaponLeft)
  (params (OverlappedComponent :type Primitive%20Component%20Object%20Reference) (OtherActor :type Actor%20Object%20Reference) (OtherComp :type Primitive%20Component%20Object%20Reference) (OtherBodyIndex :type Integer) (bFromSweep :type Boolean) (SweepResult :type Hit%20Result%20Structure%20%28by%20ref%29))
  (bind _gmi_starship (Variables|Default|GetGMI_Starship))
  (Utilities|FlowControl|Sequence
    (:then_0
      (bind _asbpa_kits_flamethrower (Utilities|Casting|CastToBPA_KitsFlamethrower OtherActor))
      (Variables|/Game/Thibaud/Blueprints/BP_Diverses/BPI_Starship.BPI_Starship_C|SetFlamethrowerLeft _gmi_starship true)
      (Variables|/Game/Thibaud/Blueprints/BP_Diverses/BPI_Starship.BPI_Starship_C|SetMissileLeft _gmi_starship false)
      (Variables|/Game/Thibaud/Blueprints/BP_Diverses/BPI_Starship.BPI_Starship_C|SetGatlineLeft _gmi_starship false)
      (Actor|DestroyActor _asbpa_kits_flamethrower))
    (:then_1
      (bind _asbpa_kits_missiles (Utilities|Casting|CastToBPA_KitsMissiles OtherActor))
      (Variables|/Game/Thibaud/Blueprints/BP_Diverses/BPI_Starship.BPI_Starship_C|SetMissileLeft _gmi_starship true)
      (Variables|/Game/Thibaud/Blueprints/BP_Diverses/BPI_Starship.BPI_Starship_C|SetFlamethrowerLeft _gmi_starship false)
      (Variables|/Game/Thibaud/Blueprints/BP_Diverses/BPI_Starship.BPI_Starship_C|SetGatlineLeft _gmi_starship false)
      (Actor|DestroyActor _asbpa_kits_missiles))
    (:then_2
      (bind _asbpa_kits_gatling (Utilities|Casting|CastToBPA_KitsGatling OtherActor))
      (Variables|/Game/Thibaud/Blueprints/BP_Diverses/BPI_Starship.BPI_Starship_C|SetGatlineLeft _gmi_starship true)
      (Variables|/Game/Thibaud/Blueprints/BP_Diverses/BPI_Starship.BPI_Starship_C|SetFlamethrowerLeft _gmi_starship false)
      (Variables|/Game/Thibaud/Blueprints/BP_Diverses/BPI_Starship.BPI_Starship_C|SetMissileLeft _gmi_starship false)
      (Actor|DestroyActor _asbpa_kits_gatling))))

(event OnComponentBeginOverlap(SwitchWeaponRight)
  (params (OverlappedComponent :type Primitive%20Component%20Object%20Reference) (OtherActor :type Actor%20Object%20Reference) (OtherComp :type Primitive%20Component%20Object%20Reference) (OtherBodyIndex :type Integer) (bFromSweep :type Boolean) (SweepResult :type Hit%20Result%20Structure%20%28by%20ref%29))
  (bind _gmi_starship (Variables|Default|GetGMI_Starship))
  (Utilities|FlowControl|Sequence
    (:then_0
      (bind _asbpa_kits_flamethrower (Utilities|Casting|CastToBPA_KitsFlamethrower OtherActor))
      (Variables|/Game/Thibaud/Blueprints/BP_Diverses/BPI_Starship.BPI_Starship_C|SetFlamethrowerRight _gmi_starship true)
      (Variables|/Game/Thibaud/Blueprints/BP_Diverses/BPI_Starship.BPI_Starship_C|SetMissileRight _gmi_starship false)
      (Variables|/Game/Thibaud/Blueprints/BP_Diverses/BPI_Starship.BPI_Starship_C|SetGatlineRight _gmi_starship false)
      (Actor|DestroyActor _asbpa_kits_flamethrower))
    (:then_1
      (bind _asbpa_kits_missiles (Utilities|Casting|CastToBPA_KitsMissiles OtherActor))
      (Variables|/Game/Thibaud/Blueprints/BP_Diverses/BPI_Starship.BPI_Starship_C|SetFlamethrowerRight _gmi_starship false)
      (Variables|/Game/Thibaud/Blueprints/BP_Diverses/BPI_Starship.BPI_Starship_C|SetMissileRight _gmi_starship true)
      (Variables|/Game/Thibaud/Blueprints/BP_Diverses/BPI_Starship.BPI_Starship_C|SetGatlineRight _gmi_starship false)
      (Actor|DestroyActor _asbpa_kits_missiles))
    (:then_2
      (bind _asbpa_kits_gatling (Utilities|Casting|CastToBPA_KitsGatling OtherActor))
      (Variables|/Game/Thibaud/Blueprints/BP_Diverses/BPI_Starship.BPI_Starship_C|SetFlamethrowerRight _gmi_starship false)
      (Variables|/Game/Thibaud/Blueprints/BP_Diverses/BPI_Starship.BPI_Starship_C|SetMissileRight _gmi_starship false)
      (Variables|/Game/Thibaud/Blueprints/BP_Diverses/BPI_Starship.BPI_Starship_C|SetGatlineRight _gmi_starship true)
      (Actor|DestroyActor _asbpa_kits_gatling))))

(event Custom|Acceleration/Decceleration
  (params (AxisValue :type Float%20%28single-precision%29))
  ;[1 1 1] Poste - Pilotage : Mouvement Physique
)

(event Custom|BackWard%20Trust
  (params (Axis%20Value :type Float%20%28single-precision%29))
  ;[1 1 1] Poste - Pilotage : Mouvement Physique
)

(event Custom|TurnLeft
  (params (AxisValue :type Float%20%28single-precision%29))
  ;[1 1 1] Poste - Pilotage : Rotation
  (Development|PrintString (Utilities|String|ToString(Float) AxisValue))
  (Transformation|AddActorLocalRotation (Math|Rotator|MakeRotator 0.0 0.0 AxisValue) false false))

(event EventBeginPlay
  ;[1 1 1] Event BeginPlay
  (Utilities|FlowControl|Sequence
    (:then_0
      (bind _asbpi_starship (Utilities|Casting|CastToBPI_Starship (Game|GetGameInstance)))
      (Variables|Default|SetGMI_Starship _asbpi_starship)
      (Utilities|FlowControl|Sequence
        (:then_0
          (bind _returnvalue (UserInterface|CreateWidget "/Game/Thibaud/Blueprints/Widgets/WG_HUD.WG_HUD_C"))
          (UserInterface|Viewport|AddtoViewport _returnvalue 0))
        (:then_1
          ;[1 1 1] creates a map of posts // NOT USED YET
          (bind _outactors (Actor|GetAllActorsOfClass "/Game/Thibaud/Blueprints/Player/Post/BPA_Post_Parent.BPA_Post_Parent_C"))
          (for _index (range 0 (- (Utilities|Array|Length _outactors) 1))
            (Utilities|Map|Add (Variables|Default|GetPost_Map) (Variables|/Game/Thibaud/Blueprints/Player/Post/BPA_Post_Parent.BPA_Post_Parent_C|GetPostName (Utilities|Array|Get(acopy) _outactors)) (Variables|/Game/Thibaud/Blueprints/Player/Post/BPA_Post_Parent.BPA_Post_Parent_C|GetPostNumber (Utilities|Array|Get(acopy) _outactors)))))))
    (:then_1
      (Utilities|FlowControl|Delay 0.2)
      (bind _outactors_2 (Actor|GetAllActorsOfClass "/Game/Thibaud/Blueprints/Player/BP_Player.BP_Player_C"))
      (for (_array_element _array_index) _outactors_2
        (bind _output_get (Variables|/Game/Thibaud/Blueprints/Player/BP_Player.BP_Player_C|SetPlayerNumber _array_element _array_index))
        (Rendering|Material|SetMaterial (Variables|/Script/Engine.Character|GetMesh _array_element) 0 (Utilities|Array|Get(acopy) (Variables|/Game/Thibaud/Blueprints/Player/BP_Player.BP_Player_C|GetPlayerColors _array_element) _output_get))
        (Rendering|Material|SetMaterial (Variables|/Game/Thibaud/Blueprints/Player/BP_Player.BP_Player_C|GetIdentity%20Circle _array_element) 0 (Utilities|Array|Get(acopy) (Variables|/Game/Thibaud/Blueprints/Player/BP_Player.BP_Player_C|GetCircleColors _array_element) _output_get))))))

(fn ConstructionScript)