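; Parent button Blueprint that triggers on any damage, notifying its target doors and lighting up linked connections.
; On BeginPlay it registers with each door, creates a dynamic material and applies any pre-triggered state.
; Activation increments door counters while a timeline moves the button and dims its color and light.
; With a SynchroDelay, it resets if doors remain untriggered afterward, decrementing counters and reversing the timeline, enabling synchronized multi-button doors.
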(event Custom|ResetButton
  (Variables|Default|SetTriggered? false)
  (Utilities|FlowControl|Sequence
    (:then_0
      (for _array_element (Variables|Default|GetTargetDoors)
        (Math|Integer|DecrementInt (Variables|/Game/Blueprints/DoorsNew/Door_Parent.Door_Parent_C|GetButtonsActivated _array_element))))
    (:then_1
      (bind _newtrack_0 (Timeline|Timeline_0 Reverse)
        (:Update
          (Rendering|Material|SetVectorParameterValue (stale EventBeginPlay _returnvalue) "Color" (Math|Color|Lerp(LinearColor) (stale EventBeginPlay _returnvalue_2) (* (stale EventBeginPlay _returnvalue_2) 0.1) _newtrack_0) :!class /Script/Engine.MaterialInstanceDynamic)
          (Transformation|SetRelativeLocation (Variables|Default|GetButton) (Math|Vector|Lerp(Vector) (Variables|Default|GetLocationStart) (Variables|Default|GetLocationEnd) _newtrack_0) false false)
          (Rendering|Components|Light|SetLightColor (Variables|Default|GetPointLight) (Math|Color|Lerp(LinearColor) (* (stale EventBeginPlay _returnvalue_2) 1.0) "(R=0.000000,G=0.000000,B=0.000000,A=0.000000)" _newtrack_0) true))))))

(event Game|Damage|EventAnyDamage
  (params (Damage :type Float%20%28single-precision%29) (DamageType :type Damage%20Type%20Object%20Reference) (InstigatedBy :type Controller%20Object%20Reference) (DamageCauser :type Actor%20Object%20Reference))
  (bind _synchrodelay (Variables|Default|GetSynchroDelay))
  (bind _targetdoors (Variables|Default|GetTargetDoors))
  (if (not (Variables|Default|GetTriggered?))
    (Variables|Default|SetTriggered? true)
    (Utilities|FlowControl|Sequence
      (:then_0
        (for _array_element _targetdoors
          (Math|Integer|IncrementInt (Variables|/Game/Blueprints/DoorsNew/Door_Parent.Door_Parent_C|GetButtonsActivated _array_element)
            (:%20%20
              (Default|OpenDoor _array_element self))))
        (for _array_element_2 (Variables|Default|GetTargetConnections)
          (Default|Lighton _array_element_2)))
      (:then_1
        (bind _newtrack_0 (Timeline|Timeline_0 Play)
          (:Update
            (Rendering|Material|SetVectorParameterValue (stale EventBeginPlay _returnvalue) "Color" (Math|Color|Lerp(LinearColor) (stale EventBeginPlay _returnvalue_2) (* (stale EventBeginPlay _returnvalue_2) 0.1) _newtrack_0) :!class /Script/Engine.MaterialInstanceDynamic)
            (Transformation|SetRelativeLocation (Variables|Default|GetButton) (Math|Vector|Lerp(Vector) (Variables|Default|GetLocationStart) (Variables|Default|GetLocationEnd) _newtrack_0) false false)
            (Rendering|Components|Light|SetLightColor (Variables|Default|GetPointLight) (Math|Color|Lerp(LinearColor) (* (stale EventBeginPlay _returnvalue_2) 1.0) "(R=0.000000,G=0.000000,B=0.000000,A=0.000000)" _newtrack_0) true))))
      (:then_2
        (if (> _synchrodelay 0.0)
          (Utilities|FlowControl|Delay _synchrodelay)
          (for _array_element_3 _targetdoors
            (if (not (Variables|/Game/Blueprints/DoorsNew/Door_Parent.Door_Parent_C|GetTriggered? _array_element_3))
              (CallFunction|ResetButton))))))))

(event EventBeginPlay
  (bind _button (Variables|Default|GetButton))
  (Rendering|Material|SetMaterial _button 0 (Variables|Default|GetMaterial))
  (Rendering|Material|SetMaterial (Variables|Default|Getr) 1 (Variables|Default|GetMaterial_frame))
  (Utilities|FlowControl|Sequence
    (:then_0
      (bind _returnvalue (Rendering|Material|CreateDynamicMaterialInstance _button 0 (Rendering|Material|GetMaterial _button 0) "None" :!class /Script/Engine.PrimitiveComponent))
      (bind _returnvalue_2 (Rendering|Material|GetVectorParameterValue _returnvalue "Color" :!class /Script/Engine.MaterialInstanceDynamic))
      (Variables|Default|SetLocationStart (Variables|/Script/Engine.SceneComponent|GetRelativeLocation _button))
      (Variables|Default|SetLocationEnd "60.000000,0.000000, 0")
      (Rendering|Components|Light|SetLightColor (Variables|Default|GetPointLight) (* _returnvalue_2 1.0) true))
    (:then_1
      (if (Variables|Default|GetTriggered?)
        (Utilities|FlowControl|Sequence
          (:then_0
            (bind _newtrack_0 (Timeline|Timeline_0 SetNewTime)
              (:Update
                (Rendering|Material|SetVectorParameterValue _returnvalue "Color" (Math|Color|Lerp(LinearColor) _returnvalue_2 (* _returnvalue_2 0.1) _newtrack_0) :!class /Script/Engine.MaterialInstanceDynamic)
                (Transformation|SetRelativeLocation (Variables|Default|GetButton) (Math|Vector|Lerp(Vector) (Variables|Default|GetLocationStart) (Variables|Default|GetLocationEnd) _newtrack_0) false false)
                (Rendering|Components|Light|SetLightColor (Variables|Default|GetPointLight) (Math|Color|Lerp(LinearColor) (* _returnvalue_2 1.0) "(R=0.000000,G=0.000000,B=0.000000,A=0.000000)" _newtrack_0) true))))
          (:then_1
            (for _array_element (Variables|Default|GetTargetDoors)
              (Math|Integer|IncrementInt (Variables|/Game/Blueprints/DoorsNew/Door_Parent.Door_Parent_C|GetButtonsActivated _array_element)))))))
    (:then_2
      (for _array_element_2 (Variables|Default|GetTargetDoors)
        (Utilities|Array|Add (Variables|/Game/Blueprints/DoorsNew/Door_Parent.Door_Parent_C|GetButtonsLinked _array_element_2) self)))))

(fn ConstructionScript)