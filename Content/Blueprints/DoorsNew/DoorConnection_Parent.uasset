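; Base Blueprint for a door connection piece whose cylinder lights up when LightOn is called.
; BeginPlay applies the Material variable to the cylinder, creates a dynamic instance, reads its Color parameter and sets the initial color.
; LightOn plays a timeline that drives the same color update, lerping between a dimmed and an overbright multiple of that color.
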(event Custom|LightOn
  (bind _newtrack_0 (Timeline|Timeline_0 Play)
    (:Update
      (Rendering|Material|SetVectorParameterValue (stale EventBeginPlay _returnvalue) "Color" (Math|Color|Lerp(LinearColor) (* (stale EventBeginPlay _returnvalue_2) 0.1) (* (stale EventBeginPlay _returnvalue_2) 1e+01) _newtrack_0) :!class /Script/Engine.MaterialInstanceDynamic))))

(event EventBeginPlay
  (bind _cylinder (Variables|Default|GetCylinder))
  (Rendering|Material|SetMaterial _cylinder 0 (Variables|Default|GetMaterial))
  (bind _returnvalue (Rendering|Material|CreateDynamicMaterialInstance _cylinder 0 (Rendering|Material|GetMaterial _cylinder 0) "None" :!class /Script/Engine.PrimitiveComponent))
  (bind _returnvalue_2 (Rendering|Material|GetVectorParameterValue _returnvalue "Color" :!class /Script/Engine.MaterialInstanceDynamic))
  (Rendering|Material|SetVectorParameterValue _returnvalue "Color" (Math|Color|Lerp(LinearColor) (* _returnvalue_2 0.1) (* _returnvalue_2 1e+01) (stale Custom|LightOn _newtrack_0)) :!class /Script/Engine.MaterialInstanceDynamic))

(fn ConstructionScript)