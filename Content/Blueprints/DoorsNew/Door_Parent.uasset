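; Base door Blueprint that opens by fading out rather than moving.
; On BeginPlay it creates a dynamic material instance on the Door component and caches its starting opacity parameter.
; OpenDoor disables Door collision and plays a timeline that lerps opacity from that starting value to zero.
; CloseDoor restores query and physics collision and reverses the same timeline to fade the door back in.
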(event Custom|OpenDoor
  (Collision|SetCollisionEnabled (Variables|Default|GetDoor) "NoCollision")
  (bind _newtrack_0 (Timeline|Timeline_0 Play)
    (:Update
      (Rendering|Material|SetScalarParameterValue (stale EventBeginPlay _returnvalue) "opacitu" (Math|Float|Lerp (stale EventBeginPlay _returnvalue_2) 0.0 _newtrack_0) :!class /Script/Engine.MaterialInstanceDynamic))))

(event Custom|CloseDoor
  (Collision|SetCollisionEnabled (Variables|Default|GetDoor) "QueryAndPhysics")
  (bind _newtrack_0 (Timeline|Timeline_0 Reverse)
    (:Update
      (Rendering|Material|SetScalarParameterValue (stale EventBeginPlay _returnvalue) "opacitu" (Math|Float|Lerp (stale EventBeginPlay _returnvalue_2) 0.0 _newtrack_0) :!class /Script/Engine.MaterialInstanceDynamic))))

(event EventBeginPlay
  (bind _door (Variables|Default|GetDoor))
  (bind _returnvalue (Rendering|Material|CreateDynamicMaterialInstance _door 0 (Rendering|Material|GetMaterial _door 0) "None" :!class /Script/Engine.PrimitiveComponent))
  (bind _returnvalue_2 (Rendering|Material|GetScalarParameterValue _returnvalue "opacitu" :!class /Script/Engine.MaterialInstanceDynamic)))

(fn ConstructionScript)