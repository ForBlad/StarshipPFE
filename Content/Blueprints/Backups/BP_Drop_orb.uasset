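; BP_Drop_orb is a pickup orb that grants a typed upgrade kit (laser, explosive, alien or bullet) to the starship.
; On BeginPlay it colors its sphere material to match its type.
; When a Bp_Starship overlaps the sphere, it spawns a BPA_Kits_Upgrade of the same type at the ship's RespawnPosition component, then destroys itself.
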(event OnComponentBeginOverlap(Sphere)
  (params (OverlappedComponent :type Primitive%20Component%20Object%20Reference) (OtherActor :type Actor%20Object%20Reference) (OtherComp :type Primitive%20Component%20Object%20Reference) (OtherBodyIndex :type Integer) (bFromSweep :type Boolean) (SweepResult :type Hit%20Result%20Structure%20%28by%20ref%29))
  (bind _asbp_starship (Utilities|Casting|CastToBp_Starship OtherActor))
  (Game|SpawnActorfromClass "/Game/Thibaud/Blueprints/Kits/BPA_Kits_Upgrade.BPA_Kits_Upgrade_C" (Math|Transform|MakeTransform (Transformation|GetWorldLocation (Variables|/Game/Thibaud/Blueprints/Player/Bp_Starship.Bp_Starship_C|GetRespawn_Position _asbp_starship)) "0, 0, 0" "1,1,1") "Undefined" 0 (Variables|Default|GetType%20%28laser/explosive/alien/bullet%29) 0)
  (Actor|DestroyActor))

(event EventBeginPlay
  (bind _sphere (Variables|Default|GetSphere))
  (switch string (Variables|Default|GetType%20%28laser/explosive/alien/bullet%29)
    (:laser
      (Rendering|Material|SetMaterial _sphere 0 "/Game/Assets/Materials/BRILLE_blue.BRILLE_blue"))
    (:explosive
      (Rendering|Material|SetMaterial _sphere 0 "/Game/Assets/Materials/BRILLE_red.BRILLE_red"))
    (:alien
      (Rendering|Material|SetMaterial _sphere 0 "/Game/Assets/Materials/BRILLE_violet.BRILLE_violet"))
    (:bullet
      (Rendering|Material|SetMaterial _sphere 0 "/Game/Assets/Materials/BRILLE_yellow.BRILLE_yellow"))))

(fn ConstructionScript)