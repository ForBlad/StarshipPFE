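; BP_Healing_Orb is a pickup that fully restores a Bp_Starship's life when the ship overlaps its sphere.
; Overlap plays heal effects, refreshes health widgets, extinguishes and destroys every BP_Post_Fire actor in the world, then destroys the orb.
; A looping timer, rather than Tick, spins the switch, wrench and repair effect components.
; The construction script orients SMSwitch from the starship camera's pitch and yaw.
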(event OnComponentBeginOverlap(Sphere)
  (params (OverlappedComponent :type Primitive%20Component%20Object%20Reference) (OtherActor :type Actor%20Object%20Reference) (OtherComp :type Primitive%20Component%20Object%20Reference) (OtherBodyIndex :type Integer) (bFromSweep :type Boolean) (SweepResult :type Hit%20Result%20Structure%20%28by%20ref%29))
  (bind _asbp_starship (Utilities|Casting|CastToBp_Starship OtherActor))
  (Effects|SpawnEmitterAttached "/Game/InfinityBladeEffects/Effects/FX_Ability/Heal/P_Health_Pickup_01.P_Health_Pickup_01" (Variables|/Game/Thibaud/Blueprints/Player/Bp_Starship.Bp_Starship_C|GetShip%20Hull _asbp_starship) "None")
  (Audio|PlaySoundatLocation "/Game/Assets/Audio/SOUNDBANK/ENVIRONMENT/ENV_HEAL.ENV_HEAL" (Transformation|GetWorldLocation (Variables|Default|GetSphere)) "0, 0, 0" 1.0 1.0 0.0 0 0 0)
  (Utilities|FlowControl|Sequence
    (:then_0
      (Variables|/Game/Thibaud/Blueprints/Player/Bp_Starship.Bp_Starship_C|SetLife _asbp_starship (Variables|/Game/Thibaud/Blueprints/Player/Bp_Starship.Bp_Starship_C|GetMax_Life _asbp_starship))
      (Default|RefreshHealthWidgets _asbp_starship))
    (:then_1
      (bind _outactors (Actor|GetAllActorsOfClass "/Game/Thibaud/Blueprints/Player/Post/FireFunctionality/BP_Post_Fire.BP_Post_Fire_C"))
      (for _array_element _outactors
        (Default|ExtinguishFire (Variables|/Game/Thibaud/Blueprints/Player/Post/FireFunctionality/BP_Post_Fire.BP_Post_Fire_C|GetPost _array_element) _array_element)
        (Actor|DestroyActor _array_element)))
    (:then_2
      (Actor|DestroyActor))))

(event Custom|Rotation
  (Transformation|AddWorldRotation (Variables|Default|GetSM_Switch) "0,2.500000, 0" false false)
  (Transformation|AddLocalRotation (Variables|Default|GetPickup_Repair_Wrench) "2.500000, 0, 0" false false)
  (Transformation|AddLocalRotation (Variables|Default|GetPickup_Repair_Wrench1) "-2.500000, 0, 0" false false)
  (Transformation|AddLocalRotation (Variables|Default|GetPickup_Repair_Effect) "0.000000,-5.000000, 0" false false))

(event EventBeginPlay
  (Utilities|Time|SetTimerbyEvent (delegate Custom|Rotation) 0.05 true))

(fn ConstructionScript
  (bind _returnvalue (Actor|GetActorOfClass "/Game/Thibaud/Blueprints/Player/Bp_Starship.Bp_Starship_C"))
  (bind _output_get (Variables|Default|SetBPA%20Vaisseau _returnvalue))
  (Transformation|SetWorldRotation (Variables|Default|GetSM_Switch) (Math|Rotator|MakeRotator (.pitch (Transformation|GetWorldRotation (Variables|/Game/Thibaud/Blueprints/Player/Bp_Starship.Bp_Starship_C|GetCamera1 _output_get))) 0.0 (+ (.yaw (Transformation|GetWorldRotation (Variables|/Game/Thibaud/Blueprints/Player/Bp_Starship.Bp_Starship_C|GetCamera1 _output_get))) 9e+01)) false false))