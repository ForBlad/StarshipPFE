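; Vaurte boss actor that fires missiles while the player is in range, plays battle music and explodes when killed.
; Tick drives missile reloading and a LASER graph that rotates the boss while spawning projectiles until heat forces a cooldown.
; TurretDestroyed arms the laser after a warning sound and delay, and damage only counts while VaurteIsVulnerable is set.
; Movement and entry animation logic is present but disconnected.
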(event OnComponentBeginOverlap(player_detector)
  (params (OverlappedComponent :type Primitive%20Component%20Object%20Reference) (OtherActor :type Actor%20Object%20Reference) (OtherComp :type Primitive%20Component%20Object%20Reference) (OtherBodyIndex :type Integer) (bFromSweep :type Boolean) (SweepResult :type Hit%20Result%20Structure%20%28by%20ref%29))
  ;[1 1 1] Combat
  (Utilities|Casting|CastToBP_Player OtherActor)
  (Variables|Default|Setplayer_in_range true))

(event OnComponentEndOverlap(player_detector)
  (params (OverlappedComponent :type Primitive%20Component%20Object%20Reference) (OtherActor :type Actor%20Object%20Reference) (OtherComp :type Primitive%20Component%20Object%20Reference) (OtherBodyIndex :type Integer))
  ;[1 1 1] Combat
  (Utilities|Casting|CastToBP_Player OtherActor)
  (Variables|Default|Setplayer_in_range false))

(event OnComponentBeginOverlap(bossfight_detector)
  (params (OverlappedComponent :type Primitive%20Component%20Object%20Reference) (OtherActor :type Actor%20Object%20Reference) (OtherComp :type Primitive%20Component%20Object%20Reference) (OtherBodyIndex :type Integer) (bFromSweep :type Boolean) (SweepResult :type Hit%20Result%20Structure%20%28by%20ref%29))
  ;[1 1 1] Vaurte Battle Theme
  (Utilities|Casting|CastToBP_Player OtherActor)
  (Utilities|FlowControl|DoOnce false
    (:Completed
      (Audio|PlaySoundatLocation "/Game/Assets/Audio/dark-souls-iii-soundtrack-ost-vordt-of-the-boreal-valley_1_.dark-souls-iii-soundtrack-ost-vordt-of-the-boreal-valley_1_" "0, 0, 0" "0, 0, 0" 1.0 1.0 0.0 0 0 0))))

(event Custom|TurretDestroyed
  ;[1 1 1] Combat
  (if (not (Variables|Default|GetLaser_isUp))
    (Audio|PlaySound2D "/Game/Assets/Audio/SOUNDBANK/SFX/SFX_SHIP/BOSS/SFX_SHIP_BOSS_StartFiring.SFX_SHIP_BOSS_StartFiring" 1.0 1.0 0.0 0 0)
    (Utilities|FlowControl|Delay 5.0)
    (Variables|Default|SetLaser_isUp true)
    (Utilities|FlowControl|Delay 9.0)
    (Audio|PlaySound2D "/Game/Assets/Audio/EnemyShot.EnemyShot" 1.0 1.0 0.0 0 0)))

(event EventBeginPlay
  ;[1 1 1] Setup References and Variables
  (Development|SetHiddeninGame (Variables|Default|GetLAZOR) true false)
  (bind _asbpi_starship (Utilities|Casting|CastToBPI_Starship (Game|GetGameInstance)))
  (Variables|Default|SetGI_Starship _asbpi_starship)
  (Utilities|Casting|CastToBP_GameMode (Game|GetGameMode)))

(event EventTick
  (params (DeltaSeconds :type Float%20%28single-precision%29))
  ;[1 1 1] Movement
  ;[1 1 1] Combat
  (Utilities|FlowControl|Sequence
    (:then_0
      (if (Variables|Default|Getplayer_in_range)
        (if (Variables|Default|GetMissile_Ready)
          (|FireMissile))))
    (:then_1
      (Utilities|FlowControl|Delay 8.0)
      (Variables|Default|SetMissile_ready true))
    (:then_2
      (goto _label execute2))
    (:then_3
      (|LASER :!label _label))))

(event Game|Damage|EventAnyDamage
  (params (Damage :type Float%20%28single-precision%29) (DamageType :type Damage%20Type%20Object%20Reference) (InstigatedBy :type Controller%20Object%20Reference) (DamageCauser :type Actor%20Object%20Reference))
  ;[1 1 1] Damages
  (if (Variables|Default|GetVaurte_isVulnerable)
    (Variables|Default|SetHealth (Math|Float|Clamp(Float) (- (Variables|Default|GetHealth) Damage) 0.0 (Variables|Default|GetMaxHealth)))
    (if (<= (Variables|Default|GetHealth) 0.0)
      (Variables|Default|SetVaurte_isDead true)
      (CallFunction|EnemyKilled))))

(event Collision|EventHit
  (params (MyComp :type Primitive%20Component%20Object%20Reference) (Other :type Actor%20Object%20Reference) (OtherComp :type Primitive%20Component%20Object%20Reference) (bSelfMoved :type Boolean) (HitLocation :type Vector :default "0, 0, 0") (HitNormal :type Vector :default "0, 0, 0") (NormalImpulse :type Vector :default "0, 0, 0") (Hit :type Hit%20Result%20Structure%20%28by%20ref%29))
  ;[1 1 1] Movement
  (Utilities|Casting|CastToBP_ProjectilePlayerBase Other
    (:CastFailed
      (Variables|Default|SetMoveDirection (not (Variables|Default|GetMoveDirection))))))

(fn ConstructionScript)

(fn EnemyKilled
  (Niagara|SpawnSystematLocation "/Game/Léa/FX/Particle/N_Explosion_RETAKES.N_Explosion_RETAKES" (Transformation|GetActorLocation) "0, 0, 0" "4.000000,4.000000,4.000000")
  (Audio|PlaySoundatLocation "/Game/Assets/Audio/Explosion.Explosion" (Transformation|GetActorLocation) "0, 0, 0" 1.0 1.0 0.0 0 0 0)
  (Actor|DestroyActor))