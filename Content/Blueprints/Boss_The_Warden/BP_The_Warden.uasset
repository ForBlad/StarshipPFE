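; The Warden boss actor, with laser and missile attacks, that reports to BP_Bossfight_The_Warden.
; A timeline spins the laser, while a looping timer started on overlap damages the overlapping Bp_Starship if the laser is up.
; Separate events briefly show an aiming beam and spawn missiles.
; While vulnerable it takes damage, calling ShieldsUp and turning invulnerable at two health thresholds, then exploding and ending the fight at zero.
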(event OnComponentBeginOverlap(LaserBody)
  (params (OverlappedComponent :type Primitive%20Component%20Object%20Reference) (OtherActor :type Actor%20Object%20Reference) (OtherComp :type Primitive%20Component%20Object%20Reference) (OtherBodyIndex :type Integer) (bFromSweep :type Boolean) (SweepResult :type Hit%20Result%20Structure%20%28by%20ref%29))
  ;[1 1 1] Laser Patern
  (Utilities|Casting|CastToBp_Starship OtherActor)
  (Utilities|Time|SetTimerbyEvent (delegate Custom|HAHA%20LASER%20GO%20BRRRRRRR) 0.1 true))

(event OnComponentEndOverlap(LaserBody)
  (params (OverlappedComponent :type Primitive%20Component%20Object%20Reference) (OtherActor :type Actor%20Object%20Reference) (OtherComp :type Primitive%20Component%20Object%20Reference) (OtherBodyIndex :type Integer))
  ;[1 1 1] Laser Patern
  (Utilities|Casting|CastToBp_Starship OtherActor)
  (Utilities|Time|ClearTimerbyFunctionName 0 "LaserDamageTick"))

(event Custom|LASER%20PATERN
  (bind _laser_body (Variables|Default|GetLaser%20Body))
  ;[1 1 1] Laser Patern
  (Utilities|FlowControl|Sequence
    (:then_0
      (Development|SetHiddeninGame _laser_body false false)
      (Variables|Default|SetLaser_isUp true))
    (:then_1
      (bind _newtrack_0 (Timeline|SPIN%20TO%20WIN PlayFromStart)
        (:Update
          (Utilities|FlowControl|Sequence
            (:then_0
              (Transformation|SetRelativeRotation (Variables|Default|GetScene) (Math|Rotator|MakeRotator 0.0 0.0 _newtrack_0) false false)
              (Effects|SpawnEmitterAttached "/Game/Léa/FX/Particle/P_Muzzle_laser_green.P_Muzzle_laser_green" (Variables|Default|GetArrow) "None" "0, 0, 0" "0, 0, 0" "12.000000,12.000000,12.000000"))
            (:then_1
              (if (> _newtrack_0 2.5e+02)
                (Utilities|FlowControl|DoOnce false :!label _label
                  (:Completed
                    (Audio|PlaySoundatLocation "/Game/Assets/Audio/SOUNDBANK/SFX/SFX_SHIP/BOSS/SFX_SHIP_BOSS_StopFiring.SFX_SHIP_BOSS_StopFiring" "0, 0, 0" "0, 0, 0" 0.6 1.0 0.0 0 0 0)))))))
        (:Finished
          (Development|SetHiddeninGame _laser_body true false)
          (Variables|Default|SetLaser_isUp false)
          (Actor|GetActorOfClass "/Game/Blueprints/Boss_The_Warden/BP_Bossfight_The_Warden.BP_Bossfight_The_Warden_C")
          (goto _label Reset))))))

(event Custom|MISSILE%20GO
  ;[1 1 1] Missile Patern
  (Game|SpawnActorfromClass (Variables|Default|GetProjectileType) (Transformation|GetWorldTransform (Variables|Default|GetArrow)) "Undefined" 0 (Variables|Default|GetProjectileColour) 0)
  (Audio|PlaySoundatLocation "/Game/Assets/Audio/SOUNDBANK/SFX/SFX_SHIP/MISSILE_CRUISER/SFX_SHIP_MAINSHIP_Missile_Launch_01.SFX_SHIP_MAINSHIP_Missile_Launch_01" (Transformation|GetActorLocation) "0, 0, 0" 1.0 1.0 0.0 0 0 0))

(event Custom|HAHA%20LASER%20GO%20BRRRRRRR
  ;[1 1 1] Laser Patern
  (if (Variables|Default|GetLaser_isUp)
    (bind _returnvalue (Actor|GetActorOfClass "/Game/Thibaud/Blueprints/Player/Bp_Starship.Bp_Starship_C"))
    (if (Collision|IsOverlappingActor _returnvalue :!class /Script/Engine.Actor)
      (Game|Damage|ApplyDamage _returnvalue 35.0 0 0))))

(event Custom|Aiming
  (bind _laser_aim (Variables|Default|GetLaser%20Aim))
  ;[1 1 1] Aiming System
  (Audio|PlaySoundatLocation "/Game/Assets/Audio/SOUNDBANK/SFX/SFX_SHIP/BOSS/SFX_SHIP_BOSS_StartFiring.SFX_SHIP_BOSS_StartFiring" "0, 0, 0" "0, 0, 0" 0.6 1.0 0.0 0 0 0)
  (Development|SetHiddeninGame _laser_aim false false)
  (Utilities|FlowControl|Delay 5.0)
  (Development|SetHiddeninGame _laser_aim true false))

(event Game|Damage|EventAnyDamage
  (params (Damage :type Float%20%28single-precision%29) (DamageType :type Damage%20Type%20Object%20Reference) (InstigatedBy :type Controller%20Object%20Reference) (DamageCauser :type Actor%20Object%20Reference))
  ;[1 1 1] Damaged !
  (if (Variables|Default|GetIsVulnerable)
    (Audio|PlaySound2D "/Game/Assets/Audio/SoundCues/SC_CruiserDamaged.SC_CruiserDamaged" 1.0 1.0 0.0 0 0)
    (Utilities|FlowControl|Sequence
      (:then_0
        (bind _output_get (Variables|Default|SetHealth (Math|Float|Clamp(Float) (- (Variables|Default|GetHealth) Damage) 0.0 (Variables|Default|GetMax_Health)))))
      (:then_1
        (if (<= (Variables|Default|GetHealth) 7e+02)
          (Utilities|FlowControl|DoOnce false
            (:Completed
              (bind _returnvalue (Actor|GetActorOfClass "/Game/Blueprints/Boss_The_Warden/BP_Bossfight_The_Warden.BP_Bossfight_The_Warden_C"))
              (Default|ShieldsUp _returnvalue)
              (Variables|Default|SetIsVulnerable false)))))
      (:then_2
        (if (<= (Variables|Default|GetHealth) 2e+02)
          (Utilities|FlowControl|DoOnce false
            (:Completed
              (bind _returnvalue_2 (Actor|GetActorOfClass "/Game/Blueprints/Boss_The_Warden/BP_Bossfight_The_Warden.BP_Bossfight_The_Warden_C"))
              (Default|ShieldsUp _returnvalue_2)
              (Variables|Default|SetIsVulnerable false)))))
      (:then_3
        (if (<= (Variables|Default|GetHealth) 0.0)
          (|Destroyed!))))))

(fn ConstructionScript)