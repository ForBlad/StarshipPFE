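; Boss fight controller for The Warden, running its shield, orbiting turrets, fighter waves, health bar and win screen.
; Every two turrets destroyed make the boss vulnerable and start the next pattern: shields drop, fighters spawn, laser fires, then turrets and shield return, with the third pattern repeating.
; A starship overlap starts timers for missiles and ground turret fire.
; Tick rotates turret pivots; laser and mine ground patterns are unwired.
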(event OnComponentBeginOverlap(bossfight_detector)
  (params (OverlappedComponent :type Primitive%20Component%20Object%20Reference) (OtherActor :type Actor%20Object%20Reference) (OtherComp :type Primitive%20Component%20Object%20Reference) (OtherBodyIndex :type Integer) (bFromSweep :type Boolean) (SweepResult :type Hit%20Result%20Structure%20%28by%20ref%29))
  ;[1 1 1] Bossfight Health Bar
  (Utilities|Casting|CastToBp_Starship OtherActor)
  (Utilities|FlowControl|Sequence
    (:then_0
      (if (> (Variables|Default|GetPatern%20Number) 0.0)
        _))
    (:then_1
      (bind _returnvalue (UserInterface|CreateWidget "/Game/Thibaud/Blueprints/Player/Balles/Widgets/WG_Warden_Healthbar.WG_Warden_Healthbar_C"))
      (UserInterface|Viewport|AddtoViewport _returnvalue 0))
    (:then_2
      (CallFunction|GroundsDefensesActivated))))

(event Custom|Turret%20Destroyed%20!
  ;[1 1 1] Turrets Counter
  (Variables|Default|SetTurretLost (+ (Variables|Default|GetTurretLost) 1.0))
  (if (>= (Variables|Default|GetTurretLost) 2.0)
    (Utilities|FlowControl|Sequence
      (:then_0
        (Utilities|FlowControl|DoOnce false
          (:Completed
            (Variables|Default|SetIsDormant false))))
      (:then_1
        (bind _returnvalue (Actor|GetActorOfClass "/Game/Blueprints/Boss_The_Warden/BP_The_Warden.BP_The_Warden_C"))
        (Variables|/Game/Blueprints/Boss_The_Warden/BP_The_Warden.BP_The_Warden_C|SetIsVulnerable _returnvalue true)
        (if (Variables|Default|GetFINAL%20FOOOORM)
          (CallFunction|BossThirdPatern)
          (Variables|Default|SetTurretLost 0.0)
          (else
            (switch int (Math|Float|Truncate (Variables|Default|GetPatern%20Number))
              (:0
                (CallFunction|BossFirstPatern)
                (Variables|Default|SetTurretLost 0.0 :!label _label)
                (Variables|Default|SetPatern%20Number (+ (Variables|Default|GetPatern%20Number) 1.0)))
              (:1
                (CallFunction|BossSecondPatern)
                (goto _label))
              (:2
                (CallFunction|BossThirdPatern)
                (Variables|Default|SetTurretLost 0.0)
                (Variables|Default|SetFINAL%20FOOOORM true)))))))))

(event Custom|Boss%20Second%20Patern
  ;[1 1 1] Boss 2nd Patern // 4th turret destroyed
  (CallFunction|ShieldsDown)
  (|Spawnfighters_2)
  (bind _returnvalue (Actor|GetActorOfClass "/Game/Blueprints/Boss_The_Warden/BP_The_Warden.BP_The_Warden_C"))
  (Rendering|Material|SetMaterial (Variables|/Game/Blueprints/Boss_The_Warden/BP_The_Warden.BP_The_Warden_C|GetBossBody _returnvalue) 0 "/Game/Léa/FX/Mat/M_RedDoor.M_RedDoor")
  (Utilities|FlowControl|Sequence
    (:then_0
      (Default|Aiming _returnvalue))
    (:then_1
      (Utilities|FlowControl|Delay 5.0)
      (Variables|Default|SetLaserIsReady true)
      (Default|LASERPATERN _returnvalue))
    (:then_2
      (Utilities|FlowControl|Delay 2e+01)
      (CallFunction|TurretRespawn)
      (Rendering|Material|SetMaterial (Variables|/Game/Blueprints/Boss_The_Warden/BP_The_Warden.BP_The_Warden_C|GetBossBody _returnvalue) 0 "/Game/Nat/Tech/Ground_Inst.Ground_Inst")
      (CallFunction|ShieldsUp))))

(event Custom|MISSILES
  ;[1 1 1] Missiles Firing
  (Default|MISSILEGO (stale EventBeginPlay _returnvalue)))

(event Custom|BOSSFIGHT%20END
  ;[1 1 1] Bossfight End
  (Actor|DestroyActor)
  (bind _asstarship_instance (Utilities|Casting|CastToStarshipInstance (Game|GetGameInstance)))
  (Variables|/Game/Blueprints/StarshipInstance.StarshipInstance_C|SetIsGameWon _asstarship_instance true)
  (bind _returnvalue (UserInterface|CreateWidget "/Game/WG_GameWin.WG_GameWin_C"))
  (UserInterface|Viewport|AddtoViewport _returnvalue 0))

(event Custom|Boss%20Third%20Patern
  ;[1 1 1] Boss 3rd Patern // 6th turret destroyed
  (CallFunction|ShieldsDown)
  (|Spawnfighters_3)
  (bind _returnvalue (Actor|GetActorOfClass "/Game/Blueprints/Boss_The_Warden/BP_The_Warden.BP_The_Warden_C"))
  (Rendering|Material|SetMaterial (Variables|/Game/Blueprints/Boss_The_Warden/BP_The_Warden.BP_The_Warden_C|GetBossBody _returnvalue) 0 "/Game/Léa/FX/Mat/M_RedDoor.M_RedDoor")
  (Utilities|FlowControl|Sequence
    (:then_0
      (Default|Aiming _returnvalue))
    (:then_1
      (Utilities|FlowControl|Delay 5.0)
      (Variables|Default|SetLaserIsReady true)
      (Default|LASERPATERN _returnvalue))
    (:then_2
      (Utilities|FlowControl|Delay 2e+01)
      (CallFunction|TurretRespawn)
      (Rendering|Material|SetMaterial (Variables|/Game/Blueprints/Boss_The_Warden/BP_The_Warden.BP_The_Warden_C|GetBossBody _returnvalue) 0 "/Game/Nat/Tech/Ground_Inst.Ground_Inst")
      (CallFunction|ShieldsUp))))

(event Custom|Boss%20First%20Patern
  ;[1 1 1] Boss 1st Patern // Upon waking up
  (CallFunction|ShieldsDown)
  (|Spawnfighters)
  (bind _returnvalue (Actor|GetActorOfClass "/Game/Blueprints/Boss_The_Warden/BP_The_Warden.BP_The_Warden_C"))
  (Rendering|Material|SetMaterial (Variables|/Game/Blueprints/Boss_The_Warden/BP_The_Warden.BP_The_Warden_C|GetBossBody _returnvalue) 0 "/Game/Léa/FX/Mat/M_RedDoor.M_RedDoor")
  (Utilities|FlowControl|Sequence
    (:then_0
      (Default|Aiming _returnvalue))
    (:then_1
      (Utilities|FlowControl|Delay 5.0)
      (Variables|Default|SetLaserIsReady true)
      (Default|LASERPATERN _returnvalue))
    (:then_2
      (Utilities|FlowControl|Delay 2e+01)
      (CallFunction|TurretRespawn)
      (Rendering|Material|SetMaterial (Variables|/Game/Blueprints/Boss_The_Warden/BP_The_Warden.BP_The_Warden_C|GetBossBody _returnvalue) 0 "/Game/Nat/Tech/Ground_Inst.Ground_Inst")
      (CallFunction|ShieldsUp))))

(event Custom|Turret%20Respawn
  ;[1 1 1] Turrets spawner
  (bind _returnvalue (Game|SpawnActorfromClass "/Game/Blueprints/Boss_The_Warden/BP_Warden_Turret.BP_Warden_Turret_C" (Math|Transform|MakeTransform (Transformation|GetWorldLocation (Variables|Default|GetTurret%20Spawn%2001)) "0,90.000000, 0" "2.000000,2.000000,2.000000") "Undefined" 0 0))
  (Transformation|AttachComponentToComponent _returnvalue (Variables|Default|GetPivot%20Point%20Turret) "None" "KeepWorld" "KeepRelative" "KeepRelative" true)
  (bind _returnvalue_2 (Game|SpawnActorfromClass "/Game/Blueprints/Boss_The_Warden/BP_Warden_Turret.BP_Warden_Turret_C" (Math|Transform|MakeTransform (Transformation|GetWorldLocation (Variables|Default|GetTurret%20Spawn%2002)) "0,90.000000, 0" "2.000000,2.000000,2.000000") "Undefined" 0 0))
  (Transformation|AttachComponentToComponent _returnvalue_2 (Variables|Default|GetPivot%20Point%20Turret%202) "None" "KeepWorld" "KeepRelative" "KeepRelative" true))

(event Custom|All%20Ground%20Turrets%20Firing
  ;[1 1 1] Ground Fire
  (bind _outactors (Actor|GetAllActorsOfClass "/Game/Blueprints/Boss_The_Warden/BP_Warden_GroundTurret.BP_Warden_GroundTurret_C"))
  (for _array_element _outactors
    (Default|FIRE _array_element)))

(event Custom|Grounds%20Defenses%20Activated
  ;[1 1 1] Activating Ground Turrets
  (Utilities|FlowControl|Sequence
    (:then_0
      (Utilities|Time|SetTimerbyEvent (delegate Custom|Ground%20Paterns) (Math|Random|RandomFloatinRange 1e+01 2e+01) true))
    (:then_1
      (Utilities|Time|SetTimerbyEvent (delegate Custom|MISSILES) 1e+01 true))))

(event Custom|Ground%20Paterns
  ;[1 1 1] Patern Selection
  (if (not (Variables|Default|GetIsDoingAPattern))
    (if (not (Variables|Default|GetIsVulnerable))
      (Variables|Default|SetIsDoingAPattern true)
      (switch int (Math|Random|RandomInteger 3)
        (:0
          _)
        (:1
          _)
        (:2
          _))
      ;[1 1 1] Pattern 1
      (bind _outactors (Actor|GetAllActorsOfClass "/Game/Blueprints/Boss_The_Warden/BP_Warden_GroundTurret.BP_Warden_GroundTurret_C"))
      (for _array_element _outactors
        (Default|FIRE _array_element)))))

(event Custom|Shields%20Down
  (bind _boss_shield (Variables|Default|GetBoss_Shield))
  ;[1 1 1] Shields
  (Development|SetHiddeninGame _boss_shield true false)
  (Collision|SetCollisionEnabled _boss_shield "NoCollision"))

(event Custom|Shields%20Up
  (bind _boss_shield (Variables|Default|GetBoss_Shield))
  ;[1 1 1] Shields
  (Development|SetHiddeninGame _boss_shield false false)
  (Collision|SetCollisionEnabled _boss_shield "QueryAndPhysics"))

(event EventBeginPlay
  ;[1 1 1] Initialisation
  (Variables|Default|SetIsVulnerable false)
  (Variables|Default|SetIsDormant true)
  (Utilities|FlowControl|Delay 1.0)
  (bind _returnvalue (Actor|GetActorOfClass "/Game/Blueprints/Boss_The_Warden/BP_The_Warden.BP_The_Warden_C")))

(event EventTick
  (params (DeltaSeconds :type Float%20%28single-precision%29))
  (bind _pivot_point_turret_2 (Variables|Default|GetPivot%20Point%20Turret%202))
  ;[1 1 1] EVENT TICK (FIND REPLACMENT)
  (Utilities|FlowControl|Sequence
    (:then_0
      (Transformation|SetRelativeRotation (Variables|Default|GetPivot%20Point%20Turret) (Math|Rotator|MakeRotator 0.0 0.0 (+ (.yaw (Variables|/Script/Engine.SceneComponent|GetRelativeRotation (Variables|Default|GetPivot%20Point%20Turret))) 0.2)) false false))
    (:then_1
      (Transformation|SetRelativeRotation _pivot_point_turret_2 (Math|Rotator|MakeRotator 0.0 0.0 (+ (.yaw (Variables|/Script/Engine.SceneComponent|GetRelativeRotation _pivot_point_turret_2)) 0.2)) false false))))

(fn ConstructionScript)