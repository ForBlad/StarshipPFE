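; Destructible ground turret for the Warden boss fight, with three attack patterns against the player starship.
; FIRE shows an aim laser then shoots a timed burst, LAZOR charges a beam that ticks damage on overlap, and MINES launches one missile.
; Each pattern ends by clearing the boss's IsDoingAPattern flag.
; AnyDamage drains clamped health, and at zero the turret explodes, notifies the boss and destroys itself.
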(event OnComponentEndOverlap(LaserBody)
  (params (OverlappedComponent :type Primitive%20Component%20Object%20Reference) (OtherActor :type Actor%20Object%20Reference) (OtherComp :type Primitive%20Component%20Object%20Reference) (OtherBodyIndex :type Integer))
  ;[1 1 1] Alien Laser // Patern II
  (Utilities|Casting|CastToBp_Starship OtherActor)
  (Utilities|Time|ClearTimerbyFunctionName 0 "HAHA LASER GO ZAP"))

(event OnComponentBeginOverlap(LaserBody)
  (params (OverlappedComponent :type Primitive%20Component%20Object%20Reference) (OtherActor :type Actor%20Object%20Reference) (OtherComp :type Primitive%20Component%20Object%20Reference) (OtherBodyIndex :type Integer) (bFromSweep :type Boolean) (SweepResult :type Hit%20Result%20Structure%20%28by%20ref%29))
  ;[1 1 1] Alien Laser // Patern II
  (Utilities|Casting|CastToBp_Starship OtherActor)
  (Utilities|Time|SetTimerbyEvent (delegate Custom|HAHA%20LASER%20GO%20ZAP) 0.1 true))

(event Custom|FIRE
  ;[1 1 1] Simple Fire // Patern 1
  (Development|SetHiddeninGame (Variables|Default|GetLaser%20Aim) false false)
  (Utilities|FlowControl|Delay 2.0)
  (Utilities|FlowControl|Sequence
    (:then_0
      (bind _recurve (Timeline|PEW PlayFromStart)
        (:Update
          (Transformation|SetRelativeRotation (Variables|Default|GetTurret_Body) (Math|Rotator|MakeRotator 0.0 _recurve 0.0) false false))))
    (:then_1
      (Utilities|FlowControl|Sequence
        (:then_0
          (Development|SetHiddeninGame (Variables|Default|GetLaser%20Aim) true false)
          (Utilities|Time|SetTimerbyEvent (delegate Custom|PEW%20PEW%20PEW) 0.2 true))
        (:then_1
          (Utilities|FlowControl|Delay 2.0)
          (Utilities|Time|ClearTimerbyFunctionName 0 "PEW PEW PEW")
          (Variables|/Game/Blueprints/Boss_The_Warden/BP_Bossfight_The_Warden.BP_Bossfight_The_Warden_C|SetIsDoingAPattern (stale EventBeginPlay _returnvalue) false))))))

(event Custom|PEW%20PEW%20PEW
  (bind _arrow (Variables|Default|GetArrow))
  ;[1 1 1] Simple Fire // Patern 1
  (Audio|PlaySoundatLocation "/Game/Assets/Audio/SoundCues/SC_BossTurretFiring.SC_BossTurretFiring" (Transformation|GetWorldLocation _arrow) "0, 0, 0" 1.0 1.0 0.0 0 0 0)
  (Game|SpawnActorfromClass "/Game/Blueprints/Projectiles/NewBP_ProjectileEnemyBase_Mine_noconstraint.NewBP_ProjectileEnemyBase_Mine_noconstraint_C" (Transformation|GetWorldTransform _arrow) "Undefined" 0 "(R=0.953125,G=0.041604,B=0.907584,A=0.000000)" 0))

(event Custom|HAHA%20LASER%20GO%20ZAP
  (bind _bpa_vaisseau (Variables|Default|GetBPA%20Vaisseau))
  ;[1 1 1] Alien Laser // Patern II
  (if (Variables|Default|GetLaser_isUp)
    (if (Collision|IsOverlappingActor _bpa_vaisseau :!class /Script/Engine.Actor)
      (Game|Damage|ApplyDamage _bpa_vaisseau 2e+01 0 0))))

(event Custom|WEAPONS%20HOT
  ;[1 1 1] Alien Laser // Patern II
  (Effects|SpawnEmitteratLocation "/Game/Léa/FX/Particle/P_Muzzle_laser_purplent.P_Muzzle_laser_purplent" (Transformation|GetWorldLocation (Variables|Default|GetArrow)) "0, 0, 0" (Math|Conversions|ToVector(Float) (stale Custom|LAZOR _newtrack_0))))

(event Custom|BLAST
  ;[1 1 1] Alien Laser // Patern II
  (Development|SetHiddeninGame (Variables|Default|GetLaser%20Body) false false)
  (Variables|Default|SetLaser_isUp true))

(event Custom|LAZOR
  ;[1 1 1] Alien Laser // Patern II
  (Utilities|FlowControl|Sequence
    (:then_0
      (bind _newtrack_0 (Timeline|LAZOR%20POWERING PlayFromStart)
        (:Finished
          (Utilities|FlowControl|Sequence
            (:then_0
              (CallFunction|BLAST))
            (:then_1
              (Utilities|FlowControl|Delay 5.0)
              (Development|SetHiddeninGame (Variables|Default|GetLaser%20Body) true false)
              (Variables|Default|SetLaser_isUp false)
              (Utilities|Time|ClearTimerbyFunctionName 0 "HAHA LASER GO ZAP")
              (Utilities|Time|ClearTimerbyFunctionName 0 "WEAPONS HOT")
              ;[1 1 1] Simple Fire // Patern 1
              (Variables|/Game/Blueprints/Boss_The_Warden/BP_Bossfight_The_Warden.BP_Bossfight_The_Warden_C|SetIsDoingAPattern (stale EventBeginPlay _returnvalue) false))))))
    (:then_1
      (Utilities|Time|SetTimerbyEvent (delegate Custom|WEAPONS%20HOT) 0.1 true))))

(event Custom|MINES
  ;[1 1 1] ROCKET // PATTERN III
  (Audio|PlaySoundatLocation "/Game/Assets/Audio/SoundCues/SC_Shield_Pulse.SC_Shield_Pulse" (.location (Transformation|GetWorldTransform (Variables|Default|GetArrow))) "0, 0, 0" 0.5 1.0 0.0 0 0 0)
  (Game|SpawnActorfromClass "/Game/Blueprints/Projectiles/NewBP_ProjectileEnemyBase_Missile_noconstraint.NewBP_ProjectileEnemyBase_Missile_noconstraint_C" (Transformation|GetWorldTransform (Variables|Default|GetArrow)) "Undefined" 0 "(R=0.953125,G=0.041604,B=0.907584,A=0.000000)" 0)
  ;[1 1 1] Simple Fire // Patern 1
  (Variables|/Game/Blueprints/Boss_The_Warden/BP_Bossfight_The_Warden.BP_Bossfight_The_Warden_C|SetIsDoingAPattern (stale EventBeginPlay _returnvalue) false))

(event EventBeginPlay
  ;[1 1 1] Initialisation
  (bind _returnvalue (Actor|GetActorOfClass "/Game/Blueprints/Boss_The_Warden/BP_Bossfight_The_Warden.BP_Bossfight_The_Warden_C"))
  (bind _returnvalue_2 (Actor|GetActorOfClass "/Game/Thibaud/Blueprints/Player/Bp_Starship.Bp_Starship_C"))
  (Variables|Default|SetBPA%20Vaisseau _returnvalue_2))

(event Game|Damage|EventAnyDamage
  (params (Damage :type Float%20%28single-precision%29) (DamageType :type Damage%20Type%20Object%20Reference) (InstigatedBy :type Controller%20Object%20Reference) (DamageCauser :type Actor%20Object%20Reference))
  ;[1 1 1] Damages
  (Audio|PlaySound2D "/Game/Assets/Audio/SoundCues/SC_FighterDamaged.SC_FighterDamaged" 1.0 1.0 0.0 0 0)
  (Variables|Default|SetHealth (Math|Float|Clamp(Float) (- (Variables|Default|GetHealth) Damage) 0.0 (Variables|Default|GetMax_Health)))
  (if (<= (Variables|Default|GetHealth) 0.0)
    (|Destroyed!)))

(fn ConstructionScript)