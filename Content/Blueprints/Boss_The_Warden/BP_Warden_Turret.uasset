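; Destructible turret for the Warden boss fight that tracks and shoots the player's starship.
; Tick uses a sphere overlap to detect the ship, turns the body toward it and fires projectiles, limited by an overheat counter with delayed reset.
; An on-screen check toggles an EnemyIndicator widget.
; Damage flashes the body red; at zero health it explodes and notifies BP_Bossfight_The_Warden, while the Raise timeline logic is never run.
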(event EventTick
  (params (DeltaSeconds :type Float%20%28single-precision%29))
  (bind _indicator_widget (Variables|Default|GetIndicator%20Widget))
  ;[1 1 1] Fighting
  (Utilities|FlowControl|Sequence
    (:then_0
      (bind _outactors (Collision|SphereOverlapActors (Transformation|GetActorLocation) 512.0 (Utilities|Array|MakeArray "ObjectTypeQuery1") "/Game/Thibaud/Blueprints/Player/Bp_Starship.Bp_Starship_C"))
      (Variables|Default|Setplayer_in_range (!= (Utilities|Array|Length _outactors) 0))
      (if (!= (Utilities|Array|Length _outactors) 0)
        (Utilities|FlowControl|DoOnce false :!label _label
          (:Completed
            (Audio|PlaySoundatLocation "/Game/Assets/Audio/SoundCues/SC_Detected.SC_Detected" (Transformation|GetWorldLocation (Variables|Default|GetArrow)) "0, 0, 0" 1.0 1.0 0.0 0 0 0)))
        (else
          (Utilities|FlowControl|Delay 1.0)
          (goto _label Reset))))
    (:then_1
      (if (> (Variables|Default|Getoverheat) 3.0)
        (Utilities|FlowControl|Delay 5.0)
        (Variables|Default|Setoverheat 0.0)))
    (:then_2
      (if (Variables|Default|Getplayer_in_range)
        (Transformation|SetWorldRotation (Variables|Default|GetTurret_Body) (Math|Rotator|Lerp(Rotator) (Transformation|GetActorRotation) (Math|Rotator|FindLookatRotation (Transformation|GetActorLocation) (Transformation|GetActorLocation (stale EventBeginPlay _returnvalue))) 0.2 true) true false)
        (if (<= (Variables|Default|Getoverheat) 2e+01)
          (|Fire))))
    (:then_3
      (bind _isonscreen_ (CallFunction|IsonScreen? self))
      (if _isonscreen_
        (Utilities|FlowControl|DoOnce false :!label _label_2
          (:Completed
            (Utilities|FlowControl|Sequence
              (:then_0
                (Widget|RemovefromParent _indicator_widget))
              (:then_1
                (goto _label_3 Reset)))))
        (else
          (Utilities|FlowControl|DoOnce false :!label _label_3
            (:Completed
              (Utilities|FlowControl|Sequence
                (:then_0
                  (goto _label_2 Reset))
                (:then_1
                  (UserInterface|Viewport|AddtoViewport _indicator_widget 0))))))))))

(event EventBeginPlay
  (bind _returnvalue (Actor|GetActorOfClass "/Game/Thibaud/Blueprints/Player/Bp_Starship.Bp_Starship_C"))
  (bind _returnvalue_2 (UserInterface|CreateWidget "/Game/Loic/AI_WIP_Behavior/EnemyIndicator.EnemyIndicator_C" (Game|GetPlayerController 0)))
  (Variables|/Game/Loic/AI_WIP_Behavior/EnemyIndicator.EnemyIndicator_C|SetWhoOwnsMe _returnvalue_2 self)
  (bind _output_get (Variables|Default|SetIndicator%20Widget _returnvalue_2))
  (UserInterface|Viewport|AddtoViewport _output_get 0))

(event Game|Damage|EventAnyDamage
  (params (Damage :type Float%20%28single-precision%29) (DamageType :type Damage%20Type%20Object%20Reference) (InstigatedBy :type Controller%20Object%20Reference) (DamageCauser :type Actor%20Object%20Reference))
  (bind _turret_body (Variables|Default|GetTurret_Body))
  ;[1 1 1] Damages
  (Audio|PlaySound2D "/Game/Assets/Audio/SoundCues/SC_FighterDamaged.SC_FighterDamaged" 1.0 1.0 0.0 0 0)
  (Variables|Default|SetHealth (Math|Float|Clamp(Float) (- (Variables|Default|GetHealth) Damage) 0.0 (Variables|Default|GetMax_Health)))
  (Utilities|FlowControl|Sequence
    (:then_0
      (Utilities|FlowControl|DoOnce false :!label _label
        (:Completed
          (Rendering|Material|SetMaterial _turret_body 0 "/Game/Thibaud/Blueprints/Player/Balles/MT_Red.MT_Red")
          (Utilities|FlowControl|Delay 0.1)
          (Rendering|Material|SetMaterial _turret_body 0 "/Game/Assets/Materials/PlayerGlow.PlayerGlow")
          (goto _label Reset))))
    (:then_1
      (if (<= (Variables|Default|GetHealth) 0.0)
        (|Destroyed!)))))

(fn ConstructionScript)

(fn IsonScreen?
  (bind _returnvalue (Game|GetPlayerController 0))
  (bind _returnvalue_2 (Viewport|GetViewportSize))
  (bind _turret_body (Variables|Default|GetTurret_Body))
  (bind _returnvalue_3 (Transformation|GetWorldLocation _turret_body))
  (bind _screenlocation (Class|PlayerController|ProjectWorldLocationtoScreen _returnvalue _returnvalue_3 false))
  (return (Math|Boolean|ANDBoolean (> (.x _screenlocation) 0.0) (> (.y _screenlocation) 0.0) (< (.x _screenlocation) (.x _returnvalue_2)) (< (.y _screenlocation) (.y _returnvalue_2)))))