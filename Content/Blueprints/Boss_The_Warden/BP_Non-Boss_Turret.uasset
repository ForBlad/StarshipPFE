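; Destructible enemy turret that tracks the player's starship and fires bursts of three missiles at it.
; Tick gates it by distance, hiding it when far; nearby, a screen-projection check arms firing while on screen and swaps in an off-screen indicator otherwise.
; Once armed, it rotates smoothly toward the ship and runs looping timed bursts with warm-up sound and material glow charge.
; Damage flashes it red and drains health until it explodes.
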(event OnComponentBeginOverlap(ActivationRadius)
  (params (OverlappedComponent :type Primitive%20Component%20Object%20Reference) (OtherActor :type Actor%20Object%20Reference) (OtherComp :type Primitive%20Component%20Object%20Reference) (OtherBodyIndex :type Integer) (bFromSweep :type Boolean) (SweepResult :type Hit%20Result%20Structure%20%28by%20ref%29))
  (Utilities|Casting|CastToBp_Starship OtherActor)
  (Utilities|FlowControl|DoOnce false))

(event Custom|Respect%20Women%20Mode
  (if (Variables|Default|GetInRange?)
    (Variables|Default|SetMax%20Glow 1.0)
    (Variables|Default|SetGlow%20Value 1.0)
    (bind _returnvalue (Audio|SpawnSoundAttached "/Game/Loic/TurretWarmingUp.TurretWarmingUp" (Variables|Default|GetArrow) "None" "0, 0, 0" "0, 0, 0" "KeepRelativeOffset" false 1.0 1.0 0.0 0 0))
    (Audio|Components|Audio|Play _returnvalue 0.0)
    (Utilities|Time|SetTimerbyEvent (delegate Custom|Respect%20Women%20Mode) 3.0 true 0.5)
    (Variables|Default|SetBurstIncr 0)
    (CallFunction|KeepYourHandsOffOfHer!)))

(event Custom|Keep%20Your%20Hands%20Off%20Of%20Her!
  (bind _arrow (Variables|Default|GetArrow))
  (bind _returnvalue (Transformation|GetWorldTransform _arrow))
  (Variables|Default|SetMax%20Glow 1e+03)
  (Utilities|FlowControl|Delay 1.0)
  (if (< (Variables|Default|GetBurstIncr) 3) :!label _label
    (Utilities|FlowControl|Sequence
      (:then_0
        (Math|Integer|IncrementInt (Variables|Default|GetBurstIncr)
          (:%20%20
            (if (Variables|Default|GetInRange?)
              (Utilities|IsValid (Variables|Default|GetBPA%20Vaisseau)
                (:Is%20Valid
                  (Variables|Default|SetGlow%20Value 0.0)
                  (Game|SpawnActorfromClass "/Game/Blueprints/Projectiles/NewBP_ProjectileEnemyBase_Missile_noconstraint1.NewBP_ProjectileEnemyBase_Missile_noconstraint1_C" (Math|Transform|MakeTransform (.location _returnvalue) (.rotation _returnvalue) "1,1,1") "AdjustIfPossibleButAlwaysSpawn" self "(R=0.567708,G=0.016375,B=0.518136,A=0.000000)" 0)
                  (Effects|SpawnEmitterAttached "/Game/Léa/FX/Particle/P_Muzzle_laser_ennemy.P_Muzzle_laser_ennemy" _arrow "None")
                  (Audio|PlaySoundatLocation "/Game/Loic/turret_shot1.turret_shot1" (.location _returnvalue) "0, 0, 0" 0.6 1.0 0.0 0 0 0)))))))
      (:then_1
        (Utilities|FlowControl|Delay 0.5)
        (goto _label)))
    (else
      (Variables|Default|SetMax%20Glow 5e+01)
      (Variables|Default|SetGlow%20Value 0.0))))

(event EventBeginPlay
  (Variables|Default|SetHealth 4e+02)
  (bind _returnvalue (Actor|GetActorOfClass "/Game/Thibaud/Blueprints/Player/Bp_Starship.Bp_Starship_C"))
  (Variables|Default|SetBPA%20Vaisseau _returnvalue)
  (bind _returnvalue_2 (UserInterface|CreateWidget "/Game/Loic/AI_WIP_Behavior/EnemyIndicator.EnemyIndicator_C" (Game|GetPlayerController 0)))
  (bind _output_get (Variables|Default|SetIndicator _returnvalue_2))
  (Variables|/Game/Loic/AI_WIP_Behavior/EnemyIndicator.EnemyIndicator_C|SetWhoOwnsMe _output_get self)
  (Rendering|Material|SetScalarParameterValueonMaterials (Variables|Default|GetStaticMesh) "Glow Power" 5e+01))

(event EventTick
  (params (DeltaSeconds :type Float%20%28single-precision%29))
  (bind _returnvalue (* DeltaSeconds 1.7))
  (bind _turret_body (Variables|Default|GetTurret_Body))
  (bind _bpa_vaisseau (Variables|Default|GetBPA%20Vaisseau))
  (bind _indicator (Variables|Default|GetIndicator))
  (bind _bpa_vaisseau_2 (Variables|Default|GetBPA%20Vaisseau))
  (bind _turret_body_2 (Variables|Default|GetTurret_Body))
  (bind _returnvalue_2 (Transformation|GetWorldRotation _turret_body_2))
  (bind _returnvalue_3 (Transformation|GetWorldLocation _turret_body_2))
  (bind _indicatorsonscreen (Variables|/Game/Thibaud/Blueprints/Player/Bp_Starship.Bp_Starship_C|GetIndicatorsOnScreen _bpa_vaisseau_2))
  (bind _collision_ship (Variables|/Game/Thibaud/Blueprints/Player/Bp_Starship.Bp_Starship_C|GetCollision_Ship _bpa_vaisseau))
  (bind _returnvalue_4 (Transformation|GetWorldLocation _collision_ship))
  (bind _returnvalue_5 (Math|Vector|GetUnitDirection(Vector) _returnvalue_3 _returnvalue_4))
  (bind _returnvalue_6 (Math|Conversions|RotationFromXVector _returnvalue_5))
  (bind _returnvalue_7 (Math|Rotator|Lerp(Rotator) (Math|Rotator|MakeRotator (.roll _returnvalue_2) (.pitch _returnvalue_2) (.yaw _returnvalue_2)) (Math|Rotator|MakeRotator (.roll _returnvalue_6) (.pitch _returnvalue_6) (.yaw _returnvalue_6)) _returnvalue true))
  (if (< (Transformation|GetDistanceTo self (Variables|Default|GetBPA%20Vaisseau)) 2e+03)
    (Utilities|FlowControl|Sequence
      (:then_0
        (if (Variables|Default|GetInRange?)
          (Transformation|SetActorRotation (Math|Rotator|MakeRotator 0.0 (.pitch _returnvalue_7) (.yaw _returnvalue_7)))))
      (:then_1
        ;[1 1 1] OFF-SCREEN INDICATOR
        (bind _isonscreen_ (CallFunction|IsonScreen?))
        (if _isonscreen_
          (Utilities|FlowControl|DoOnce false :!label _label
            (:Completed
              (Utilities|FlowControl|Sequence
                (:then_0
                  (Widget|RemovefromParent _indicator)
                  (Math|Integer|DecrementInt _indicatorsonscreen
                    (:%20%20
                      ;[1 1 1] ALLOW TO FIRE
                      (Variables|Default|SetInRange? true)
                      (CallFunction|RespectWomenMode))))
                (:then_1
                  (goto _label_2 Reset)))))
          (elif (Variables|Default|GetInRange?)
            (Utilities|FlowControl|DoOnce false :!label _label_2
              (:Completed
                (Utilities|FlowControl|Sequence
                  (:then_0
                    (goto _label Reset))
                  (:then_1
                    (UserInterface|Viewport|AddtoViewport _indicator 0)
                    (Math|Integer|IncrementInt _indicatorsonscreen
                      (:%20%20
                        (Variables|Default|SetInRange? false)
                        (Utilities|IsValid (stale Custom|Respect%20Women%20Mode _returnvalue)
                          (:Is%20Valid
                            (Audio|Components|Audio|Stop (stale Custom|Respect%20Women%20Mode _returnvalue)))))))))))))
      (:then_2
        ;[1 1 1] MAKE INVISIBLE/VISIBLE
        (Utilities|FlowControl|DoOnce true :!label _label_3
          (:Completed
            (Rendering|SetVisibility _turret_body true true)
            (goto _label_4 Reset))))
      (:then_3
        (if (< (Variables|Default|GetGlow%20Value) (Variables|Default|GetMax%20Glow))
          (bind _output_get (Variables|Default|SetGlow%20Value (+ (Variables|Default|GetGlow%20Value) 5.0))))
        (Rendering|Material|SetScalarParameterValueonMaterials (Variables|Default|GetStaticMesh) "Glow Power" _output_get)))
    (else
      (Utilities|FlowControl|DoOnce false :!label _label_4
        (:Completed
          (Widget|RemovefromParent (Variables|Default|GetIndicator))
          (Rendering|SetVisibility _turret_body false true)
          (goto _label_3 Reset))))))

(event Game|Damage|EventAnyDamage
  (params (Damage :type Float%20%28single-precision%29) (DamageType :type Damage%20Type%20Object%20Reference) (InstigatedBy :type Controller%20Object%20Reference) (DamageCauser :type Actor%20Object%20Reference))
  (bind _staticmesh (Variables|Default|GetStaticMesh))
  (Utilities|FlowControl|Sequence
    (:then_0
      (Utilities|FlowControl|DoOnce false :!label _label
        (:Completed
          (Rendering|Material|SetMaterial _staticmesh 0 "/Game/Thibaud/Blueprints/Player/Balles/MT_Red.MT_Red")
          (Utilities|FlowControl|Delay 0.1)
          (Rendering|Material|SetMaterial _staticmesh 0 "/Game/Nat/Tech/M_Walls_Barres.M_Walls_Barres")
          (goto _label Reset))))
    (:then_1
      (Audio|PlaySound2D "/Game/Assets/Audio/SoundCues/SC_FighterDamaged.SC_FighterDamaged" 1.0 1.0 0.0 0 0)
      (Variables|Default|SetHealth (Math|Float|Clamp(Float) (- (Variables|Default|GetHealth) Damage) 0.0 (Variables|Default|GetMax_Health)))
      (if (<= (Variables|Default|GetHealth) 0.0)
        (|Destroyed!_2)))))

(fn ConstructionScript
  (|CallParentFunction))

(fn IsonScreen?
  (bind _returnvalue (Game|GetPlayerController 0))
  (bind _returnvalue_2 (Viewport|GetViewportSize))
  (bind _arrow (Variables|Default|GetArrow))
  (bind _returnvalue_3 (Transformation|GetWorldLocation _arrow))
  (bind _screenlocation (Class|PlayerController|ProjectWorldLocationtoScreen _returnvalue _returnvalue_3 false))
  (return (Math|Boolean|ANDBoolean (> (.x _screenlocation) 0.0) (> (.y _screenlocation) 0.0) (< (.x _screenlocation) (.x _returnvalue_2)) (< (.y _screenlocation) (.y _returnvalue_2)))))