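; Player rail projectile that pierces what it overlaps, damaging every actor except starships.
; Box overlaps apply damage and spawn a pixel explosion tinted to the projectile colour without destroying the projectile.
; A static mesh hit spawns the same explosion and destroys it.
; The construction script creates and stores a dynamic material, stretches the projectile by its scale, and sets initial and maximum movement speed.
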(event OnComponentHit(StaticMesh)
  (params (HitComponent :type Primitive%20Component%20Object%20Reference) (OtherActor :type Actor%20Object%20Reference) (OtherComp :type Primitive%20Component%20Object%20Reference) (NormalImpulse :type Vector :default "0, 0, 0") (Hit :type Hit%20Result%20Structure%20%28by%20ref%29))
  (bind _returnvalue (Effects|SpawnEmitteratLocation "/Game/Assets/Particles/P_Pixel_ExplosionColorable.P_Pixel_ExplosionColorable" (Transformation|GetActorLocation)))
  (Effects|Components|ParticleSystem|SetVectorParameter _returnvalue "ColorMuzzle" (Math|Conversions|ToVector(LinearColor) (Variables|Default|GetProjectileColour)))
  (Actor|DestroyActor))

(event OnComponentBeginOverlap(Box)
  (params (OverlappedComponent :type Primitive%20Component%20Object%20Reference) (OtherActor :type Actor%20Object%20Reference) (OtherComp :type Primitive%20Component%20Object%20Reference) (OtherBodyIndex :type Integer) (bFromSweep :type Boolean) (SweepResult :type Hit%20Result%20Structure%20%28by%20ref%29))
  (Utilities|Casting|CastToBp_Starship OtherActor
    (:CastFailed
      (Game|Damage|ApplyDamage OtherActor (Variables|Default|GetDamage) 0 0)
      (bind _returnvalue (Effects|SpawnEmitteratLocation "/Game/Assets/Particles/P_Pixel_ExplosionColorable.P_Pixel_ExplosionColorable" (Transformation|GetActorLocation)))
      (Effects|Components|ParticleSystem|SetVectorParameter _returnvalue "ColorMuzzle" (Math|Conversions|ToVector(LinearColor) (Variables|Default|GetProjectileColour))))))

(fn ConstructionScript
  (bind _projectilemovement (Variables|Default|GetProjectileMovement))
  (bind _returnvalue (Rendering|Material|CreateDynamicMaterialInstance (Variables|Default|GetProjectile) 0 0 "None" :!class /Script/Engine.PrimitiveComponent))
  (Variables|Default|SetProjectileMaterial _returnvalue)
  (Transformation|SetWorldScale3D (Variables|Default|GetProjectile) (* "4.000000,1.500000,1.500000" (Variables|Default|GetScale)))
  (bind _output_get (Variables|/Script/Engine.ProjectileMovementComponent|SetMaxSpeed _projectilemovement (Variables|Default|GetSpeed)))
  (Variables|/Script/Engine.ProjectileMovementComponent|SetInitialSpeed _projectilemovement _output_get))