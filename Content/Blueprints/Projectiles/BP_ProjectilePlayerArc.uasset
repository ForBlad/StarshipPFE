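; BP_ProjectilePlayerArc is a player projectile that travels a jittering path from StartPoint to EndPoint, then destroys itself.
; After a brief delay on BeginPlay, a timeline moves the root by lerping between the two points.
; A high-frequency sine with a per-instance random frequency offsets all axes equally, scaled by the distance between the points.
; It performs no sweep or hit logic, so the motion is purely positional.
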(event EventBeginPlay
  (Utilities|FlowControl|Delay 0.01)
  (bind _output_get (Variables|Default|SetRandomFloat (Math|Random|RandomFloat)))
  (bind _newtrack_0 (Timeline|Timeline_0 PlayFromStart)
    (:Update
      (Transformation|SetWorldLocation (Variables|Default|GetDefaultSceneRoot) (+ (Math|Vector|Lerp(Vector) (Variables|Default|GetStartPoint) (Variables|Default|GetEndPoint) _newtrack_0) (* (Math|Trig|Sin(Radians) (* _newtrack_0 1e+04 _output_get)) 15.0 (/ (Math|Vector|VectorLength (- (Variables|Default|GetStartPoint) (Variables|Default|GetEndPoint))) 2e+02))) false false))
    (:Finished
      (Utilities|FlowControl|Delay 0.05)
      (Actor|DestroyActor))))

(fn ConstructionScript)