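; Enemy flame projectile that attaches a flamethrower emitter, colored by its AI_Cruser2 owner, and grows via a scale timeline.
; Tick adds the owner's velocity to its initial velocity.
; Box overlap ignores other projectiles, damages the starship, and reverses velocity on forcefields, destroying itself unless the bouncer is on.
; Bounced flames take the shield player's color, replay the scaling and damage enemy fighters, cruisers and turrets instead.
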(event OnComponentBeginOverlap(Projectile)
  (params (OverlappedComponent :type Primitive%20Component%20Object%20Reference) (OtherActor :type Actor%20Object%20Reference) (OtherComp :type Primitive%20Component%20Object%20Reference) (OtherBodyIndex :type Integer) (bFromSweep :type Boolean) (SweepResult :type Hit%20Result%20Structure%20%28by%20ref%29)))

(event OnComponentBeginOverlap(Box)
  (params (OverlappedComponent :type Primitive%20Component%20Object%20Reference) (OtherActor :type Actor%20Object%20Reference) (OtherComp :type Primitive%20Component%20Object%20Reference) (OtherBodyIndex :type Integer) (bFromSweep :type Boolean) (SweepResult :type Hit%20Result%20Structure%20%28by%20ref%29))
  (bind _returnvalue (Math|Random|RandomFloatinRange 1.5 3.0))
  (bind _returnvalue_2 (Transformation|GetActorLocation))
  (bind _self self)
  (bind _projectile (Variables|Default|GetProjectile))
  (bind _damage (Variables|Default|GetDamage))
  (bind _asbp_projectile_enemy_base (Utilities|Casting|CastToBP_ProjectileEnemyBase OtherActor)
    (:then
      (Collision|IgnoreActorwhenMoving (Variables|/Game/Blueprints/Projectiles/BP_ProjectileEnemyBase.BP_ProjectileEnemyBase_C|GetStaticMesh _asbp_projectile_enemy_base) _self true))
    (:CastFailed
      (bind _asbp_projectile_enemy_flame (Utilities|Casting|CastToBP_ProjectileEnemyFlame OtherActor)
        (:then
          (Collision|IgnoreActorwhenMoving (Variables|BP_ProjectileEnemyFlame_C|GetProjectile _asbp_projectile_enemy_flame) _self true)
          (Collision|IgnoreActorwhenMoving (Variables|BP_ProjectileEnemyFlame_C|GetBox _asbp_projectile_enemy_flame) _self true))
        (:CastFailed
          (bind _asbp_projectile_player_base (Utilities|Casting|CastToBP_ProjectilePlayerBase OtherActor)
            (:then
              (Collision|IgnoreActorwhenMoving OverlappedComponent _asbp_projectile_player_base true)
              (Development|PrintString "AM IGNORING"))
            (:CastFailed
              (if (Variables|Default|GetBounced!)
                (bind _asai_fighter_new_2 (Utilities|Casting|CastToAI_Fighter_New2 OtherActor)
                  (:then
                    (Game|Damage|ApplyDamage _asai_fighter_new_2 8.0 0 0))
                  (:CastFailed
                    (bind _asai_cruser_2 (Utilities|Casting|CastToAI_Cruser2 OtherActor)
                      (:then
                        (Development|PrintString "Hello")
                        (Game|Damage|ApplyDamage _asai_cruser_2 8.0 0 0))
                      (:CastFailed
                        (bind _asbp_non__boss_turret (Utilities|Casting|CastToBP_Non-Boss_Turret OtherActor))
                        (Game|Damage|ApplyDamage _asbp_non__boss_turret 8.0 0 0)))))
                (Effects|SpawnEmitteratLocation "/Game/Léa/FX/Particle/P_Impact_ship.P_Impact_ship" (Transformation|GetActorLocation) "0, 0, 0" "0.100000,0.100000,0.100000")
                (else
                  (bind _asforcefield_actor (Utilities|Casting|CastToForcefieldActor OtherActor)
                    (:then
                      (Variables|Default|SetInitialVelocity (* (Variables|Default|GetInitialVelocity) -1.0))
                      (Effects|SpawnEmitteratLocation "/Game/Léa/FX/Particle/P_Impact_shield.P_Impact_shield" _returnvalue_2 "0, 0, 0" (Math|Vector|MakeVector _returnvalue _returnvalue _returnvalue))
                      (if (Variables|/Game/Assets/Meshes/AsstesUpdated/Shield/ForcefieldActor.ForcefieldActor_C|GetBouncer_on _asforcefield_actor)
                        (Audio|PlaySoundatLocation "/Game/Assets/Audio/SOUNDBANK/SFX/SFX_SHIP/MAINSHIP/MAINSHIP_SHIELD/shield2_bounce.shield2_bounce" _returnvalue_2 "0, 0, 0" 1.0 1.0 0.0 0 0 0)
                        (Variables|Default|SetBounced! true)
                        (Utilities|FlowControl|Sequence
                          (:then_0
                            (bind _asbp_player (Utilities|Casting|CastToBP_Player (Variables|/Game/Thibaud/Blueprints/Player/Post/BPA_Post_Parent.BPA_Post_Parent_C|GetCurrentPlayer (Variables|/Game/Assets/Meshes/AsstesUpdated/Shield/ForcefieldActor.ForcefieldActor_C|GetPostShield _asforcefield_actor))))
                            (bind _returnvalue_3 (Rendering|Material|GetVectorParameterValue "/Game/Assets/Assets_Jules/PlayersColorsCollection.PlayersColorsCollection" (Utilities|String|StringToName (Utilities|String|Append "Player" (Utilities|String|ToString(Integer) (+ (Variables|/Game/Thibaud/Blueprints/Player/BP_Player.BP_Player_C|GetPlayerNumber _asbp_player) 1)))) :!class /Script/Engine.KismetMaterialLibrary))
                            (bind _output_get (Variables|Default|SetCruiserColor _returnvalue_3))
                            (CallFunction|ColoronSpawn 0 1e+02 (stale EventBeginPlay _returnvalue) 1e+02)
                            (Rendering|Components|Light|SetLightColor (Variables|Default|GetPointLight) _output_get true))
                          (:then_1
                            (bind _wasssup (Timeline|SCAAAAAAAAALE PlayFromStart)
                              (:Update
                                (Transformation|SetWorldScale3D (Variables|Default|GetBox) (Math|Conversions|ToVector(Float) _wasssup))
                                (Utilities|IsValid _projectile
                                  (:Is%20Valid
                                    (Transformation|SetWorldScale3D _projectile (Math|Conversions|ToVector(Float) _wasssup))))))))
                        (else
                          (Audio|PlaySoundatLocation "/Game/Assets/Audio/SOUNDBANK/SFX/SFX_SHIP/MAINSHIP/MAINSHIP_SHIELD/shield2.shield2" _returnvalue_2 "0, 0, 0" 0.7 0.9 0.0 0 0 0)
                          (Actor|DestroyActor))))
                    (:CastFailed
                      (bind _asbp_starship (Utilities|Casting|CastToBp_Starship OtherActor)
                        (:then
                          (if (not (Variables|Default|GetBounced!))
                            (Effects|SpawnEmitteratLocation "/Game/Léa/FX/Particle/P_Impact_ship.P_Impact_ship" _returnvalue_2 "0, 0, 0" "0.500000,0.500000,0.500000")
                            (Game|Damage|ApplyDamage _asbp_starship _damage 0 0)
                            (Default|DamageStack _asbp_starship _damage)
                            (Actor|DestroyActor)))
                        (:CastFailed
                          (Effects|SpawnEmitteratLocation "/Game/Assets/Particles/P_Pixel_Explosion.P_Pixel_Explosion" _returnvalue_2)
                          (Development|PrintString (Utilities|GetDisplayName OverlappedComponent))
                          (Actor|DestroyActor))))))))))))))

(event OnComponentHit(StaticMesh)
  (params (HitComponent :type Primitive%20Component%20Object%20Reference) (OtherActor :type Actor%20Object%20Reference) (OtherComp :type Primitive%20Component%20Object%20Reference) (NormalImpulse :type Vector :default "0, 0, 0") (Hit :type Hit%20Result%20Structure%20%28by%20ref%29))
  (Actor|DestroyActor))

(event OnComponentHit(Projectile)
  (params (HitComponent :type Primitive%20Component%20Object%20Reference) (OtherActor :type Actor%20Object%20Reference) (OtherComp :type Primitive%20Component%20Object%20Reference) (NormalImpulse :type Vector :default "0, 0, 0") (Hit :type Hit%20Result%20Structure%20%28by%20ref%29)))

(event EventBeginPlay
  (bind _projectile (Variables|Default|GetProjectile))
  (bind _arrow (Variables|Default|GetArrow))
  (Utilities|FlowControl|Sequence
    (:then_0
      (Variables|Default|SetInitialVelocity (Variables|/Script/Engine.MovementComponent|GetVelocity (Variables|Default|GetProjectileMovement)))
      (bind _returnvalue (Effects|SpawnEmitterAttached "/Game/Assets/Particles/P_FlamethrowerColorable.P_FlamethrowerColorable" (Variables|Default|GetProjectile) "None" (Transformation|GetWorldLocation _arrow) (Transformation|GetWorldRotation _arrow) "1.000000,2.000000,2.000000" "KeepWorldPosition"))
      (bind _asai_cruser_2 (Utilities|Casting|CastToAI_Cruser2 (Components|GetOwner)))
      (Default|ColoronSpawn _asai_cruser_2 0 1e+02 _returnvalue 1e+02 0 false))
    (:then_1
      (Rendering|Material|SetVectorParameterValue (Variables|Default|GetProjectileMaterial) "Colour" (Variables|Default|GetProjectileColour) :!class /Script/Engine.MaterialInstanceDynamic)
      (Rendering|Components|Light|SetLightColor (Variables|Default|GetPointLight) (Variables|Default|GetCruiserColor) true)
      (bind _wasssup (Timeline|SCAAAAAAAAALE PlayFromStart)
        (:Update
          (Transformation|SetWorldScale3D (Variables|Default|GetBox) (Math|Conversions|ToVector(Float) _wasssup))
          (Utilities|IsValid _projectile
            (:Is%20Valid
              (Transformation|SetWorldScale3D _projectile (Math|Conversions|ToVector(Float) _wasssup)))))))))

(event EventTick
  (params (DeltaSeconds :type Float%20%28single-precision%29))
  (bind _returnvalue (Components|GetOwner))
  (Utilities|IsValid _returnvalue
    (:Is%20Valid
      (Variables|/Script/Engine.MovementComponent|SetVelocity (Variables|Default|GetProjectileMovement) (+ (Variables|Default|GetInitialVelocity) (Transformation|GetVelocity _returnvalue))))))

(fn ConstructionScript
  (bind _projectilemovement (Variables|Default|GetProjectileMovement))
  (bind _returnvalue (Rendering|Material|CreateDynamicMaterialInstance (Variables|Default|GetProjectile) 0 0 "None" :!class /Script/Engine.PrimitiveComponent))
  (Variables|Default|SetProjectileMaterial _returnvalue)
  (Transformation|SetWorldScale3D (Variables|Default|GetProjectile) (Variables|Default|GetScale))
  (bind _output_get (Variables|/Script/Engine.ProjectileMovementComponent|SetMaxSpeed _projectilemovement (Variables|Default|GetSpeed)))
  (Variables|/Script/Engine.ProjectileMovementComponent|SetInitialSpeed _projectilemovement _output_get)
  (bind _returnvalue_2 (Actor|GetActorOfClass "/Game/Thibaud/Blueprints/Player/Bp_Starship.Bp_Starship_C"))
  (Variables|Default|SetBPA%20Vaisseau _returnvalue_2))

(fn ColoronSpawn
  (params (NewParam :type Static%20Mesh%20Component%20Object%20Reference) (NewParam1 :type Float%20%28single-precision%29) (NewParam2 :type Particle%20System%20Component%20Object%20Reference) (NewParam3 :type Float%20%28single-precision%29) (NewParam4 :type Niagara%20Component%20Object%20Reference))
  (bind _cruisercolor (Variables|Default|GetCruiserColor))
  (Utilities|FlowControl|Sequence
    (:then_0
      (Utilities|IsValid 0
        (:Is%20Valid
          (Rendering|Material|SetMaterial NewParam 0 (Utilities|Array|Get(acopy) (Rendering|Material|GetMaterials (Variables|/Game/Loic/AI_WIP_Behavior/AI_Cruser2.AI_Cruser2_C|GetHull (Variables|Default|GetWhoOwnsMe)))))
          (Rendering|Material|SetScalarParameterValueonMaterials NewParam "emissive" NewParam1)
          (Utilities|IsValid 0
            (:Is%20Valid
              (Niagara|SetNiagaraVariable(LinearColor) NewParam4 "ColorTrail" _cruisercolor)
              (Rendering|Components|Light|SetLightColor (Variables|Default|GetPointLight) _cruisercolor true))))))
    (:then_1
      (Utilities|IsValid NewParam2
        (:Is%20Valid
          (Effects|Components|ParticleSystem|SetVectorParameter NewParam2 "ColorMuzzle" (Math|Conversions|ToVector(LinearColor) (* _cruisercolor NewParam3))))))))