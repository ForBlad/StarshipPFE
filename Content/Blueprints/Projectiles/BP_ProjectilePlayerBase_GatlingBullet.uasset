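; Gatling bullet variant of the player projectile, handling its material, scale and launch speed.
; The construction script creates a dynamic material instance, applies the scale and calls DelayedSetSpeed, without running the parent construction script.
; That event caps max speed at Speed, sets initial speed to a fraction of it, then multiplies velocity after a near-zero delay for a kicked-up launch.
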(event Custom|DelayedSetSpeed
  (bind _speed (Variables|Default|GetSpeed))
  (bind _projectilemovement (Variables|Default|GetProjectileMovement))
  (Utilities|FlowControl|Sequence
    (:then_0
      (Variables|/Script/Engine.ProjectileMovementComponent|SetMaxSpeed _projectilemovement _speed)
      (Variables|/Script/Engine.ProjectileMovementComponent|SetInitialSpeed _projectilemovement (/ _speed 5.0)))
    (:then_1
      (Utilities|FlowControl|Delay 0.0001)
      (Variables|/Script/Engine.MovementComponent|SetVelocity _projectilemovement (* (Variables|/Script/Engine.MovementComponent|GetVelocity _projectilemovement) 1e+01)))))

(fn ConstructionScript
  (bind _returnvalue (Rendering|Material|CreateDynamicMaterialInstance (Variables|Default|GetProjectile) 0 0 "None" :!class /Script/Engine.PrimitiveComponent))
  (Variables|Default|SetProjectileMaterial _returnvalue)
  (Transformation|SetWorldScale3D (Variables|Default|GetProjectile) (Variables|Default|GetScale))
  (CallFunction|DelayedSetSpeed))