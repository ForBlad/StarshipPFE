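; Alien bomb projectile that flies for five seconds, then explodes and destroys itself.
; Construction creates a dynamic material and applies the configured scale and initial speed.
; On BeginPlay, the FlyAway timeline drives the movement component's max speed while a delay counts down to detonation.
; Detonation spawns an alien bomb area-of-effect actor and an enlarged explosion particle effect at the projectile's location.
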(event Custom|BOOOOOM
  (Game|SpawnActorfromClass "/Game/Blueprints/Projectiles/BP_AOE_AlienBomb.BP_AOE_AlienBomb_C" (Math|Conversions|ToTransform(Vector) (Transformation|GetWorldLocation (Variables|Default|GetProjectile))) "Undefined" 0 0)
  (Effects|SpawnEmitteratLocation "/Game/Assets/Particles/Explosion_v2/P_ExplosionV3.P_ExplosionV3" (Transformation|GetWorldLocation (Variables|Default|GetProjectile)) "0, 0, 0" "3.000000,3.000000,3.000000")
  (Actor|DestroyActor))

(event EventBeginPlay
  (Utilities|FlowControl|Sequence
    (:then_0
      (bind _spedo (Timeline|fly%20away PlayFromStart)
        (:Update
          (Variables|/Script/Engine.ProjectileMovementComponent|SetMaxSpeed (Variables|Default|GetProjectileMovement) _spedo))))
    (:then_1
      (Utilities|FlowControl|Delay 5.0)
      (CallFunction|BOOOOOM))))

(fn ConstructionScript
  (bind _returnvalue (Rendering|Material|CreateDynamicMaterialInstance (Variables|Default|GetProjectile) 0 0 "None" :!class /Script/Engine.PrimitiveComponent))
  (Variables|Default|SetProjectileMaterial _returnvalue)
  (Transformation|SetWorldScale3D (Variables|Default|GetProjectile) (Variables|Default|GetScale))
  (Variables|/Script/Engine.ProjectileMovementComponent|SetInitialSpeed (Variables|Default|GetProjectileMovement) (Variables|Default|GetSpeed)))