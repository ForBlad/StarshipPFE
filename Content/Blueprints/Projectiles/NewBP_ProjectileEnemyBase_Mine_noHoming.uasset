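; Enemy mine projectile that damages Bp_Starship on mesh contact and self-destructs with a small particle burst.
; BeginPlay targets the starship, with homing gated by IsHoming, while timelines drive homing acceleration and speed, then zero MaxSpeed.
; It also destroys itself after a delay, on any damage or when its box overlaps a ForcefieldActor.
; Capsule overlaps feed a collide event that makes other enemy projectiles' meshes ignore it when moving.
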(event OnComponentBeginOverlap(Box)
  (params (OverlappedComponent :type Primitive%20Component%20Object%20Reference) (OtherActor :type Actor%20Object%20Reference) (OtherComp :type Primitive%20Component%20Object%20Reference) (OtherBodyIndex :type Integer) (bFromSweep :type Boolean) (SweepResult :type Hit%20Result%20Structure%20%28by%20ref%29))
  ;[1 1 1] Detect close activity
  (Utilities|Casting|CastToForcefieldActor OtherActor)
  ;[1 1 1] Destroy mines after 7 sec
  (Actor|DestroyActor))

(event OnComponentBeginOverlap(Capsule)
  (params (OverlappedComponent :type Primitive%20Component%20Object%20Reference) (OtherActor :type Actor%20Object%20Reference) (OtherComp :type Primitive%20Component%20Object%20Reference) (OtherBodyIndex :type Integer) (bFromSweep :type Boolean) (SweepResult :type Hit%20Result%20Structure%20%28by%20ref%29))
  (CallFunction|Collide? OtherActor))

(event OnComponentBeginOverlap(StaticMesh)
  (params (OverlappedComponent :type Primitive%20Component%20Object%20Reference) (OtherActor :type Actor%20Object%20Reference) (OtherComp :type Primitive%20Component%20Object%20Reference) (OtherBodyIndex :type Integer) (bFromSweep :type Boolean) (SweepResult :type Hit%20Result%20Structure%20%28by%20ref%29))
  (Utilities|Casting|CastToBp_Starship OtherActor)
  (Game|Damage|ApplyDamage OtherActor 5.0 0 0)
  ;[1 1 1] Destroy mines after 7 sec
  (Actor|DestroyActor))

(event EventBeginPlay
  (bind _projectilemovement (Variables|Default|GetProjectileMovement))
  (bind _projectilemovement_2 (Variables|Default|GetProjectileMovement))
  (|CallParentFunction)
  ;[1 1 1] Homing
  (bind _returnvalue (Actor|GetActorOfClass "/Game/Thibaud/Blueprints/Player/Bp_Starship.Bp_Starship_C"))
  (Variables|/Script/Engine.ProjectileMovementComponent|SetHomingTargetComponent _projectilemovement_2 (Variables|/Script/Engine.Actor|GetRootComponent _returnvalue))
  (Variables|/Script/Engine.ProjectileMovementComponent|SetbIsHomingProjectile _projectilemovement_2 (Variables|Default|GetIsHoming))
  (Utilities|FlowControl|Sequence
    (:then_0
      (bind _targeting_system (Timeline|NYOOOM PlayFromStart)
        (:Update
          (Variables|/Script/Engine.ProjectileMovementComponent|SetHomingAccelerationMagnitude _projectilemovement_2 _targeting_system))))
    (:then_1
      ;[1 1 1] Speed
      (bind _time_slow (Timeline|SO%20SLOOOW PlayFromStart)
        (:Update
          (Variables|/Script/Engine.ProjectileMovementComponent|SetInitialSpeed _projectilemovement _time_slow)
          (Variables|Default|SetSpeed _time_slow)
          (Variables|/Script/Engine.ProjectileMovementComponent|SetMaxSpeed _projectilemovement _time_slow))
        (:Finished
          (Variables|/Script/Engine.ProjectileMovementComponent|SetMaxSpeed _projectilemovement 0.0))))
    (:then_2
      ;[1 1 1] Destroy mines after 7 sec
      (Utilities|FlowControl|Delay 9.0)
      (Actor|DestroyActor))))

(event EventDestroyed
  ;[1 1 1] Explode
  (Effects|SpawnEmitteratLocation "/Game/Assets/Particles/Lea_particles/Explosion-FINALE/ROUGENT.ROUGENT" (Transformation|GetActorLocation) "0, 0, 0" "0.200000,0.200000,0.200000"))

(event Game|Damage|EventAnyDamage
  (params (Damage :type Float%20%28single-precision%29) (DamageType :type Damage%20Type%20Object%20Reference) (InstigatedBy :type Controller%20Object%20Reference) (DamageCauser :type Actor%20Object%20Reference))
  (Actor|DestroyActor))

(event EventCollide?
  (params (Actor :type Actor%20Object%20Reference))
  (bind _asbp_projectile_enemy_base (Utilities|Casting|CastToBP_ProjectileEnemyBase Actor))
  (Collision|IgnoreActorwhenMoving (Variables|/Game/Blueprints/Projectiles/BP_ProjectileEnemyBase.BP_ProjectileEnemyBase_C|GetStaticMesh _asbp_projectile_enemy_base) self true))

(fn ConstructionScript
  (|CallParentFunction))