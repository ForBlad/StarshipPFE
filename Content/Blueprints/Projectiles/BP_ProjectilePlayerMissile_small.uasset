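; Small player missile projectile that steers toward a target rotation, easing its forward vector and velocity every tick.
; Overlapping anything but a starship deals damage and detonates it; mesh hits or a one-second lifetime detonate it without direct damage.
; Detonation plays sound, camera shake and force feedback, spawns an area-of-effect missile actor and destroys itself.
; BeginPlay picks the explosion particle from the ring material, apparently one per player colour.
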(event OnComponentHit(StaticMesh)
  (params (HitComponent :type Primitive%20Component%20Object%20Reference) (OtherActor :type Actor%20Object%20Reference) (OtherComp :type Primitive%20Component%20Object%20Reference) (NormalImpulse :type Vector :default "0, 0, 0") (Hit :type Hit%20Result%20Structure%20%28by%20ref%29))
  (bind _returnvalue (Transformation|GetActorLocation))
  (Effects|SpawnEmitteratLocation (Variables|Default|GetExplosion) _returnvalue)
  (Utilities|FlowControl|Sequence
    (:then_0
      (Audio|PlaySoundatLocation "/Game/Assets/Audio/explosion_light.explosion_light" _returnvalue "0, 0, 0" 1.0 1.0 0.0 0 0 0)
      (Class|PlayerController|ClientPlayCameraShake (Game|GetPlayerController 0) "/Game/Blueprints/CS_Wall_Impact.CS_Wall_Impact_C" 0.05 "CameraLocal" "0, 0, 0")
      (bind _outactors (Actor|GetAllActorsOfClass "/Game/Thibaud/Blueprints/Player/BP_Player.BP_Player_C"))
      (for _array_element _outactors
        (Default|ForceFeedback _array_element 0.3 0.2 true)))
    (:then_1
      (Game|SpawnActorfromClass "/Game/Blueprints/Projectiles/BP_AOE_Missile.BP_AOE_Missile_C" (Math|Transform|MakeTransform _returnvalue "0, 0, 0" "1,1,1") "Undefined" 0 0)
      (Actor|DestroyActor))))

(event OnComponentBeginOverlap(Detection_box)
  (params (OverlappedComponent :type Primitive%20Component%20Object%20Reference) (OtherActor :type Actor%20Object%20Reference) (OtherComp :type Primitive%20Component%20Object%20Reference) (OtherBodyIndex :type Integer) (bFromSweep :type Boolean) (SweepResult :type Hit%20Result%20Structure%20%28by%20ref%29))
  (bind _returnvalue (Transformation|GetActorLocation))
  (Utilities|Casting|CastToBp_Starship OtherActor
    (:CastFailed
      (Game|Damage|ApplyDamage OtherActor (Variables|Default|GetDamage) 0 0)
      (Effects|SpawnEmitteratLocation (Variables|Default|GetExplosion) _returnvalue)
      (Utilities|FlowControl|Sequence
        (:then_0
          (Audio|PlaySoundatLocation "/Game/Assets/Audio/explosion_light.explosion_light" _returnvalue "0, 0, 0" 1.0 1.0 0.0 0 0 0)
          (Class|PlayerController|ClientPlayCameraShake (Game|GetPlayerController 0) "/Game/Blueprints/CS_Wall_Impact.CS_Wall_Impact_C" 0.05 "CameraLocal" "0, 0, 0")
          (bind _outactors (Actor|GetAllActorsOfClass "/Game/Thibaud/Blueprints/Player/BP_Player.BP_Player_C"))
          (for _array_element _outactors
            (Default|ForceFeedback _array_element 0.3 0.2 true)))
        (:then_1
          (Game|SpawnActorfromClass "/Game/Blueprints/Projectiles/BP_AOE_Missile.BP_AOE_Missile_C" (Math|Transform|MakeTransform _returnvalue "0, 0, 0" "1,1,1") "Undefined" 0 0)
          (Actor|DestroyActor))))))

(event EventBeginPlay
  (bind _returnvalue (Transformation|GetActorLocation))
  (bind _ringmaterial (Variables|Default|GetRingMaterial))
  (Utilities|FlowControl|Sequence
    (:then_0
      (if (== _ringmaterial "/Game/Assets/Assets_Jules/Spaceman_MAT_BODY_CIRCLE.Spaceman_MAT_BODY_CIRCLE")
        (Variables|Default|SetExplosion "/Game/Assets/Particles/Lea_particles/Explosion-FINALE/P_Explosion_FinaleP1.P_Explosion_FinaleP1")
        (elif (== _ringmaterial "/Game/Assets/Assets_Jules/Spaceman_MAT_BODY2_CIRCLE.Spaceman_MAT_BODY2_CIRCLE")
          (Variables|Default|SetExplosion "/Game/Assets/Particles/Lea_particles/Explosion-FINALE/P_Explosion_FinaleP2.P_Explosion_FinaleP2")
          (elif (== _ringmaterial "/Game/Assets/Assets_Jules/Spaceman_MAT_BODY3_CIRCLE.Spaceman_MAT_BODY3_CIRCLE")
            (Variables|Default|SetExplosion "/Game/Assets/Particles/Lea_particles/Explosion-FINALE/P_Explosion_FinaleP3.P_Explosion_FinaleP3")
            (else
              (Variables|Default|SetExplosion "/Game/Assets/Particles/Lea_particles/Explosion-FINALE/P_Explosion_FinaleP4.P_Explosion_FinaleP4"))))))
    (:then_1
      (bind _output_get (Variables|Default|SetCanRotate? true))
      (Utilities|FlowControl|Delay 1.0)
      (Effects|SpawnEmitteratLocation (Variables|Default|GetExplosion) _returnvalue)
      (Utilities|FlowControl|Sequence
        (:then_0
          (Audio|PlaySoundatLocation "/Game/Assets/Audio/explosion_light.explosion_light" _returnvalue "0, 0, 0" 1.0 1.0 0.0 0 0 0)
          (Class|PlayerController|ClientPlayCameraShake (Game|GetPlayerController 0) "/Game/Blueprints/CS_Wall_Impact.CS_Wall_Impact_C" 0.05 "CameraLocal" "0, 0, 0")
          (bind _outactors (Actor|GetAllActorsOfClass "/Game/Thibaud/Blueprints/Player/BP_Player.BP_Player_C"))
          (for _array_element _outactors
            (Default|ForceFeedback _array_element 0.3 0.2 true)))
        (:then_1
          (Game|SpawnActorfromClass "/Game/Blueprints/Projectiles/BP_AOE_Missile.BP_AOE_Missile_C" (Math|Transform|MakeTransform _returnvalue "0, 0, 0" "1,1,1") "Undefined" 0 0)
          (Actor|DestroyActor))))))

(event EventTick
  (params (DeltaSeconds :type Float%20%28single-precision%29))
  (bind _projectile (Variables|Default|GetProjectile))
  (if (stale EventBeginPlay _output_get)
    (Transformation|SetWorldRotation _projectile (Math|Conversions|RotationFromXVector (Math|Vector|Lerp(Vector) (Math|Rotator|GetRotationXVector (Transformation|GetWorldRotation _projectile)) (Math|Rotator|GetRotationXVector (Variables|Default|GetTargetRotation)) 0.06)) false false)
    (Variables|/Script/Engine.MovementComponent|SetVelocity (Variables|Default|GetProjectileMovement) (* (Math|Vector|GetForwardVector _projectile) (Variables|Default|GetSpeed)))))

(fn ConstructionScript
  (bind _projectilemovement (Variables|Default|GetProjectileMovement))
  (Transformation|SetWorldScale3D (Variables|Default|GetStaticMesh) (Variables|Default|GetScale))
  (bind _output_get (Variables|/Script/Engine.ProjectileMovementComponent|SetMaxSpeed _projectilemovement (Variables|Default|GetSpeed)))
  (Variables|/Script/Engine.ProjectileMovementComponent|SetInitialSpeed _projectilemovement _output_get))